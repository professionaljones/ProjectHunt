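; BP_HOLE is a configurable wormhole effect built from a particle system and a point light.
; Exposed variables set the light's color, intensity and source radius, plus the particle's color and size, with one color shared by both.
; A dynamic material instance on the particle receives the flipbook diffuse and normal textures, distortion, intensity and rotation speed.
; The Construction Script and BeginPlay run identical setup, applying the look at construction and again when play starts.
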(event `self.ReceiveBeginPlay`
  (bind _pointlight (`self.PointLight`))
  (bind _hole_particle (`self.hole_particle`))
  ;[0 0.2829 1] Set Light Color
  (`LightComponent.SetLightColor` _pointlight (`self.Color_rays`) true)
  ;[0 0.2829 1] Set Light intensity
  (`LightComponent.SetIntensity` _pointlight (`self.Light_intensity`))
  ;[0 0.2829 1] Set Light Radius
  (`PointLightComponent.SetSourceRadius` _pointlight (`self.Light_radius`))
  ;[0 0.2829 1] Set Material dymanic instance
  (bind _returnvalue (`PrimitiveComponent.CreateDynamicMaterialInstance` _hole_particle 0 (`self.Material`)))
  ;[0 0.2829 1] Set color Rays
  (`ParticleSystemComponent.SetVectorParameter` _hole_particle "Color" (`KismetMathLibrary.Conv_LinearColorToVector` (`self.Color_rays`)))
  ;[0 0.2829 1] Set flipbook diffuse texture
  (`MaterialInstanceDynamic.SetTextureParameterValue` _returnvalue "Diffusetexture" (`self.Diffuse_texture`))
  ;[0 0.2829 1] Set flipbook normal texture
  (`MaterialInstanceDynamic.SetTextureParameterValue` _returnvalue "Normaltexture" (`self.Normal_texture`))
  ;[0 0.2829 1] Distortion effect value<1
  (`MaterialInstanceDynamic.SetScalarParameterValue` _returnvalue "Distortion" (`self.Distortion`))
  ;[0 0.2829 1] Color intensity
  (`MaterialInstanceDynamic.SetScalarParameterValue` _returnvalue "intensity" (`self.Color_Intensity`))
  ;[0 0.2829 1] rotation speed
  (`MaterialInstanceDynamic.SetScalarParameterValue` _returnvalue "timer" (`self.Speed`))
  ;[0 0.2829 1] Wormhole size
  (`ParticleSystemComponent.SetVectorParameter` (`self.hole_particle`) "Size" (`KismetMathLibrary.Conv_DoubleToVector` (`self.Particle_Size`))))

(fn `UserConstructionScript`
  (bind _pointlight (`self.PointLight`))
  (bind _hole_particle (`self.hole_particle`))
  ;[0 0.2829 1] Set Light Color
  (`LightComponent.SetLightColor` _pointlight (`self.Color_rays`) true)
  ;[0 0.2829 1] Set Light intensity
  (`LightComponent.SetIntensity` _pointlight (`self.Light_intensity`))
  ;[0 0.2829 1] Set Light Radius
  (`PointLightComponent.SetSourceRadius` _pointlight (`self.Light_radius`))
  ;[0 0.2829 1] Set Material dymanic instance
  (bind _returnvalue (`PrimitiveComponent.CreateDynamicMaterialInstance` _hole_particle 0 (`self.Material`)))
  ;[0 0.2829 1] Set color Rays
  (`ParticleSystemComponent.SetVectorParameter` _hole_particle "Color" (`KismetMathLibrary.Conv_LinearColorToVector` (`self.Color_rays`)))
  ;[0 0.2829 1] Set flipbook diffuse texture
  (`MaterialInstanceDynamic.SetTextureParameterValue` _returnvalue "Diffusetexture" (`self.Diffuse_texture`))
  ;[0 0.2829 1] Set flipbook normal texture
  (`MaterialInstanceDynamic.SetTextureParameterValue` _returnvalue "Normaltexture" (`self.Normal_texture`))
  ;[0 0.2829 1] Distortion effect value<1
  (`MaterialInstanceDynamic.SetScalarParameterValue` _returnvalue "Distortion" (`self.Distortion`))
  ;[0 0.2829 1] Color intensity
  (`MaterialInstanceDynamic.SetScalarParameterValue` _returnvalue "intensity" (`self.Color_Intensity`))
  ;[0 0.2829 1] rotation speed
  (`MaterialInstanceDynamic.SetScalarParameterValue` _returnvalue "timer" (`self.Speed`))
  ;[0 0.2829 1] Wormhole size
  (`ParticleSystemComponent.SetVectorParameter` (`self.hole_particle`) "Size" (`KismetMathLibrary.Conv_DoubleToVector` (`self.Particle_Size`))))