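; BP_CoverBase is a damageable, self-regenerating cover actor that stops blocking a custom collision channel when depleted.
; AnyDamage lowers health in the HuntStats component; at zero the mesh ignores GameTraceChannel1 and the regen timer restarts if inactive.
; A looping timer starts at BeginPlay for periodic regeneration, and RegenHealth restores blocking at full health.
; Both damage and regen push the health percentage into a dynamic material parameter for visual feedback.
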(event `self.ReceiveBeginPlay`
  (bind _staticmesh (`self.StaticMesh`))
  (bind _huntstats (`self.HuntStats`))
  (bind _returnvalue (`PrimitiveComponent.CreateDynamicMaterialInstance` _staticmesh 0 (`PrimitiveComponent.GetMaterial` _staticmesh 0) "None"))
  (set `self.DynMat` _returnvalue)
  (set `HuntStatsComponent.CurrentHealth` (`HuntStatsComponent.MaxHealth` _huntstats) _huntstats)
  (bind _returnvalue_2 (`KismetSystemLibrary.K2_SetTimerDelegate` (`|CreateDelegate` :!event `RegenHealth`) 0.5 true))
  (set `self.RegenHealthTimer` _returnvalue_2))

(event `self.ReceiveAnyDamage`
  (params (Damage :type "Float (single-precision)") (DamageType :type "DamageType Object Reference") (InstigatedBy :type "Controller Object Reference") (DamageCauser :type "Actor Object Reference"))
  (bind _huntstats (`self.HuntStats`))
  (`HuntStatsComponent.DamageHealth` _huntstats Damage)
  (`MaterialInstanceDynamic.SetScalarParameterValue` (`self.DynMat`) (`self.NewVar_0`) (`HuntStatsComponent.GetHealthPercentage` _huntstats))
  (if (<= (`HuntStatsComponent.GetCurrentHealth` _huntstats) 0.0)
    (`PrimitiveComponent.SetCollisionResponseToChannel` (`self.StaticMesh`) "ECC_GameTraceChannel1" "ECR_Ignore")
    (if (not (`KismetSystemLibrary.K2_IsTimerActiveHandle` (`self.RegenHealthTimer`)))
      (bind _returnvalue (`KismetSystemLibrary.K2_SetTimerDelegate` (`|CreateDelegate` :!event `RegenHealth`) 0.5 true))
      (set `self.RegenHealthTimer` _returnvalue))))

(event `RegenHealth`
  (bind _huntstats (`self.HuntStats`))
  (`HuntStatsComponent.RecoverHealth` _huntstats 1.0)
  (`MaterialInstanceDynamic.SetScalarParameterValue` (`self.DynMat`) (`self.NewVar_0`) (`HuntStatsComponent.GetHealthPercentage` _huntstats))
  (if (>= (`HuntStatsComponent.GetCurrentHealth` _huntstats) (`HuntStatsComponent.GetMaxHealth` _huntstats))
    (`PrimitiveComponent.SetCollisionResponseToChannel` (`self.StaticMesh`) "ECC_GameTraceChannel1" "ECR_Block")))

(fn `UserConstructionScript`)