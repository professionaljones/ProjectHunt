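; BP_Dark_Rifle_AI is a rifle weapon Blueprint, named as the AI variant of the Dark Rifle.
; It relies on its parent class for begin play, construction and firing, adding only a fire sound played at the weapon's location on each OnWeaponFire.
; A node setting the weapon owner from a ProjectHuntCharacter cast is left unconnected and never runs.
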(event `self.ReceiveBeginPlay`
  (`parent.ReceiveBeginPlay`))

(event `HuntWeaponInterface.OnWeaponFire`
  (`parent.OnWeaponFire`)
  (`GameplayStatics.PlaySoundAtLocation` (`self.WeaponFireSound`) (`self.K2_GetActorLocation`) (struct) 1.0 1.0 0.0 null null null))

(fn `UserConstructionScript`
  (`parent.UserConstructionScript`))