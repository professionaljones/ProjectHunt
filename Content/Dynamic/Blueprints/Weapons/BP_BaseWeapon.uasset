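; Base weapon Blueprint for the Hunt characters, handling equip, switching and projectile firing.
; BeginPlay loads stats and upgrade data from DataTables, calculates damage and creates a dynamic material for the timeline-driven materialize effect.
; Firing spawns projectile classes mapped by state, from the muzzle for the player or eye view for other instigators, with a debug sphere.
; Alt fire consumes player missiles and launches normal or charged alt projectiles.
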(event `self.ReceiveBeginPlay`
  (bind _weaponmeshfp (`self.WeaponMeshFP`))
  (bind _weaponstatstable (`self.WeaponStatsTable`))
  (bind _weaponupgradedatatable (`self.WeaponUpgradeDataTable`))
  (bind _weaponupgradedata (`self.WeaponUpgradeData`))
  (`parent.ReceiveBeginPlay`)
  (bind _returnvalue (`PrimitiveComponent.CreateDynamicMaterialInstance` _weaponmeshfp 0 (`PrimitiveComponent.GetMaterial` _weaponmeshfp 0) "None"))
  (set `self.DynWeaponMaterial` _returnvalue)
  (`|ExecutionSequence`
    (:`then_0`
      (`/Engine/EditorBlueprintResources/StandardMacros.IsValid` _weaponstatstable
        (:`Is Valid`
          (bind _returnvalue_2 (`|GetDataTableRow` _weaponstatstable (`self.WeaponBaseStatRowName`))
            (:`then`
              (`self.SetWeaponStats` _returnvalue_2)
              (`self.CalculateDamage`))))))
    (:`then_1`
      (`/Engine/EditorBlueprintResources/StandardMacros.IsValid` _weaponupgradedatatable
        (:`Is Valid`
          (bind _returnvalue_3 (`|GetDataTableRow` _weaponupgradedatatable "1")
            (:`then`
              (bind (_weapondamagelevel _damageupgradeamount _damageupgradeprice _fireratelevel _firerateupgradeamount _firerateupgradeprice _chargeratelevel _chargerateamountincrease _chargerateupgradeprice _chargelimitlevel _chargelimitamountincrease _chargelimitupgradeprice) (break `WeaponUpgradeData` _returnvalue_3))
              (setmembers `WeaponUpgradeData` :`StructRef` _weaponupgradedata :`WeaponDamageLevel` _weapondamagelevel :`DamageUpgradeAmount` _damageupgradeamount :`DamageUpgradePrice` _damageupgradeprice :`FireRateLevel` _fireratelevel :`FireRateUpgradeAmount` _firerateupgradeamount :`FireRateUpgradePrice` _firerateupgradeprice :`ChargeRateLevel` _chargeratelevel :`ChargeRateAmountIncrease` _chargerateamountincrease :`ChargeRateUpgradePrice` _chargerateupgradeprice :`ChargeLimitLevel` _chargelimitlevel :`ChargeLimitAmountIncrease` _chargelimitamountincrease :`ChargeLimitUpgradePrice` _chargelimitupgradeprice))
            (:`RowNotFound`
              (setmembers `WeaponUpgradeData` :`StructRef` _weaponupgradedata :`WeaponDamageLevel` 0 :`DamageUpgradeAmount` 0.0 :`DamageUpgradePrice` 0.0 :`FireRateLevel` 0 :`FireRateUpgradeAmount` 0.0 :`FireRateUpgradePrice` 0.0 :`ChargeRateLevel` 0 :`ChargeRateAmountIncrease` 0.0 :`ChargeRateUpgradePrice` 0.0 :`ChargeLimitLevel` 0 :`ChargeLimitAmountIncrease` 0.0 :`ChargeLimitUpgradePrice` 0.0 :!label _label))))
        (:`Is Not Valid`
          (goto _label))))))

(event `HuntWeaponInterface.OnWeaponFire`
  (if (or (`KismetSystemLibrary.IsValid` (`self.WeaponOwner`)) (`KismetSystemLibrary.IsValid` (`self.GetInstigator`)))
    (`self.SpawnProjectile`)))

(event `HuntWeaponInterface.OnWeaponAltFire`
  (bind _ashunt_player_character (cast `HuntPlayerCharacter` (`GameplayStatics.GetPlayerCharacter` 0) :!pure true))
  (if (`KismetSystemLibrary.IsValid` (`self.WeaponOwner`))
    (if (`self.bIsCharging`)
      (set `self.CurrentWeaponCharge` 0.0)
      (`self.EndFire`)
      (`HuntPlayerCharacter.ConsumeMissiles` _ashunt_player_character 5)
      (`self.FireCAltProjectile`)
      (else
        (`self.EndFire`)
        (`HuntPlayerCharacter.ConsumeMissiles` _ashunt_player_character 1)
        (`self.FireAltProjectile`)))
    (else
      (`self.SetWeaponOwner` _ashunt_player_character))))

(event `self.ReceiveEndPlay`
  (params (EndPlayReason :type "EEndPlayReason Enum" :default "Destroyed"))
  (switch `EEndPlayReason` EndPlayReason
    (:`Destroyed`
      (`TimelineComponent.ReverseFromEnd` (`self.SpawnWeaponAnimTimeline`)))))

(fn `CheckProjectileStatus`)

(fn `FireAltProjectile`
  (bind (_value _returnvalue) (`BlueprintMapLibrary.Map_Find` (`self.WeaponProjectiles`) (`self.WeaponProjectileState`)))
  (if (not (`HuntPlayerCharacter.bAreMissilesEmpty` (cast `HuntPlayerCharacter` (`self.WeaponOwner`) :!pure true)))
    (set `self.WeaponProjectileState` "Projectile_Alt")
    (if _returnvalue
      (`|SpawnActorFromClass` _value (`KismetMathLibrary.MakeTransform` (`SceneComponent.GetSocketLocation` (`self.WeaponMeshFP`) (`self.WeaponMuzzlePoint`)) (`Pawn.GetControlRotation` (`self.WeaponOwner`)) (0.5 0.5 0.5)) "AdjustIfPossibleButAlwaysSpawn" "OverrideRootScale" self 0.0 null)
      (`AudioComponent.SetSound` (`self.WeaponAudioComponent`) (`self.WeaponAltFireSound`))
      (`AudioComponent.Play` (`self.WeaponAudioComponent`) 0.0))))

(fn `FireCAltProjectile`
  (bind (_value _returnvalue) (`BlueprintMapLibrary.Map_Find` (`self.WeaponProjectiles`) "Projectile_ChargeAlt"))
  (if _returnvalue
    (`|SpawnActorFromClass` _value (`KismetMathLibrary.MakeTransform` (`SceneComponent.GetSocketLocation` (`self.WeaponMeshFP`) (`self.WeaponMuzzlePoint`)) (`Pawn.GetControlRotation` (`self.WeaponOwner`)) (0.25 0.25 0.25)) "AdjustIfPossibleButAlwaysSpawn" "OverrideRootScale" self 0.0 null)
    (`GameplayStatics.PlaySoundAtLocation` "/Game/Static/Audio/SFX/Player/172631__qubodup__power-up-charge-remix-of-legolunatic-s-charged-laser-151243.172631__qubodup__power-up-charge-remix-of-legolunatic-s-charged-laser-151243" (`self.K2_GetActorLocation`) (struct) 1.0 1.0 0.0 null null null)))

(fn `OnSpawn`
  (`TimelineComponent.PlayFromStart` (`self.SpawnWeaponAnimTimeline`))
  (`GameplayStatics.PlaySoundAtLocation` (`self.WeaponEquipSound`) (`self.K2_GetActorLocation`) (struct) 1.0 1.0 0.0 null null null))

(fn `OnSwitch`
  (`TimelineComponent.ReverseFromEnd` (`self.SpawnWeaponAnimTimeline`))
  (`self.SetActorHiddenInGame` true)
  (`AudioComponent.Stop` (`self.WeaponAudioComponent`))
  (`AudioComponent.Stop` (`self.WeaponAltAudioComponent`))
  (`self.EndFire`))

(fn `SpawnChargeVFX`
  (bind _weaponmeshfp (`self.WeaponMeshFP`))
  (bind _weaponmuzzlepoint (`self.WeaponMuzzlePoint`))
  (if (`self.bIsCharging`)
    (`GameplayStatics.SpawnEmitterAttached` (`ParticleSystemComponent.Template` (`/Game/Dynamic/Blueprints/Weapons/Projectiles/BP_HuntProjectile_Base.MainParticleSystem` (cast `/Game/Dynamic/Blueprints/Weapons/Projectiles/BP_HuntProjectile_Base` (`self.ProjectileToSpawn`) :!pure true))) _weaponmeshfp _weaponmuzzlepoint (`SceneComponent.GetSocketLocation` _weaponmeshfp _weaponmuzzlepoint) (struct) (* (1.0 1.0 1.0) (`self.CurrentWeaponCharge`)))))

(fn `SpawnProjectile`
  (bind _returnvalue (`self.GetInstigator`))
  (bind _returnvalue_2 (`self.GetInstigator`))
  (bind ((`WeaponDamageLevel` _weapondamagelevel) (`FireRateLevel` _fireratelevel) (`ChargeRateLevel` _chargeratelevel) (`ChargeLimitLevel` _chargelimitlevel) (`BaseDamage` _basedamage) (`TotalDamage` _totaldamage)) (break `WeaponStatsData` (`self.WeaponStatsData`)))
  (bind (_value _returnvalue_3) (`BlueprintMapLibrary.Map_Find` (`self.WeaponProjectiles`) (`self.WeaponProjectileState`)))
  (bind (_outlocation _outrotation) (`self.GetActorEyesViewPoint` _returnvalue))
  (set `self.WeaponProjectileState` "Projectile_Normal")
  (if _returnvalue_3
    (if (!= _returnvalue_2 (`GameplayStatics.GetPlayerPawn` 0))
      (`|SpawnActorFromClass` _value (`KismetMathLibrary.MakeTransform` _outlocation _outrotation) "Undefined" "OverrideRootScale" (`ProjectHuntCharacter.GetCurrentWeapon` (cast `ProjectHuntCharacter` _returnvalue :!pure true)) _totaldamage _returnvalue)
      (`KismetSystemLibrary.DrawDebugSphere` _outlocation 100.0 12 (struct :`R` 1.0 :`G` 1.0 :`B` 1.0 :`A` 1.0) 15.0 3.0)
      (else
        (`|SpawnActorFromClass` _value (`KismetMathLibrary.MakeTransform` (`SceneComponent.GetSocketLocation` (`self.WeaponMeshFP`) (`self.WeaponMuzzlePoint`)) (`Pawn.GetControlRotation` (`self.WeaponOwner`)) (0.5 0.5 0.5)) "Undefined" "OverrideRootScale" self _totaldamage _returnvalue_2)
        (message `HuntCharacterInterface.OnWeaponFire` (`GameplayStatics.GetPlayerCharacter` 0))))))

(fn `UserConstructionScript`)