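; Base projectile for Project Hunt weapons, handling damage, critical hits, homing and impact effects.
; It copies damage stats from its owning weapon, then on hit applies point or regular damage, reporting player style and damage scoring.
; Non-stat targets and refusing doors can make it bounce.
; Homing sphere-traces ahead and interpolates toward hits; AI projectiles damaged by the player drop health or missile pickups.
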(event `self.ReceiveBeginPlay`
  (bind _returnvalue (`self.GetOwner`))
  (bind _weaponref (`self.WeaponRef`))
  (if (`self.bFromWeapon`)
    (`/Engine/EditorBlueprintResources/StandardMacros.IsValid` _returnvalue
      (:`Is Valid`
        (bind _output_get (set `self.WeaponRef` (cast `/Game/Dynamic/Blueprints/Weapons/BP_BaseWeapon` _returnvalue :!pure true)))
        (bind ((`BaseDamage` _basedamage) (`TotalDamage` _totaldamage) (`CriticalHitDamage` _criticalhitdamage)) (break `WeaponStatsData` (`HuntWeapon.WeaponStatsData` _output_get)))
        (set `self.StyleModifer` _basedamage)
        (if (not (> (`self.DamageOutput`) 0.0))
          (set `self.DamageOutput` _totaldamage))
        (set `self.CriticalHitOutput` _criticalhitdamage)
        (`/Engine/EditorBlueprintResources/StandardMacros.IsValid` _weaponref
          (:`Is Valid`
            (set `self.WeaponOwner` (`HuntWeapon.WeaponOwner` _weaponref)))))))
  (if (`self.bIsHomingTarget?`)
    (bind _returnvalue_2 (`KismetSystemLibrary.K2_SetTimerDelegate` (`|CreateDelegate` :!event `FindHomingTarget`) (`self.HomingTimerRate`) true))
    (set `self.HomingTimer` _returnvalue_2)))

(event `self.SphereCollision.OnComponentHit`
  (params (HitComponent :type "PrimitiveComponent Object Reference") (OtherActor :type "Actor Object Reference") (OtherComp :type "PrimitiveComponent Object Reference") (NormalImpulse :type "Vector Structure") (Hit :type "HitResult Structure (by ref)"))
  (if (`self.bFromWeapon`)
    (if (!= OtherActor (`self.WeaponOwner`))
      (bind _output_get (set `self.ProjHit` Hit))
      (bind (_bblockinghit _binitialoverlap _time _distance _location _impactpoint _normal _impactnormal _physmat _hitactor _hitcomponent _hitbonename) (`GameplayStatics.BreakHitResult` _output_get))
      (if (!= _hitactor self)
        (bind _output_get_2 (set `self.HitActor` _hitactor))
        (`self.DealDamage` _output_get_2 _hitbonename)
        (`|ExecutionSequence`
          (:`then_1`
            (if (`self.bShouldDestroyOnContact?`)
              (`self.K2_DestroyActor`)))
          (:`then_2`
            (if (`self.ActorHasTag` _hitactor "Door")
              (bind _asbp_door_base (cast `/Game/Dynamic/Blueprints/Interactables/Doors/BP_DoorBase` _hitactor :!pure true))
              (if (`/Game/Dynamic/Blueprints/Interactables/Doors/BP_DoorBase.bShouldOpenDoor?` _asbp_door_base)
                (`self.K2_DestroyActor` :!label _label)
                (else
                  (`/Engine/EditorBlueprintResources/StandardMacros.IsValid` self
                    (:`Is Valid`
                      (if (`/Game/Dynamic/Blueprints/Interactables/Doors/BP_DoorBase.bDoOverlapCheck` _asbp_door_base)
                        (`self.K2_DestroyActor`)
                        (else
                          (message `HuntPlayerInterface.OnDoorOpenRefuse` (`GameplayStatics.GetPlayerController` 0))
                          (set `ProjectileMovementComponent.bShouldBounce` true (`self.ProjectileMovementComponent`))))))))
              (else
                (goto _label)))))))))

(event `self.ReceiveEndPlay`
  (params (EndPlayReason :type "EEndPlayReason Enum" :default "Destroyed"))
  (switch `EEndPlayReason` EndPlayReason
    (:`Destroyed`
      (`GameplayStatics.SpawnEmitterAtLocation` (`self.DestroyVFX`) (`self.K2_GetActorLocation`) (struct) (0.75 0.75 0.75))
      (`GameplayStatics.PlaySoundAtLocation` (`self.DestroySFX`) (`self.K2_GetActorLocation`) (struct) 1.0 1.0 0.0 null null null)
      (`KismetSystemLibrary.K2_ClearAndInvalidateTimerHandle` (`self.HomingTimer`)))))

(event `self.ReceiveAnyDamage`
  (params (Damage :type "Float (single-precision)") (DamageType :type "DamageType Object Reference") (InstigatedBy :type "Controller Object Reference") (DamageCauser :type "Actor Object Reference"))
  (bind _returnvalue (`self.K2_GetActorLocation`))
  (bind _returnvalue_2 (`self.K2_GetActorRotation`))
  (if (`self.FromAI?`)
    (if (== InstigatedBy (`GameplayStatics.GetPlayerController` 0))
      (if (`KismetMathLibrary.RandomBool`)
        (`|SpawnActorFromClass` "/Game/Dynamic/Blueprints/Interactables/Pickups/BP_HealthPickup_Medium.BP_HealthPickup_Medium_C" (`KismetMathLibrary.MakeTransform` _returnvalue _returnvalue_2) "Undefined" "OverrideRootScale" null null)
        (else
          (`|SpawnActorFromClass` "/Game/Dynamic/Blueprints/Interactables/Pickups/BP_MissilePickupBase_Low.BP_MissilePickupBase_Low_C" (`KismetMathLibrary.MakeTransform` _returnvalue _returnvalue_2) "Undefined" "OverrideRootScale" null null))))))

(event `self.ReceiveTick`
  (params (DeltaSeconds :type "Float (single-precision)"))
  (`self.FindHomingTarget`))

(fn `DealDamage`
  (params (DamagedActor :type "Actor Object Reference") (HitBoneName :type Name))
  (bind _returnvalue (`GameplayStatics.GetPlayerCharacter` 0))
  (bind _returnvalue_2 (`GameplayStatics.GetGameMode`))
  (bind _returnvalue_3 (`self.GetOwner`))
  (bind _asproject_hunt_character (cast `ProjectHuntCharacter` DamagedActor :!pure true))
  (bind _projhit (`self.ProjHit`))
  (bind _weaponowner (`self.WeaponOwner`))
  (`/Engine/EditorBlueprintResources/StandardMacros.IsValid` DamagedActor
    (:`Is Valid`
      (`/Engine/EditorBlueprintResources/StandardMacros.IsValid` (`self.GetComponentByClass` DamagedActor "/Script/ProjectHunt.HuntStatsComponent")
        (:`Is Valid`
          (if (== DamagedActor _asproject_hunt_character)
            (if (!= DamagedActor (`GameplayStatics.GetPlayerCharacter` 0))
              (for _array_element (`ProjectHuntCharacter.CriticalHitLocations` _asproject_hunt_character)
                (if (== _array_element HitBoneName)
                  (`GameplayStatics.ApplyPointDamage` DamagedActor (`self.CriticalHitOutput`) (`.ImpactPoint` (`GameplayStatics.BreakHitResult` _projhit)) _projhit (`self.GetInstigatorController`) self)
                  (else
                    (bind _returnvalue_4 (`GameplayStatics.ApplyDamage` DamagedActor (`self.DamageOutput`) (`self.GetInstigatorController`) _returnvalue_3 :!label _label))
                    (if (or (`self.ActorHasTag` DamagedActor (`self.ProjectileTargetTag`)) (`self.ActorHasTag` DamagedActor "Hazard"))
                      (`/Engine/EditorBlueprintResources/StandardMacros.IsValid` _weaponowner
                        (:`Is Valid`
                          (if (== _weaponowner _returnvalue)
                            (message `HuntPlayerInterface.OnModifyStyle` _returnvalue (`self.StyleModifer`))
                            (message `HuntDifficultyInterface.PlayerDealtDamage` _returnvalue_2 (* (/ _returnvalue_4 (`self.DamageOutput`)) 80.0))
                            (else
                              (message `HuntDifficultyInterface.PlayerReceivedDamage` _returnvalue_2 (* (/ _returnvalue_4 (`self.DamageOutput`)) 60.0)))))
                        (:`Is Not Valid`
                          _)))
                    (`self.K2_DestroyActor`)
                    (return))))
              (else
                (goto _label)))
            (else
              (goto _label))))
        (:`Is Not Valid`
          (`GameplayStatics.ApplyDamage` DamagedActor 1.0 (`GameplayStatics.GetPlayerController` 0) _returnvalue_3)
          (set `ProjectileMovementComponent.bShouldBounce` true (`self.ProjectileMovementComponent`))
          (`self.SetLifeSpan` 0.5))))))

(fn `FindHomingTarget`
  (bind _spherecollision (`self.SphereCollision`))
  (bind _returnvalue (`SceneComponent.K2_GetComponentLocation` _spherecollision))
  (bind _outhit (`KismetSystemLibrary.SphereTraceSingleForObjects` :`Start` _returnvalue :`End` (+ _returnvalue (* (`KismetMathLibrary.GetForwardVector` (`SceneComponent.K2_GetComponentRotation` _spherecollision)) 400.0)) :`Radius` (`self.HomingSearchRadius`) :`ObjectTypes` (`self.HomingTargetsArray`) :`bTraceComplex` true :`DrawDebugType` "ForOneFrame" :`TraceColor` (struct :`G` 0.01 :`B` 1.0 :`A` 1.0) :`TraceHitColor` (struct :`R` 1.0 :`G` 0.470967 :`A` 1.0)))
  (bind (_bblockinghit _binitialoverlap _time _distance _location _impactpoint _normal _impactnormal _physmat _hitactor) (`GameplayStatics.BreakHitResult` _outhit))
  (if _bblockinghit
    (`/Engine/EditorBlueprintResources/StandardMacros.IsValid` _hitactor
      (:`Is Valid`
        (`self.K2_SetActorLocation` (`KismetMathLibrary.VInterpTo` (`self.K2_GetActorLocation`) _impactpoint (`GameplayStatics.GetWorldDeltaSeconds`) 10.0) true)))))

(fn `OnActivateWeaponEffect`
  (params (bLooping :type Boolean))
  (bind _returnvalue (`KismetSystemLibrary.K2_SetTimerDelegate` (`|CreateDelegate` :!event `StartWeaponEffect`) (`self.WeaponEffectTimeLimit`) bLooping))
  (set `self.WeaponEffectTimer` _returnvalue))

(fn `RevertEffect`)

(fn `StartWeaponEffect`)

(fn `UserConstructionScript`)