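; Chrono player projectile for ProjectHunt that slows actors through CustomTimeDilation.
; BeginPlay starts a fast looping timer, while SlowDownTarget sphere-traces from the projectile toward a forward vector not offset by its location, with debug drawing.
; Blocking hits are slowed to quarter speed, as are hit ProjectHuntCharacters' current weapons.
; Hit damage and speed restoration are disconnected, so the slow never reverts here.
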(event `self.ReceiveBeginPlay`
  (`parent.ReceiveBeginPlay`)
  (bind _returnvalue (`KismetSystemLibrary.K2_SetTimerDelegate` (`|CreateDelegate` :!event `SlowDownTarget`) 0.1 true))
  (set `self.ChronoTimer` _returnvalue))

(event `self.SphereCollision.OnComponentHit`
  (params (HitComponent :type "PrimitiveComponent Object Reference") (OtherActor :type "Actor Object Reference") (OtherComp :type "PrimitiveComponent Object Reference") (NormalImpulse :type "Vector Structure") (Hit :type "HitResult Structure (by ref)")))

(fn `SlowDownTarget`
  (bind _returnvalue (`KismetMathLibrary.GetForwardVector` (`self.K2_GetActorRotation`)))
  (bind _outhits (`KismetSystemLibrary.SphereTraceMultiForObjects` :`Start` (`self.K2_GetActorLocation`) :`End` (+ (* _returnvalue 300.0) (* _returnvalue 1000.0)) :`Radius` 400.0 :`ObjectTypes` (`self.TraceObjectsArray`) :`DrawDebugType` "ForDuration"))
  (for _array_element _outhits
    (bind (_bblockinghit _binitialoverlap _time _distance _location _impactpoint _normal _impactnormal _physmat _hitactor) (`GameplayStatics.BreakHitResult` _array_element))
    (if _bblockinghit
      (set `Actor.CustomTimeDilation` 0.25 _hitactor)
      (bind _asproject_hunt_character (cast `ProjectHuntCharacter` _hitactor :!pure true))
      (if (== _hitactor _asproject_hunt_character)
        (set `Actor.CustomTimeDilation` 0.25 (`ProjectHuntCharacter.GetCurrentWeapon` _asproject_hunt_character))))))

(fn `UserConstructionScript`
  (`parent.UserConstructionScript`))