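; Player grenade projectile that bounces with a sound and deals radial falloff damage, sparing the player.
; Sphere hits on anything but the player trigger Explode, immediately for contact grenades or after a delay otherwise.
; Explode draws debug spheres, but only awards a style modifier and destroys the actor if damage was applied.
; Explosion VFX and sound spawn from the Destroyed event.
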(event `self.ReceiveBeginPlay`
  (`parent.ReceiveBeginPlay`))

(event `Explode`
  (params (`ExplodeImmediately?` :type Boolean))
  (bind _returnvalue (`self.K2_GetActorLocation`))
  (if (not `ExplodeImmediately?`)
    (`KismetSystemLibrary.Delay` 5.0))
  (bind _returnvalue_2 (`GameplayStatics.ApplyRadialDamageWithFalloff` 20.0 5.0 _returnvalue 250.0 600.0 1.0 (`self.DamageTypeClass`) (`|MakeArray` (`GameplayStatics.GetPlayerPawn` 0) :!type "Actor Object Reference") self (`GameplayStatics.GetPlayerController` 0) "ECC_GameTraceChannel4"))
  (`KismetSystemLibrary.DrawDebugSphere` _returnvalue 250.0 12 (struct :`G` 1.0 :`B` 0.045588 :`A` 1.0) 10.0)
  (`KismetSystemLibrary.DrawDebugSphere` _returnvalue 500.0 12 (struct :`R` 1.0 :`A` 1.0) 10.0)
  (if _returnvalue_2
    (message `HuntPlayerInterface.OnModifyStyle` (`GameplayStatics.GetPlayerCharacter` 0) (`self.StyleModifer`))
    (`self.K2_DestroyActor`)))

(event `self.StaticMesh.OnComponentHit`
  (params (HitComponent :type "PrimitiveComponent Object Reference") (OtherActor :type "Actor Object Reference") (OtherComp :type "PrimitiveComponent Object Reference") (NormalImpulse :type "Vector Structure") (Hit :type "HitResult Structure (by ref)"))
  (`|ExecutionSequence`
    (:`then_0`
      (if (!= OtherActor (`self.WeaponOwner`))
        (bind _output_get (set `self.ProjHit` Hit))))))

(event `self.SphereCollision.OnComponentHit`
  (params (HitComponent :type "PrimitiveComponent Object Reference") (OtherActor :type "Actor Object Reference") (OtherComp :type "PrimitiveComponent Object Reference") (NormalImpulse :type "Vector Structure") (Hit :type "HitResult Structure (by ref)"))
  (bind (_bblockinghit _binitialoverlap _time _distance _location _impactpoint _normal _impactnormal _physmat _hitactor) (`GameplayStatics.BreakHitResult` Hit))
  (`GameplayStatics.PlaySoundAtLocation` "/Game/Static/SciFiWeapDark/Sound/GrenadeLauncher/GrenadeLauncher_Bounce_Cue.GrenadeLauncher_Bounce_Cue" _impactpoint (struct) 1.0 1.0 0.0 null null null)
  (if (!= _hitactor (`GameplayStatics.GetPlayerPawn` 0))
    (`self.Explode` (`self.bIsContactGrenade?`))))

(event `self.ReceiveDestroyed`
  (`self.SpawnExplosionFeedback`))

(fn `SpawnExplosionFeedback`
  (bind _returnvalue (`self.K2_GetActorLocation`))
  (`GameplayStatics.SpawnEmitterAtLocation` (`self.ExplosionVFX`) _returnvalue (`self.K2_GetActorRotation`))
  (`GameplayStatics.PlaySoundAtLocation` (`self.ExplosionSFX`) _returnvalue (struct) 1.0 1.0 0.0 null null null))

(fn `UserConstructionScript`
  (`parent.UserConstructionScript`))