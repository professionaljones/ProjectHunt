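; BP_RifleChargeProjectile is a player rifle charge-shot projectile that moves with a wobble.
; After parent Tick, it sweeps its relative location forward along X at fixed speed from its world location.
; A time-based sine drives a lerp that oscillates Y and Z around zero, ignoring their current values and the projectile's facing.
; Disconnected ProjectileMovementComponent velocity experiments remain in the graph and never run.
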(event `self.ReceiveTick`
  (params (DeltaSeconds :type "Float (single-precision)"))
  (bind _returnvalue_x (`KismetMathLibrary.BreakVector` (`self.K2_GetActorLocation`)))
  (bind _returnvalue (+ _returnvalue_x (* DeltaSeconds 3000.0)))
  (`parent.ReceiveTick` DeltaSeconds)
  (`self.K2_SetActorRelativeLocation` (`KismetMathLibrary.VLerp` (`KismetMathLibrary.MakeVector` _returnvalue 1.0 2.0) (`KismetMathLibrary.MakeVector` _returnvalue -1.0 -2.0) (* (`KismetMathLibrary.Sin` (`GameplayStatics.GetTimeSeconds`)) 50.0)) true))

(fn `UserConstructionScript`
  (`parent.UserConstructionScript`))