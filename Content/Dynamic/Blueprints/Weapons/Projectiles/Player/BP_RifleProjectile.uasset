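; BP_RifleProjectile is the player's rifle projectile, a child Blueprint that adds little logic of its own.
; On BeginPlay it runs the parent's logic and starts a timeline, with no timeline output logic shown in this graph.
; StartWeaponEffect is empty, and a disconnected branch that would apply damage to a valid hit actor never runs.
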(event `self.ReceiveBeginPlay`
  (`parent.ReceiveBeginPlay`)
  (`TimelineComponent.PlayFromStart` (`self.Timeline_0`)))

(event `self.StartWeaponEffect`)

(fn `UserConstructionScript`
  (`parent.UserConstructionScript`))