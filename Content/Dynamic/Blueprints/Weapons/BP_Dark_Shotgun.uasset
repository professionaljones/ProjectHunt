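; BP_Dark_Shotgun is a weapon Blueprint that fires two projectiles at once, one from each of its left and right charge points.
; On weapon fire, it looks up the projectile class for the current projectile state in the WeaponProjectiles map.
; It spawns both at half scale along the owner's control rotation, passing in the weapon's total damage.
; The parent fire logic runs afterward, only when a matching projectile class is found.
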(event `self.ReceiveBeginPlay`
  (`parent.ReceiveBeginPlay`))

(event `self.OnWeaponFire`
  (bind (_value _returnvalue) (`BlueprintMapLibrary.Map_Find` (`self.WeaponProjectiles`) (`self.WeaponProjectileState`)))
  (if _returnvalue
    (`|ExecutionSequence`
      (:`then_0`
        (`|SpawnActorFromClass` _value (`KismetMathLibrary.MakeTransform` (`SceneComponent.K2_GetComponentLocation` (`self.ChargePointL`)) (`Pawn.GetControlRotation` (`self.WeaponOwner`)) (0.5 0.5 0.5)) "Undefined" "OverrideRootScale" self (`.TotalDamage` (break `WeaponStatsData` (`self.WeaponStatsData`))) null))
      (:`then_1`
        (`|SpawnActorFromClass` _value (`KismetMathLibrary.MakeTransform` (`SceneComponent.K2_GetComponentLocation` (`self.ChargePointR`)) (`Pawn.GetControlRotation` (`self.WeaponOwner`)) (0.5 0.5 0.5)) "Undefined" "OverrideRootScale" self (`.TotalDamage` (break `WeaponStatsData` (`self.WeaponStatsData`))) null))
      (:`then_2`
        (`parent.OnWeaponFire`)))))

(fn `UserConstructionScript`
  (`parent.UserConstructionScript`))