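; Gameplay player controller that manages the HUD, pause menu, character journal, door-refusal message and player-death UI cleanup.
; Menus toggle game pause, input mode and HUD visibility.
; Holding the weapon wheel input opens a radial menu, locks look input, toggles a character effect and plays a timeline for time dilation and audio modulation.
; Startup uses level names to skip the main-menu HUD and show arena score, adding touch controls off desktop.
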(event `self.ReceiveBeginPlay`
  (`parent.ReceiveBeginPlay`)
  (`self.Init GUI`))

(event `HuntPlayerInterface.OnDoorOpenRefuse`
  (bind _gameplaymessagewbp (`self.GameplayMessageWBP`))
  (`/Engine/EditorBlueprintResources/StandardMacros.IsValid` _gameplaymessagewbp
    (:`Is Valid`
      (`Widget.RemoveFromParent` _gameplaymessagewbp)
      (set `self.GameplayMessageWBP` null))
    (:`Is Not Valid`
      _))
  (bind _returnvalue (`|CreateWidget` :`Class` "/Game/Dynamic/UI/Gameplay/WBP_GameplayMessage.WBP_GameplayMessage_C" :`OwningPlayer` (`GameplayStatics.GetPlayerController` 0) :`IconImage` null))
  (set `self.GameplayMessageWBP` _returnvalue)
  (`UserWidget.AddToViewport` _returnvalue 0)
  (`GameplayStatics.PlaySound2D` "/Game/Static/Audio/SFX/PM_CS_beep_denied5.PM_CS_beep_denied5" 1.0 1.0 0.0 null null)
  (`KismetSystemLibrary.Delay` 5.0)
  (`Widget.RemoveFromParent` _returnvalue))

(event `InputAction|WeaponWheel`
  (params (Key :type "Key Structure"))
  (bind _returnvalue (`GameplayStatics.GetPlayerController` 0))
  (bind _radialmenudilationtimeline (`self.RadialMenuDilationTimeline`))
  (bind _chamreference (`/Game/Dynamic/Blueprints/Player/BP_TrishPlayerCharacter.ChamReference` (cast `/Game/Dynamic/Blueprints/Player/BP_TrishPlayerCharacter` (`|ConvertAsset` (`self.PCRef`)) :!pure true)))
  (:`Pressed`
    (`TimelineComponent.PlayFromStart` _radialmenudilationtimeline)
    (bind _returnvalue_2 (`|CreateWidget` "/Game/Dynamic/UI/Gameplay/WBP_WeaponWheel.WBP_WeaponWheel_C"))
    (`UserWidget.AddToViewport` _returnvalue_2 0)
    (bind _output_get (set `self.RadialMenuWBP` _returnvalue_2))
    (`WidgetBlueprintLibrary.SetInputMode_GameAndUIEx` _returnvalue _output_get "LockAlways")
    (`self.SetIgnoreLookInput` _returnvalue true)
    (`/Game/Chameleon/BP_HuntChameleon.ToggleRadialMenuEffect` _chamreference true))
  (:`Released`
    (`TimelineComponent.ReverseFromEnd` _radialmenudilationtimeline)
    (`Widget.RemoveFromParent` (`self.RadialMenuWBP`))
    (set `self.RadialMenuWBP` null)
    (`WidgetBlueprintLibrary.SetInputMode_GameOnly` _returnvalue)
    (`self.ResetIgnoreLookInput` _returnvalue)
    (`/Game/Chameleon/BP_HuntChameleon.ToggleRadialMenuEffect` _chamreference false)))

(event `InputAction|Pause` :paused true
  (params (Key :type "Key Structure"))
  (:`Pressed`
    (`HuntPlayerInterface.TogglePauseMenu`)))

(event `InputAction|CharacterMenu` :paused true
  (params (Key :type "Key Structure"))
  (:`Pressed`
    (`self.ToggleChar`)))

(event `HuntPlayerInterface.TogglePauseMenu`
  (`self.TogglePause`)
  (`KismetSystemLibrary.Delay` 0.2))

(event `HuntPlayerInterface.OnReturnToGame`
  (bind _currentdialoguewidget (`self.CurrentDialogueWidget`))
  (`self.ReturnToGame`)
  (if (and (`KismetSystemLibrary.IsValid` _currentdialoguewidget) (`Widget.IsInViewport` _currentdialoguewidget))
    (set `self.bShowMouseCursor` true)))

(event `HuntPlayerInterface.OnPlayerDeath`
  (`parent.OnPlayerDeath`)
  (`Widget.RemoveFromParent` (`self.GameplayWBP`))
  (`Widget.RemoveFromParent` (`self.CharMenuWBP`)))

(fn `GetJoystickDirection`
  (params (Stick :type "/Game/GenericRadialMenus/UMG/EJoystickTypes Enum" :default "NewEnumerator0"))
  (returns (StickInput :type "Vector2D Structure"))
  (bind _stickinput (`parent.GetJoystickDirection` Stick))
  (return _stickinput))

(fn `Init GUI`
  (`WidgetBlueprintLibrary.SetInputMode_GameOnly` (`GameplayStatics.GetPlayerController` 0))
  (`|ExecutionSequence`
    (:`then_0`
      (bind _returnvalue (`GameplayStatics.GetCurrentLevelName` true))
      (if (`KismetStringLibrary.NotEqual_StrStr` _returnvalue "LM_MainMenu")
        (`UserWidget.AddToViewport` (`self.GameplayWBP`) 0)))
    (:`then_1`
      (set `self.PCRef` (`|ConvertAsset` (cast `HuntPlayerCharacter` (`GameplayStatics.GetPlayerCharacter` 0) :!pure true)))
      (if (not (`/Game/Dynamic/Blueprints/Game/BPFL_SystemStats.IsRunningOnDesktop`))
        (`self.ActivateTouchInterface` "/Game/Dynamic/TI_DefaultPreset.TI_DefaultPreset")))
    (:`then_2`
      (`self.IsThisArenaMode?`))))

(fn `IsThisArenaMode?`
  (bind _gameplaywbp (`self.GameplayWBP`))
  (bind _returnvalue (`GameplayStatics.GetCurrentLevelName` true))
  (if (`KismetStringLibrary.StartsWith` _returnvalue "LA_")
    (set `/Game/Dynamic/UI/Gameplay/WBP_GameplayHUD.bIsScoreVisible?` true _gameplaywbp)
    (else
      (set `/Game/Dynamic/UI/Gameplay/WBP_GameplayHUD.bIsScoreVisible?` false _gameplaywbp))))

(fn `ReturnToGame`
  (`self.ToggleHUDVisibility` true))

(fn `ToggleChar`
  (bind _charmenuwbp (`self.CharMenuWBP`))
  (`/Engine/EditorBlueprintResources/StandardMacros.IsValid` (`self.CharMenuWBP`)
    (:`Is Valid`
      (`self.ReturnToGame` :!label _label)
      (`UINavWidget.ReturnToParent` _charmenuwbp false 0)
      (set `self.CharMenuWBP` null))
    (:`Is Not Valid`
      (bind _returnvalue (`|CreateWidget` "/Game/Dynamic/UI/CharacterMenu/WBP_CharJournal.WBP_CharJournal_C" null (`self.GameplayWBP`)))
      (set `self.CharMenuWBP` _returnvalue)
      (if (`GameplayStatics.IsGamePaused`)
        (goto _label)
        (else
          (`WidgetBlueprintLibrary.SetInputMode_GameAndUIEx` (`GameplayStatics.GetPlayerController` 0) null "DoNotLock" false)
          (set `self.bShowMouseCursor` true)
          (`UserWidget.AddToViewport` _charmenuwbp 0)
          (`GameplayStatics.SetGamePaused` true)
          (`Widget.SetVisibility` (`self.GameplayWBP`) "Hidden"))))))

(fn `TogglePause`
  (`/Engine/EditorBlueprintResources/StandardMacros.IsValid` (`self.PauseMenuWBP`)
    (:`Is Valid`
      (`self.ReturnToGame`)
      (`UINavWidget.ReturnToParent` (`self.PauseMenuWBP`) false 0)
      (set `self.PauseMenuWBP` null))
    (:`Is Not Valid`
      (`WidgetBlueprintLibrary.SetInputMode_GameAndUIEx` (`GameplayStatics.GetPlayerController` 0) null "DoNotLock" false)
      (`GameplayStatics.SetGamePaused` true)
      (set `self.bShowMouseCursor` true)
      (bind _returnvalue (`|CreateWidget` "/Game/Dynamic/UI/Gameplay/WBP_PauseMenu_Updated.WBP_PauseMenu_Updated_C" (`GameplayStatics.GetPlayerController` 0) null))
      (set `self.PauseMenuWBP` _returnvalue)
      (`UserWidget.AddToViewport` _returnvalue 0)
      (`Widget.SetVisibility` (`self.GameplayWBP`) "Hidden"))))

(fn `UserConstructionScript`)