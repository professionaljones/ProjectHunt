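; Base player controller for Project Hunt that handles menu input, a console window and the game-over screen.
; BeginPlay pre-creates console, options and game-over widgets; Tilde or Touch 4 toggles the console, freezing play through zero time dilation, while player death pauses and shows game over.
; While paused, UI Back and Accept act on the last widget, and numpad keys drive GameInstance replay recording and playback.
; Input-type and stage-ID getters return fixed defaults.
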(event `InputAction|UI_Back` :consume false :paused true :overrideparent false
  (params (Key :type "Key Structure"))
  (:`Pressed`
    (if (`GameplayStatics.IsGamePaused`)
      (`/Game/Dynamic/Blueprints/Player/BPI_PlayerUserInterface.OnReturnToPreviousMenu` (`self.LastWBP`)))))

(event `InputAction|UI_Accept` :consume false :paused true :overrideparent false
  (params (Key :type "Key Structure"))
  (:`Pressed`
    (if (`GameplayStatics.IsGamePaused`)
      (message `/Game/Dynamic/Blueprints/Player/BPI_PlayerUserInterface.OnUIAccept` (`self.LastWBP`)))))

(event `Key|NumPadZero`
  (params (Key :type "Key Structure"))
  (:`Pressed`
    (`ProjectHuntGameInstance.StartRecording` (cast `/Game/Dynamic/Blueprints/Game/BP_ProjectHuntGameInstance` (`GameplayStatics.GetGameInstance`) :!pure true))))

(event `Key|NumPadOne`
  (params (Key :type "Key Structure"))
  (:`Pressed`
    (`ProjectHuntGameInstance.StopRecording` (cast `/Game/Dynamic/Blueprints/Game/BP_ProjectHuntGameInstance` (`GameplayStatics.GetGameInstance`) :!pure true))))

(event `Key|NumPadThree`
  (params (Key :type "Key Structure"))
  (:`Pressed`
    (`ProjectHuntGameInstance.StartReplay` (cast `/Game/Dynamic/Blueprints/Game/BP_ProjectHuntGameInstance` (`GameplayStatics.GetGameInstance`) :!pure true))))

(event `self.ReceiveBeginPlay`
  (`parent.ReceiveBeginPlay`)
  (bind _returnvalue (`|CreateWidget` "/Game/Dynamic/UI/WBP_ConsoleWindow.WBP_ConsoleWindow_C" self))
  (set `self.ConsoleWBP` _returnvalue)
  (bind _returnvalue_2 (`|CreateWidget` "/Game/Dynamic/UI/Options/WBP_OptionsMenu.WBP_OptionsMenu_C" self))
  (set `self.OptionsWBP` _returnvalue_2)
  (bind _returnvalue_3 (`|CreateWidget` "/Game/Dynamic/UI/WBP_GameOver.WBP_GameOver_C" self))
  (set `self.GameOverWBP` _returnvalue_3))

(event `Key|Tilde` :paused true
  (params (Key :type "Key Structure"))
  (bind _consolewbp (`self.ConsoleWBP`))
  (:`Pressed`
    (if (`self.ConsoleVisible?`) :!label _label
      (`Widget.RemoveFromParent` _consolewbp)
      (set `self.bShowMouseCursor` false)
      (`GameplayStatics.SetGlobalTimeDilation` 1.0)
      (`WidgetBlueprintLibrary.SetInputMode_GameOnly` self)
      (set `self.ConsoleVisible?` false)
      (else
        (`UserWidget.AddToViewport` _consolewbp 0)
        (set `self.bShowMouseCursor` true)
        (`GameplayStatics.SetGlobalTimeDilation` 0.0)
        (`WidgetBlueprintLibrary.SetInputMode_GameAndUIEx` self _consolewbp "DoNotLock" false)
        (set `self.ConsoleVisible?` true)))))

(event `Key|Touch4`
  (params (Key :type "Key Structure"))
  (:`Pressed`
    (goto _label)))

(event `HuntPlayerInterface.OnPlayerDeath`
  (`self.DisableGameplayInput` true true)
  (`UserWidget.AddToViewport` (`self.GameOverWBP`) 0))

(event `/Game/Dynamic/Blueprints/Player/BPI_PlayerUserInterface.OnReturnToPreviousMenu`
  (params (ExitingWidget :type "UserWidget Object Reference"))
  (`/Engine/EditorBlueprintResources/StandardMacros.IsValid` ExitingWidget
    (:`Is Valid`
      (if (!= ExitingWidget (`/Game/Dynamic/UI/BP_ProjectHuntHUD_Base.MainMenuWBP` (cast `/Game/Dynamic/UI/BP_ProjectHuntHUD_Base` (`self.GetHUD`) :!pure true)))
        (`Widget.RemoveFromParent` ExitingWidget)))))

(fn `DisableGameplayInput`
  (params (bShowMouseCursor :type Boolean) (bPaused :type Boolean))
  (`WidgetBlueprintLibrary.SetInputMode_GameAndUIEx` (`GameplayStatics.GetPlayerController` 0) null "DoNotLock" false)
  (set `self.bShowMouseCursor` bShowMouseCursor)
  (`GameplayStatics.SetGamePaused` bPaused))

(fn `GetCurrentInputType`
  (returns (InputType :type "/Game/FILab/MTS/EInputType Enum"))
  (return "NewEnumerator0"))

(fn `GetCurrentStageID`
  (returns (CurrentStage :type Name))
  (return "None"))

(fn `UserConstructionScript`)