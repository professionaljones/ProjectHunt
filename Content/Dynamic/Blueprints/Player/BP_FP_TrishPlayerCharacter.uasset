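; First-person player character for Trish, with wall running, limited jumps and dashes, and a two-weapon inventory.
; Capsule hits start wall runs that disable gravity, tilt the camera and re-trace the wall through a timeline, ending on jump or lost contact or input.
; Landing refills jumps and dashes; Tick clamps airborne horizontal speed and blocks damage while dashing.
; BeginPlay spawns hidden weapons for equipping by key; debug keys trigger save, load and self-damage.
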(event `Key|Gamepad_DPad_Left`
  (params (Key :type "Key Structure"))
  (:`Pressed`
    (`self.EquipWeapon` 1)))

(event `Key|Gamepad_DPad_Right`
  (params (Key :type "Key Structure"))
  (:`Pressed`
    (`self.EquipWeapon` 2)))

(event `Key|One`
  (params (Key :type "Key Structure"))
  (:`Pressed`
    (`self.EquipWeapon` 1)))

(event `Key|Two`
  (params (Key :type "Key Structure"))
  (:`Pressed`
    (`self.EquipWeapon` 2)))

(event `self.ReceiveBeginPlay`
  (bind _mesh1p (`self.Mesh1P`))
  (set `CharacterMovementComponent.MaxWalkSpeed` (`self.WalkSpeed`) (`self.CharacterMovement`))
  (`self.ResetJump` (`self.MaxJumps`))
  (`MovementComponent.SetPlaneConstraintEnabled` (`self.CharacterMovement`) true)
  (`self.ResetDash` (`self.DashLimit`))
  (bind _returnvalue (`PrimitiveComponent.CreateDynamicMaterialInstance` _mesh1p 0 (`PrimitiveComponent.GetMaterial` _mesh1p 0) "None"))
  (set `self.Mesh1P_DynMat` _returnvalue)
  (`TimelineComponent.PlayFromStart` (`self.CharSpawnTimeline`))
  (`GameplayStatics.PlaySound2D` "/Game/Static/Audio/SFX/Sci-fi_Teleport.Sci-fi_Teleport" 1.0 1.0 0.0 null null)
  (`self.SpawnWeapon` "/Game/Dynamic/Blueprints/Weapons/BP_DarkPistol.BP_DarkPistol_C" 1)
  (`self.SpawnWeapon` "/Game/Dynamic/Blueprints/Weapons/BP_Dark_Rifle.BP_Dark_Rifle_C" 2))

(event `InputAction|Dash`
  (params (Key :type "Key Structure"))
  (bind (_returnvalue_x _returnvalue_y) (`KismetMathLibrary.BreakVector` (`self.GetVelocity`)))
  (:`Pressed`
    (`self.ConsumeDash`
      (:`Consumed`
        (`CharacterMovementComponent.AddImpulse` (`self.CharacterMovement`) (* (`KismetMathLibrary.MakeVector` _returnvalue_x _returnvalue_y) (`self.DashVelocityMod`)) true)
        (set `self.bIsDashing?` true))
      (:`NotConsumed`
        (set `self.bIsDashing?` false)))))

(event `InputAction|Jump`
  (params (Key :type "Key Structure"))
  (:`Pressed`
    (`self.ConsumeJump`
      (:`Consumed`
        (`self.LaunchCharacter` (`self.FindLaunchVelocity`) false true)
        (`self.IsPlayerOnWall`
          (:`true`
            (`self.OnWallRunEnd` "NewEnumerator1"))))))
  (:`Released`
    (`self.StopJumping`)))

(event `InputAxis|MoveForward` :overrideparent false
  (params (AxisValue :type "Float (single-precision)"))
  (set `self.ForwardAxis` AxisValue))

(event `InputAction|Pause`
  (params (Key :type "Key Structure")))

(event `self.OnLanded`
  (params (Hit :type "HitResult Structure (by ref)"))
  (`self.ResetJump` (`self.MaxJumps`))
  (`self.ResetDash` (`self.DashLimit`)))

(event `InputAxis|MoveRight` :overrideparent false
  (params (AxisValue :type "Float (single-precision)"))
  (set `self.RightAxis` AxisValue))

(event `ResetDash`
  (params (Dash :type Integer))
  (set `self.DashCount` (`KismetMathLibrary.Clamp` Dash 0 (`self.DashLimit`)))
  (if (`self.bIsDashing?`)
    (set `self.bIsDashing?` false)))

(event `ResetJump`
  (params (Jumps :type Integer))
  (set `self.JumpCount` (`KismetMathLibrary.Clamp` Jumps 0 (`self.MaxJumps`))))

(event `Key|NumPadFive`
  (params (Key :type "Key Structure"))
  (:`Pressed`
    (`/Game/Dynamic/Blueprints/Game/BP_ProjectHuntGameInstance.AsyncLoadSlot` (cast `/Game/Dynamic/Blueprints/Game/BP_ProjectHuntGameInstance` (`GameplayStatics.GetGameInstance`) :!pure true) "SaveSlot01")))

(event `Key|NumPadFour`
  (params (Key :type "Key Structure"))
  (:`Pressed`
    (`/Game/Dynamic/Blueprints/Game/BP_ProjectHuntGameInstance.AsyncSaveSlot` (cast `/Game/Dynamic/Blueprints/Game/BP_ProjectHuntGameInstance` (`GameplayStatics.GetGameInstance`) :!pure true) "SaveSlot01")))

(event `self.CapsuleComponent.OnComponentHit`
  (params (HitComponent :type "PrimitiveComponent Object Reference") (OtherActor :type "Actor Object Reference") (OtherComp :type "PrimitiveComponent Object Reference") (NormalImpulse :type "Vector Structure") (Hit :type "HitResult Structure (by ref)"))
  (bind (_direction _side) (`self.FindRunDirection` Hit_ImpactNormal))
  (`self.IsPlayerOnWall`
    (:`false`
      (if (`self.CanPlayerWallrun?` Hit_ImpactNormal)
        (if (`NavMovementComponent.IsFalling` (`self.CharacterMovement`))
          (set `self.WallrunDirection` _direction)
          (set `self.WallrunSide` _side)
          (if (`self.AreRequiredKeysDown`)
            (`self.OnWallRunStart`)
            (`KismetSystemLibrary.PrintString` "Mirror's Edge")
            (else
              (`self.OnWallRunEnd` "NewEnumerator0"))))))))

(event `self.ReceiveTick`
  (params (DeltaSeconds :type "Float (single-precision)"))
  (`self.ClampHorizontalVelocity`)
  (if (`self.bIsDashing?`)
    (set `self.bCanBeDamaged` false)
    (else
      (set `self.bCanBeDamaged` true))))

(event `OnWallRunStart`
  (bind _charactermovement (`self.CharacterMovement`))
  (set `CharacterMovementComponent.AirControl` 1.0 _charactermovement)
  (set `CharacterMovementComponent.GravityScale` 0.0 _charactermovement)
  (`MovementComponent.SetPlaneConstraintNormal` _charactermovement (0.0 0.0 1.0))
  (set `self.bIsWallrunning?` true)
  (`self.StartCameraTilt`)
  (`GameplayStatics.PlaySound2D` "/Game/Static/Audio/SFX/Player/Movement/PH_Wallrun_Start.PH_Wallrun_Start" 1.0 1.0 0.0 null null)
  (`Timeline|UpdateWallrunTimeline` :!label _label
    (:`Update`
      (`self.UpdateWallrun`))))

(event `OnWallRunEnd`
  (params (EndWallRunReason :type "/Game/Dynamic/Blueprints/Player/EWallrunEndReason Enum" :default "NewEnumerator0"))
  (bind _charactermovement (`self.CharacterMovement`))
  (`self.ResetJump` (select `/Game/Dynamic/Blueprints/Player/EWallrunEndReason` EndWallRunReason :`NewEnumerator0` 1 :`NewEnumerator1` (- (`self.MaxJumps`) 1)))
  (set `CharacterMovementComponent.AirControl` 0.05 _charactermovement)
  (set `CharacterMovementComponent.GravityScale` 1.0 _charactermovement)
  (`MovementComponent.SetPlaneConstraintNormal` _charactermovement (0.0 0.0 0.0))
  (set `self.bIsWallrunning?` false)
  (`self.EndCameraTilt`)
  (`GameplayStatics.PlaySound2D` "/Game/Static/Audio/SFX/Player/Movement/PH_Wallrun_End.PH_Wallrun_End" 1.0 1.0 0.0 null null)
  (goto _label :!via `Stop`))

(event `StartCameraTilt`
  (bind _returnvalue (`self.GetController`))
  (bind (_returnvalue_roll _returnvalue_pitch _returnvalue_yaw) (`KismetMathLibrary.BreakRotator` (`Controller.GetControlRotation` _returnvalue)))
  (bind (_direction _cameraroll) (`Timeline|CameraLean` :!via `PlayFromStart` :!label _label_2)
    (:`Update`
      (`Controller.SetControlRotation` _returnvalue (`KismetMathLibrary.MakeRotator` (* _cameraroll (select `/Game/Dynamic/Blueprints/Player/EWallrunSide` (`self.WallrunSide`) :`NewEnumerator0` -1.0 :`NewEnumerator1` 1.0 :!type "Float (single-precision)")) _returnvalue_pitch _returnvalue_yaw)))))

(event `Key|Divide`
  (params (Key :type "Key Structure"))
  (:`Pressed`
    (`GameplayStatics.ApplyDamage` self 10.0 null self)))

(event `EndCameraTilt`
  (goto _label_2 :!via `ReverseFromEnd`))

(fn `AreRequiredKeysDown`
  (returns (`ButtonPressed?` :type Boolean))
  (bind _rightaxis (`self.RightAxis`))
  (if (> (`self.ForwardAxis`) 0.1)
    (switch `/Game/Dynamic/Blueprints/Player/EWallrunSide` (`self.WallrunSide`)
      (:`NewEnumerator0`
        (return (> _rightaxis 0.1)))
      (:`NewEnumerator1`
        (return (> _rightaxis -0.1))))
    (else
      (return false))))

(fn `CanPlayerWallrun?`
  (params (SurfaceNormal :type "Vector Structure"))
  (returns (`CanWallrun?` :type Boolean))
  (if (< (.z SurfaceNormal) -0.05)
    (return false)
    (else
      (return (< (`KismetMathLibrary.DegAcos` (`KismetMathLibrary.Dot_VectorVector` (`KismetMathLibrary.Normal` (`KismetMathLibrary.MakeVector` (.x SurfaceNormal) (.y SurfaceNormal))) SurfaceNormal)) (`CharacterMovementComponent.K2_GetWalkableFloorAngle` (`self.CharacterMovement`)))))))

(fn `ClampHorizontalVelocity`
  (bind _charactermovement (`self.CharacterMovement`))
  (bind _returnvalue (/ (`KismetMathLibrary.VSize2D` (`self.GetHorizontalVelocity`)) (`MovementComponent.K2_GetModifiedMaxSpeed` _charactermovement)))
  ;[1 1 1] If we are falling...
  (if (`NavMovementComponent.IsFalling` _charactermovement)
    (if (> _returnvalue 1.0)
      (`self.SetHorizontalVelocity` (/ (`self.GetHorizontalVelocity`) _returnvalue)))))

(fn `EquipWeapon`
  (params (Key :type "Integer (by ref)"))
  (bind (_value _returnvalue) (`BlueprintMapLibrary.Map_Find` (`self.WeaponInventory`) Key))
  (if _returnvalue
    (`/Engine/EditorBlueprintResources/StandardMacros.IsValid` (`self.CurrentWeapon`)
      (:`Is Valid`
        (set `self.CurrentWeapon` null)
        (`self.SetActorHiddenInGame` _value false))
      (:`Is Not Valid`
        (`self.SetActorHiddenInGame` _value false)))
    (bind _output_get (set `self.CurrentWeapon` _value))
    (`self.K2_AttachToComponent` _output_get (`self.Mesh1P`) (`HuntWeapon.WeaponAttachPoint` _output_get) "KeepRelative" "KeepRelative" "KeepRelative" true)
    (`/Game/Dynamic/Blueprints/Weapons/BP_BaseWeapon.OnSpawn` (cast `/Game/Dynamic/Blueprints/Weapons/BP_BaseWeapon` _output_get :!pure true))))

(fn `FindDashVelocity`
  (returns (LaunchVelocity :type "Vector Structure"))
  (locals (DashDirection :type "Vector Structure"))
  (`|ExecutionSequence`
    (:`then_0`
      (if (`self.bIsWallrunning?`)
        (set `local.DashDirection` (`KismetMathLibrary.Cross_VectorVector` (`self.WallrunDirection`) (select `/Game/Dynamic/Blueprints/Player/EWallrunSide` (`self.WallrunSide`) :`NewEnumerator0` (0.0 0.0 1.0) :`NewEnumerator1` (0.0 0.0 -1.0) :!type "Vector Structure")))
        (else
          (set `local.DashDirection` (+ (* (`self.GetActorRightVector`) (`self.RightAxis`)) (* (`self.GetActorForwardVector`) (`self.ForwardAxis`)))))))
    (:`then_1`
      (return (* (+ (`local.DashDirection`) (1.0 0.0 0.0)) (`self.DashVelocityMod`))))))

(fn `FindLaunchVelocity`
  (returns (LaunchVelocity :type "Vector Structure"))
  (locals (LaunchDirection :type "Vector Structure"))
  (`|ExecutionSequence`
    (:`then_0`
      (if (`self.bIsWallrunning?`)
        (set `local.LaunchDirection` (`KismetMathLibrary.Cross_VectorVector` (`self.WallrunDirection`) (select `/Game/Dynamic/Blueprints/Player/EWallrunSide` (`self.WallrunSide`) :`NewEnumerator0` (0.0 0.0 1.0) :`NewEnumerator1` (0.0 0.0 -1.0) :!type "Vector Structure")))
        (elif (`NavMovementComponent.IsFalling` (`self.CharacterMovement`))
          (set `local.LaunchDirection` (+ (* (`self.GetActorRightVector`) (`self.RightAxis`)) (* (`self.GetActorForwardVector`) (`self.ForwardAxis`)))))))
    (:`then_1`
      (return (* (+ (`local.LaunchDirection`) (0.0 0.0 1.0)) (`CharacterMovementComponent.JumpZVelocity` (`self.CharacterMovement`)))))))

(fn `FindRunDirection`
  (params (WallNormal :type "Vector Structure"))
  (returns (Direction :type "Vector Structure") (Side :type "/Game/Dynamic/Blueprints/Player/EWallrunSide Enum"))
  (locals (WallSide :type "/Game/Dynamic/Blueprints/Player/EWallrunSide Enum"))
  (bind _output_get (set `local.WallSide` (select `bool` (> (`KismetMathLibrary.DotProduct2D` (`KismetMathLibrary.Conv_VectorToVector2D` WallNormal) (`KismetMathLibrary.Conv_VectorToVector2D` (`self.GetActorRightVector`))) 0.0) :`false` "NewEnumerator0" :`true` "NewEnumerator1" :!type "/Game/Dynamic/Blueprints/Player/EWallrunSide Enum")))
  (return (`KismetMathLibrary.Cross_VectorVector` (`local.WallNormal`) (select `/Game/Dynamic/Blueprints/Player/EWallrunSide` _output_get :`NewEnumerator0` (0.0 0.0 -1.0) :`NewEnumerator1` (0.0 0.0 1.0) :!type "Vector Structure")) _output_get))

(fn `GetHorizontalVelocity`
  (returns (ReturnValue :type "Vector2D Structure"))
  (return (`KismetMathLibrary.Conv_VectorToVector2D` (`MovementComponent.Velocity` (`self.CharacterMovement`)))))

(fn `ModifyWalkSpeed`
  (params (MaxWalkSpeed :type "Float (double-precision)"))
  (set `CharacterMovementComponent.MaxWalkSpeed` MaxWalkSpeed (`self.CharacterMovement`))
  (return))

(fn `SetHorizontalVelocity`
  (params (HorizontalVelocity :type "Vector2D Structure"))
  (bind _charactermovement (`self.CharacterMovement`))
  (bind (_velocity_x _velocity_y _velocity_z) (`KismetMathLibrary.BreakVector` (`MovementComponent.Velocity` _charactermovement)))
  (set `MovementComponent.Velocity` (`KismetMathLibrary.MakeVector` HorizontalVelocity_X HorizontalVelocity_Y _velocity_z) _charactermovement))

(fn `SpawnWeapon`
  (params (NewWeapon :type "/Game/Dynamic/Blueprints/Weapons/BP_BaseWeapon Class Reference") (Key :type "Integer (by ref)"))
  (bind _returnvalue (`|SpawnActorFromClass` NewWeapon (`KismetMathLibrary.MakeTransform` (0.0 0.0 0.0)) "Undefined" "OverrideRootScale" null null))
  (`self.SetActorHiddenInGame` _returnvalue true)
  (`BlueprintMapLibrary.Map_Add` (`self.WeaponInventory`) Key _returnvalue)
  (return))

(fn `UpdateWallrun`
  (bind _returnvalue (`self.K2_GetActorLocation`))
  (bind _charactermovement (`self.CharacterMovement`))
  (if (`self.AreRequiredKeysDown`)
    (bind (_outhit _returnvalue_2) (`KismetSystemLibrary.LineTraceSingle` _returnvalue (+ _returnvalue (* (`KismetMathLibrary.Cross_VectorVector` (`self.WallrunDirection`) (select `/Game/Dynamic/Blueprints/Player/EWallrunSide` (`self.WallrunSide`) :`NewEnumerator0` (0.0 0.0 -1.0) :`NewEnumerator1` (0.0 0.0 1.0) :!type "Vector Structure")) 600.0)) "TraceTypeQuery1"))
    (if _returnvalue_2
      (bind (_direction _side) (`self.FindRunDirection` (`.ImpactNormal` (`GameplayStatics.BreakHitResult` _outhit))))
      (if (== _side (`self.WallrunSide`))
        (bind _output_get (set `self.WallrunDirection` _direction))
        (bind (_returnvalue_x _returnvalue_y) (`KismetMathLibrary.BreakVector` (* _output_get (`MovementComponent.K2_GetModifiedMaxSpeed` _charactermovement))))
        (set `MovementComponent.Velocity` (`KismetMathLibrary.MakeVector` _returnvalue_x _returnvalue_y) _charactermovement)
        (else
          (`self.OnWallRunEnd` "NewEnumerator0")))
      (else
        (`self.OnWallRunEnd` "NewEnumerator0")))
    (else
      (`self.OnWallRunEnd` "NewEnumerator0"))))

(fn `UserConstructionScript`)