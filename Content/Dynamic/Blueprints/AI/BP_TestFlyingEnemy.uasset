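; Test flying enemy AI pawn that chases a blackboard-assigned target, damages it, and explodes when killed.
; BeginPlay registers it with the GameState and starts a looping timer, while Search moves it toward the EnemyActor blackboard value.
; On arrival, a line trace turns it toward any hit and damages HuntCharacterInterface actors.
; Damage drains HuntStats, with death triggering physics, radial impulse, sound and delayed destruction with an explosion emitter.
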(event `self.ReceiveBeginPlay`
  (bind _returnvalue (`KismetSystemLibrary.K2_SetTimerDelegate` (`|CreateDelegate` :!event `Search`) 0.5 true))
  (message `HuntGameInterface.AddEnemyToArray` (`GameplayStatics.GetGameState`) self))

(event `Search`
  (bind _returnvalue (`self.K2_GetActorLocation`))
  (bind _returnvalue_2 (`BlackboardComponent.GetValueAsObject` (`AIBlueprintHelperLibrary.GetBlackboard` self) "EnemyActor"))
  (bind _asactor (cast `Actor` _returnvalue_2 :!pure true))
  (`/Engine/EditorBlueprintResources/StandardMacros.IsValid` _returnvalue_2
    (:`Is Valid`
      (bind _movementresult (`|AIMoveTo` self (+ (`self.K2_GetActorLocation` _asactor) (0.0 250.0 0.0)) _asactor 500.0)
        (:`then`
          (switch `EPathFollowingResult` _movementresult))
        (:`OnSuccess`
          (bind _outhit (`KismetSystemLibrary.LineTraceSingleForObjects` :`Start` _returnvalue :`End` (* _returnvalue 200.0) :`ObjectTypes` (`|MakeArray` "ObjectTypeQuery9" :!type "EObjectTypeQuery Enum") :`bTraceComplex` true :`DrawDebugType` "ForOneFrame"))
          (bind (_bblockinghit _binitialoverlap _time _distance _location _impactpoint _normal _impactnormal _physmat _hitactor) (`GameplayStatics.BreakHitResult` _outhit))
          (if _bblockinghit
            (`self.K2_SetActorRotation` (`KismetMathLibrary.FindLookAtRotation` (`self.K2_GetActorLocation`) (`self.K2_GetActorLocation` _hitactor)))
            (if (`KismetSystemLibrary.DoesImplementInterface` _hitactor "/Script/ProjectHunt.HuntCharacterInterface")
              (`GameplayStatics.ApplyDamage` _hitactor 5.0))))))))

(event `self.ReceiveAnyDamage`
  (params (Damage :type "Float (single-precision)") (DamageType :type "DamageType Object Reference") (InstigatedBy :type "Controller Object Reference") (DamageCauser :type "Actor Object Reference"))
  (bind _huntstats (`self.HuntStats`))
  (`HuntStatsComponent.DamageHealth` _huntstats Damage)
  (if (<= (`HuntStatsComponent.GetCurrentHealth` _huntstats) 0.0)
    (`/Engine/EditorBlueprintResources/StandardMacros.DoOnce` false :!label _label
      (:`Completed`
        (`self.Explode`)))
    (else
      (goto _label :!via `Reset`))))

(event `Explode`
  (bind _radialforce (`self.RadialForce`))
  (set `self.bCanBeDamaged` false)
  (`PrimitiveComponent.SetSimulatePhysics` (`self.StaticMesh`) true)
  (`ActorComponent.Activate` _radialforce true)
  (`RadialForceComponent.FireImpulse` _radialforce)
  (`GameplayStatics.PlaySoundAtLocation` "/Game/Static/MobileStarterContent/Audio/Explosion_Cue.Explosion_Cue" (`self.K2_GetActorLocation`) (struct) 1.0 1.0 0.0 null null null)
  (`self.SetLifeSpan` 2.0))

(event `self.ReceiveEndPlay`
  (params (EndPlayReason :type "EEndPlayReason Enum" :default "Destroyed"))
  (switch `EEndPlayReason` EndPlayReason
    (:`Destroyed`
      (`GameplayStatics.SpawnEmitterAtLocation` "/Game/Static/SciFiWeapDark/FX/Particles/P_Grenade_Explosion_Dark.P_Grenade_Explosion_Dark" (`self.K2_GetActorLocation`)))))

(fn `UserConstructionScript`)