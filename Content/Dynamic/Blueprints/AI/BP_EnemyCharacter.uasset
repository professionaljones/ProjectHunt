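; Enemy character Blueprint that sets starting health and reacts to damage with sound.
; On BeginPlay it copies MaxStartHealth into the StatsComponent's current health.
; AnyDamage defers to the parent implementation, then plays the enemy damage cue through CharacterAudioComponent.
; UpdateWalkSpeed sets the movement component's max walk speed.
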(event `self.ReceiveBeginPlay`
  (set `HuntStatsComponent.CurrentHealth` (`self.MaxStartHealth`) (`self.StatsComponent`)))

(event `self.ReceiveAnyDamage`
  (params (Damage :type "Float (single-precision)") (DamageType :type "DamageType Object Reference") (InstigatedBy :type "Controller Object Reference") (DamageCauser :type "Actor Object Reference"))
  (bind _characteraudiocomponent (`self.CharacterAudioComponent`))
  (`parent.ReceiveAnyDamage` Damage DamageType InstigatedBy DamageCauser)
  (`AudioComponent.SetSound` _characteraudiocomponent "/Game/Static/Audio/SFX/Enemy/Damage/A_EnemyDamage_Cue.A_EnemyDamage_Cue")
  (`AudioComponent.Play` _characteraudiocomponent 0.0))

(fn `UpdateWalkSpeed`
  (params (NewWalkSpeed :type "Float (double-precision)"))
  (set `CharacterMovementComponent.MaxWalkSpeed` NewWalkSpeed (`self.CharacterMovement`)))

(fn `UserConstructionScript`)