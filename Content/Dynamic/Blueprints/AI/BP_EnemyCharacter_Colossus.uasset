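; Colossus boss enemy character that drives a dedicated boss health bar on the player's gameplay HUD.
; BeginPlay registers it and its name with the boss widget, then binds health updates that set the bar material's Progress parameter.
; Activation reveals the bar.
; Player overlap with its Box applies knockback and damage, and spawns an enlarged Chrono AI hunt projectile.
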(event `self.ReceiveBeginPlay`
  (bind _wbp_bosshealth (`/Game/Dynamic/UI/WBP_GameplayHUD.WBP_BossHealth` (`/Game/Dynamic/Blueprints/Player/BP_HuntPlayerController_Base.GameplayWBP` (cast `/Game/Dynamic/Blueprints/Player/BP_Gameplay_PlayerController` (`GameplayStatics.GetPlayerController` 0) :!pure true))))
  (`parent.ReceiveBeginPlay`)
  (set `/Game/Dynamic/UI/WBP_BossHealth.EnemyReference` (`|ConvertAsset` self) _wbp_bosshealth)
  (`TextBlock.SetText` (`/Game/Dynamic/UI/WBP_BossHealth.EnemyName` _wbp_bosshealth) (`KismetTextLibrary.Conv_StringToText` (`HuntStatsComponent.CharacterName` (`self.StatsComponent`))))
  (bind _returnvalue (`Image.GetDynamicMaterial` (`/Game/Dynamic/UI/WBP_BossHealth.HealthBarImage` _wbp_bosshealth)))
  (set `self.HealthBarImage_DynMat` _returnvalue)
  (add `self.UpdateHealthStats` (`|CreateDelegate` :!event `UpdateBossUI`))
  (`self.UpdateBossUI`))

(event `UpdateBossUI`
  (bind _statscomponent (`self.StatsComponent`))
  (if (not (`HuntStatsComponent.bIsDead` _statscomponent))
    (`MaterialInstanceDynamic.SetScalarParameterValue` (`self.HealthBarImage_DynMat`) "Progress" (/ (`HuntStatsComponent.GetCurrentHealth` _statscomponent) (`HuntStatsComponent.GetMaxHealth` _statscomponent)))))

(event `self.Box.OnComponentBeginOverlap`
  (params (OverlappedComponent :type "PrimitiveComponent Object Reference") (OtherActor :type "Actor Object Reference") (OtherComp :type "PrimitiveComponent Object Reference") (OtherBodyIndex :type Integer) (bFromSweep :type Boolean) (SweepResult :type "HitResult Structure (by ref)"))
  (bind _returnvalue (`GameplayStatics.GetPlayerCharacter` 0))
  (if (== OtherActor _returnvalue)
    (`CharacterMovementComponent.AddImpulse` (`Character.CharacterMovement` _returnvalue) (`self.PlayerKnockbackVector`) true)
    (`GameplayStatics.ApplyDamage` OtherActor 4.0)
    (`|SpawnActorFromClass` "/Game/Dynamic/Blueprints/Weapons/Projectiles/BP_HuntProjectile_Chrono_AI.BP_HuntProjectile_Chrono_AI_C" (`KismetMathLibrary.MakeTransform` (`SceneComponent.K2_GetComponentLocation` (`self.Scene`)) (`self.GetControlRotation`) (2.0 2.0 2.0)) "Undefined" "OverrideRootScale" null 0.0 null)))

(event `self.Box.OnComponentHit`
  (params (HitComponent :type "PrimitiveComponent Object Reference") (OtherActor :type "Actor Object Reference") (OtherComp :type "PrimitiveComponent Object Reference") (NormalImpulse :type "Vector Structure") (Hit :type "HitResult Structure (by ref)")))

(fn `OnActivateEnemy`
  (`Widget.SetVisibility` (`/Game/Dynamic/UI/WBP_GameplayHUD.WBP_BossHealth` (`/Game/Dynamic/Blueprints/Player/BP_HuntPlayerController_Base.GameplayWBP` (cast `/Game/Dynamic/Blueprints/Player/BP_Gameplay_PlayerController` (`GameplayStatics.GetPlayerController` 0) :!pure true))) "HitTestInvisible"))

(fn `UserConstructionScript`
  (`parent.UserConstructionScript`))