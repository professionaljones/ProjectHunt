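; BP_C13Drone is an AI drone that steers around obstacles and can fire a damaging line trace.
; Each Tick, while outside player range, component-aimed traces switch its direction state, which drives world-axis movement input.
; First coming within range permanently switches it to NoDirection, which heads toward a fixed point near world origin, not the player.
; OnAttackTarget calls Fire, whose trace end scales actor location, ignoring facing, and damages HuntCharacterInterface actors.
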(event `self.ReceiveBeginPlay`
  (bind _huntstats (`self.HuntStats`))
  (`self.DroneMovementCalculation` (`self.bIsNearPlayer`))
  (set `HuntStatsComponent.CurrentHealth` (`HuntStatsComponent.GetMaxHealth` _huntstats) _huntstats))

(event `self.ReceiveTick`
  (params (DeltaSeconds :type "Float (single-precision)"))
  (`|ExecutionSequence`
    (:`then_0`
      (bind _output_get (set `self.bIsNearPlayer` (not (> (`self.GetDistanceToPlayer`) (`self.PlayerProximityRange`)))))
      (`self.DroneMovementCalculation` _output_get))
    (:`then_1`
      (switch `/Game/Dynamic/Blueprints/Enemies/EDroneMovementDirection` (`self.DroneMovementDirection`)
        (:`NewEnumerator0`
          (`self.AddMovementInput` (0.0 1.0 0.0) 1.0 true))
        (:`NewEnumerator1`
          (`self.AddMovementInput` (0.0 0.0 1.0) 1.0 true))
        (:`NewEnumerator2`
          (`self.AddMovementInput` (0.0 0.0 -1.0) 1.0 true))
        (:`NewEnumerator3`
          (`self.AddMovementInput` (0.0 -1.0 0.0) 1.0 true))
        (:`NewEnumerator4`
          (`self.AddMovementInput` (`KismetMathLibrary.GetDirectionUnitVector` (`self.K2_GetActorLocation`) (+ (0.0 0.0 0.0) (0.0 0.0 55.0))) 1.0 true))))))

(event `Fire`
  (bind _returnvalue (`self.K2_GetActorLocation`))
  (bind _outhit (`KismetSystemLibrary.LineTraceSingleForObjects` :`Start` _returnvalue :`End` (* _returnvalue 300.0) :`ObjectTypes` (`|MakeArray` "ObjectTypeQuery9" :!type "EObjectTypeQuery Enum") :`bTraceComplex` true :`DrawDebugType` "ForOneFrame"))
  (bind (_bblockinghit _binitialoverlap _time _distance _location _impactpoint _normal _impactnormal _physmat _hitactor) (`GameplayStatics.BreakHitResult` _outhit))
  (if _bblockinghit
    (if (`KismetSystemLibrary.DoesImplementInterface` _hitactor "/Script/ProjectHunt.HuntCharacterInterface")
      (`GameplayStatics.ApplyDamage` _hitactor 5.0))))

(event `HuntCharacterInterface.OnAttackTarget`
  (`self.Fire`))

(event `OnNearPlayer`
  (set `self.DroneMovementDirection` "NewEnumerator4"))

(fn `DroneMovementCalculation`
  (params (`bIsNearPlayer?` :type Boolean))
  (bind _returnvalue (`self.K2_GetActorLocation`))
  (if `bIsNearPlayer?`
    (`|ExecutionSequence`
      (:`then_0`
        (`/Engine/EditorBlueprintResources/StandardMacros.DoOnce` false
          (:`Completed`
            (`self.OnNearPlayer`)))))
    (else
      (switch `/Game/Dynamic/Blueprints/Enemies/EDroneMovementDirection` (`self.DroneMovementDirection`)
        (:`NewEnumerator0`
          (bind (_outhit _returnvalue_2) (`KismetSystemLibrary.LineTraceSingleForObjects` :`Start` (`self.K2_GetActorLocation`) :`End` (`SceneComponent.K2_GetComponentLocation` (`self.ForwardTrace`)) :`ObjectTypes` (`self.ObjectTypeArray`) :`DrawDebugType` "ForDuration"))
          (if _returnvalue_2
            (set `self.DroneMovementDirection` "NewEnumerator1")
            (else
              (`KismetSystemLibrary.LineTraceSingleForObjects` :`Start` (`self.K2_GetActorLocation`) :`End` (`SceneComponent.K2_GetComponentLocation` (`self.UpTrace`)) :`ObjectTypes` (`self.ObjectTypeArray`) :`DrawDebugType` "ForOneFrame"))))
        (:`NewEnumerator1`
          (bind (_outhit_2 _returnvalue_3) (`KismetSystemLibrary.LineTraceSingleForObjects` :`Start` _returnvalue :`End` (`SceneComponent.K2_GetComponentLocation` (`self.ForwardTrace`)) :`ObjectTypes` (`self.ObjectTypeArray`) :`DrawDebugType` "ForDuration"))
          (if (not _returnvalue_3)
            (set `self.DroneMovementDirection` "NewEnumerator0")))
        (:`NewEnumerator2`
          (bind (_outhit_3 _returnvalue_4) (`KismetSystemLibrary.LineTraceSingleForObjects` :`Start` _returnvalue :`End` (`SceneComponent.K2_GetComponentLocation` (`self.UpTrace`)) :`ObjectTypes` (`self.ObjectTypeArray`) :`DrawDebugType` "ForDuration"))
          (if (not _returnvalue_4)
            (set `self.DroneMovementDirection` "NewEnumerator0")))))))

(fn `GetDistanceToPlayer`
  (returns (ReturnValue :type "Float (double-precision)"))
  (return (`KismetMathLibrary.VSize` (- (`self.K2_GetActorLocation`) (`self.K2_GetActorLocation` (`GameplayStatics.GetPlayerPawn` 0))))))

(fn `UserConstructionScript`
  (`parent.UserConstructionScript`))