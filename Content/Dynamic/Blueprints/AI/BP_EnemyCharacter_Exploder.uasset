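; Exploder enemy character that explodes when it leaves play.
; EndPlay spawns a dark rocket-launcher explosion effect and sound at the actor's location, then applies radial damage with falloff from configurable base damage and inner and outer radii.
; The explosion hangs on EndPlay without checking the end reason, so it is not limited to death.
; Debug spheres for both radii are present but unconnected.
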(event `self.ReceiveEndPlay`
  (params (EndPlayReason :type "EEndPlayReason Enum" :default "Destroyed"))
  (bind _returnvalue (`self.K2_GetActorLocation`))
  (`GameplayStatics.SpawnEmitterAtLocation` "/Game/Static/SciFiWeapDark/FX/Particles/P_RocketLauncher_Explosion_Dark.P_RocketLauncher_Explosion_Dark" _returnvalue)
  (`GameplayStatics.PlaySoundAtLocation` "/Game/Static/SciFiWeapDark/Sound/RocketLauncher/RocketLauncher_Explosion_Cue.RocketLauncher_Explosion_Cue" _returnvalue (struct) 1.0 1.0 0.0 null null null)
  (`GameplayStatics.ApplyRadialDamageWithFalloff` :`BaseDamage` (`self.BaseExplosionDamage`) :`MinimumDamage` 1.0 :`Origin` _returnvalue :`DamageInnerRadius` (`self.DamageInnerRadius`) :`DamageOuterRadius` (`self.DamageOuterRadius`) :`DamageFalloff` 1.5 :`DamageCauser` self :`InstigatedByController` (`self.GetInstigatorController`)))

(fn `UserConstructionScript`
  (`parent.UserConstructionScript`))