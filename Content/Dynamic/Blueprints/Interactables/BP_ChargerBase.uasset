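; Base charger station that the player charges by damaging it, playing a power-up sound when full.
; Damage adds charge, requiring a matching weapon ammo type unless RequiresStandardAmmo is set, which skips the check.
; Looping one-second timers cache the player's weapon and drive charge decay, and both stop at full charge.
; Tick tints a dynamic material green by ChargePercentage, which only updates on accepted hits.
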(event `self.ReceiveBeginPlay`
  (bind _staticmesh1 (`self.StaticMesh1`))
  (bind _returnvalue (`KismetSystemLibrary.K2_SetTimerDelegate` (delegate `CheckForWeapon`) 1.0 true))
  (set `self.CheckTimer` _returnvalue)
  (bind _returnvalue_2 (`PrimitiveComponent.CreateDynamicMaterialInstance` _staticmesh1 0 (`PrimitiveComponent.GetMaterial` _staticmesh1 0) "None"))
  (set `self.ChargerMat` _returnvalue_2)
  (bind _returnvalue_3 (`KismetSystemLibrary.K2_SetTimerDelegate` (`|CreateDelegate` :!event `DecreaseCharge`) 1.0 true))
  (set `self.ChargeDecTimer` _returnvalue_3)
  (if (`self.bRequiresStandardAmmo?`)
    (set `self.RequiredAmmoType` "AT_Standard")))

(event `CheckForWeapon`
  (bind _ashunt_player_character (cast `HuntPlayerCharacter` (`GameplayStatics.GetPlayerCharacter` 0) :!pure true))
  (`/Engine/EditorBlueprintResources/StandardMacros.IsValid` _ashunt_player_character
    (:`Is Valid`
      (set `self.PC_Weapon` (`ProjectHuntCharacter.CurrentWeapon` _ashunt_player_character)))
    (:`Is Not Valid`
      (`KismetSystemLibrary.K2_ClearAndInvalidateTimerHandle` (`self.checkTimer`)))))

(event `self.ReceiveAnyDamage`
  (params (Damage :type "Float (single-precision)") (DamageType :type "DamageType Object Reference") (InstigatedBy :type "Controller Object Reference") (DamageCauser :type "Actor Object Reference"))
  (bind _pc_weapon (`self.PC_Weapon`))
  (if (== InstigatedBy (`GameplayStatics.GetPlayerController` 0))
    (if (`self.bRequiresStandardAmmo?`)
      (set `self.ChargePercentage` (/ (`self.CurrentChargeLimit`) (`self.MaxChargeLimit`)) :!label _label)
      (bind _output_get (set `self.CurrentChargeLimit` (+ (`self.CurrentChargeLimit`) Damage)))
      (`|ExecutionSequence`
        (:`then_0`
          (if (`KismetSystemLibrary.K2_TimerExistsHandle` (`self.ChargeDecTimer`))
            _))
        (:`then_1`
          (if (>= _output_get (`self.MaxChargeLimit`))
            (set `self.bIsStationCharged?` true)
            (`/Engine/EditorBlueprintResources/StandardMacros.DoOnce` false :!label _label_2
              (:`Completed`
                (`KismetSystemLibrary.K2_ClearAndInvalidateTimerHandle` (`self.ChargeDecTimer`))
                (`KismetSystemLibrary.K2_ClearAndInvalidateTimerHandle` (`self.CheckTimer`))
                (`GameplayStatics.PlaySoundAtLocation` "/Game/Static/Audio/SFX/ChargerStation_PowerUp.ChargerStation_PowerUp" (`self.K2_GetActorLocation`) (struct) 1.0 1.0 0.0 null null null)))
            (else
              (goto _label_2 :!via `Reset`)))))
      (else
        (`/Engine/EditorBlueprintResources/StandardMacros.IsValid` _pc_weapon
          (:`Is Valid`
            (if (`|EnumEquality` (`self.RequiredAmmoType`) (`.WeaponAmmoType` (break `WeaponStatsData` (`HuntWeapon.WeaponStatsData` _pc_weapon))))
              (goto _label))))))))

(event `DecreaseCharge`
  (if (> (`self.CurrentChargeLimit`) 1.0)
    (set `self.CurrentChargeLimit` (- (`self.CurrentChargeLimit`) 1.0))))

(event `self.ReceiveTick`
  (params (DeltaSeconds :type "Float (single-precision)"))
  (`self.UpdateChargerColor` 0.0 (`self.ChargePercentage`)))

(fn `UpdateChargerColor`
  (params (R :type "Float (double-precision)") (G :type "Float (double-precision)") (B :type "Float (double-precision)"))
  (`MaterialInstanceDynamic.SetVectorParameterValue` (`self.ChargerMat`) "Color" (`KismetMathLibrary.MakeColor` R G B)))

(fn `UserConstructionScript`)