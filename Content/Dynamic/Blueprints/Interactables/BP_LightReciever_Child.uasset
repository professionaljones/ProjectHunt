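; Child light receiver interactable that builds up charge when the player damages it.
; Its AnyDamage event adds the damage to Charge only when the damage causer is the player character, then prints the new total on screen in orange.
; The construction script defers to the parent, and the BeginPlay, Tick and overlap events are disabled stubs.
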(event `self.ReceiveAnyDamage`
  (params (Damage :type "Float (single-precision)") (DamageType :type "DamageType Object Reference") (InstigatedBy :type "Controller Object Reference") (DamageCauser :type "Actor Object Reference"))
  (if (== DamageCauser (`GameplayStatics.GetPlayerCharacter` 0))
    (bind _output_get (set `self.Charge` (+ (`self.Charge`) Damage)))
    (`KismetSystemLibrary.PrintString` (`KismetStringLibrary.Conv_DoubleToString` _output_get) true true (struct :`R` 1.0 :`G` 0.652018 :`A` 1.0))))

(fn `UserConstructionScript`
  (`parent.UserConstructionScript`))