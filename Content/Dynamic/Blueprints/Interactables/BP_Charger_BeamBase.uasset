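; Base Blueprint for a charger interactable that drives a light beam from its charge level.
; On BeginPlay it spawns an actor of its configured light beam class at its scene component's world transform and keeps a reference to it.
; Every Tick it passes its charge percentage to that beam to adjust the beam's length.
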(event `self.ReceiveBeginPlay`
  (`parent.ReceiveBeginPlay`)
  (bind _returnvalue (`|SpawnActorFromClass` (`self.MyLightBeamClass`) (`SceneComponent.K2_GetComponentToWorld` (`self.Scene`)) "Undefined" "OverrideRootScale" null null))
  (set `self.MyLightBeam` _returnvalue))

(event `self.ReceiveTick`
  (params (DeltaSeconds :type "Float (single-precision)"))
  (`/Game/Dynamic/Blueprints/Interactables/BP_LightBeam.AdjustBeamLength` (`self.MyLightBeam`) (`self.ChargePercentage`)))

(fn `UserConstructionScript`
  (`parent.UserConstructionScript`))