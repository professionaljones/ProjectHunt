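; BP_LightReciever is an interactable that tracks whether all of its assigned light beams are charged.
; A looping one-second timer started at BeginPlay is meant to poll BeamsToRecieve, adding nearly full beams to ChargedBeams and removing the rest.
; Once every beam counts as charged it clears the timer; no further response is wired, apart from a debug print per charged beam.
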(event `self.ReceiveBeginPlay`
  (bind _returnvalue (`KismetSystemLibrary.K2_SetTimerDelegate` (`|CreateDelegate` :!event `CheckBeams`) 1.0 true))
  (set `self.CheckBeamsTimerHandle` _returnvalue))

(fn `CheckBeams`
  (bind _beamstorecieve (`self.BeamsToRecieve`))
  (`|ExecutionSequence`
    (:`then_0`
      (for _array_element _beamstorecieve
        (if (>= (`/Game/Dynamic/Blueprints/Interactables/BP_ChargerBase.ChargePercentage` _array_element) 0.99)
          (`KismetSystemLibrary.PrintString` (`KismetStringLibrary.Concat_StrStr` (`KismetSystemLibrary.GetDisplayName` _array_element) " " "is charged!"))
          (`KismetArrayLibrary.Array_AddUnique` (`self.ChargedBeams`) _array_element)
          (else
            (`KismetArrayLibrary.Array_RemoveItem` (`self.ChargedBeams`) _array_element)))))
    (:`then_1`
      (if (>= (`KismetArrayLibrary.Array_Length` (`self.ChargedBeams`)) (`KismetArrayLibrary.Array_Length` _beamstorecieve))
        (`KismetSystemLibrary.K2_ClearAndInvalidateTimerHandle` (`self.CheckBeamsTimerHandle`))))))

(fn `UserConstructionScript`)