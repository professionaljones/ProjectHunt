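; Debug trigger that gives the player a preset stats loadout, one of Base, Low, Mid, High or Max.
; On BeginPlay its text render shows the name of the selected loadout.
; When activated, it switches on that loadout and sends the matching give-stats message to the player character.
; Leftover code to turn the text by the player's control rotation is disconnected and never runs.
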(event `self.ReceiveBeginPlay`
  (`parent.ReceiveBeginPlay`)
  (`TextRenderComponent.K2_SetText` (`self.TextRender`) (`KismetTextLibrary.Conv_StringToText` (`self.DesiredStatsLoadout`))))

(event `self.ReceiveTick`
  (params (DeltaSeconds :type "Float (single-precision)"))
  (`parent.ReceiveTick` DeltaSeconds))

(event `self.ActivateTrigger`
  (bind _returnvalue (`GameplayStatics.GetPlayerCharacter` 0))
  (switch `string` (`self.DesiredStatsLoadout`)
    (:`Base`
      (message `/Game/Dynamic/Blueprints/Game/BPI_CheatsAndDebug.OnGivePlayerBaseStats` _returnvalue))
    (:`Low`
      (message `/Game/Dynamic/Blueprints/Game/BPI_CheatsAndDebug.OnGivePlayerLowStats` _returnvalue))
    (:`Mid`
      (message `/Game/Dynamic/Blueprints/Game/BPI_CheatsAndDebug.OnGivePlayerMidStats` _returnvalue))
    (:`High`
      (message `/Game/Dynamic/Blueprints/Game/BPI_CheatsAndDebug.OnGivePlayerHighStats` _returnvalue))
    (:`Max`
      (message `/Game/Dynamic/Blueprints/Game/BPI_CheatsAndDebug.OnGivePlayerMaxStats` _returnvalue))))

(fn `UserConstructionScript`
  (`parent.UserConstructionScript`))