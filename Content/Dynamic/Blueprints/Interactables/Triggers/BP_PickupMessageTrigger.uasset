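; BP_PickupMessageTrigger is an interactable trigger that shows a timed pickup message while briefly freezing the player.
; On ActivateTrigger, if no widget is valid, it creates WBP_PickupMessage with MessageText, then disables gameplay input and stops player movement.
; After a delay it reverses the widget's construct animation, removes it and restores input and movement.
; It finally disables the Box collision, apparently to make the trigger one-shot.
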(event `self.ActivateTrigger`
  (bind _messagewbp (`self.MessageWBP`))
  (bind _asbp_trish_player_character (cast `/Game/Dynamic/Blueprints/Player/BP_TrishPlayerCharacter` (`GameplayStatics.GetPlayerCharacter` 0) :!pure true))
  (bind _asbp_hunt_player_controller_base (cast `/Game/Dynamic/Blueprints/Player/BP_HuntPlayerController_Base` (`GameplayStatics.GetPlayerController` 0) :!pure true))
  (`/Engine/EditorBlueprintResources/StandardMacros.IsValid` (`self.MessageWBP`)
    (:`Is Not Valid`
      (bind _returnvalue (`|CreateWidget` "/Game/Dynamic/UI/WBP_PickupMessage.WBP_PickupMessage_C" null (`self.MessageText`)))
      (bind _output_get (set `self.MessageWBP` _returnvalue))
      (`UserWidget.AddToViewport` (`self.MessageWBP`) 0)
      (`/Game/Dynamic/Blueprints/Player/BP_HuntPlayerController_Base.DisableGameplayInput` _asbp_hunt_player_controller_base false false)
      (`/Game/Dynamic/Blueprints/Player/BP_TrishPlayerCharacter.StopPlayerMovement` _asbp_trish_player_character)
      (`KismetSystemLibrary.Delay` 3.0)
      (`UserWidget.PlayAnimationReverse` _messagewbp (`/Game/Dynamic/UI/WBP_PickupMessage.ConstructAnimation` _output_get) 1.0 false)
      (`KismetSystemLibrary.Delay` 1.0)
      (`Widget.RemoveFromParent` _messagewbp)
      (`/Game/Dynamic/Blueprints/Player/BP_HuntPlayerController_Base.EnableGameplayInput` _asbp_hunt_player_controller_base)
      (`/Game/Dynamic/Blueprints/Player/BP_TrishPlayerCharacter.StartPlayerMovement` _asbp_trish_player_character)
      (`PrimitiveComponent.SetCollisionEnabled` (`self.Box`) "NoCollision"))))

(fn `UserConstructionScript`
  (`parent.UserConstructionScript`))