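; BP_AmmoTypeChanger is an interactable trigger that changes the ammo type of the player's currently held weapon.
; ActivateTrigger casts player 0 to BP_FP_TrishPlayerCharacter and, if CurrentWeapon is valid, writes NewAmmoType into its WeaponStatsData struct.
; Fire ammo also sets the weapon's damage modifier to a boosted fixed value; other types leave that modifier untouched.
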(event `self.ActivateTrigger`
  (bind _newammotype (`self.NewAmmoType`))
  (bind _currentweapon (`ProjectHuntCharacter.CurrentWeapon` (cast `/Game/Dynamic/Blueprints/Player/BP_FP_TrishPlayerCharacter` (`GameplayStatics.GetPlayerCharacter` 0) :!pure true)))
  (bind _weaponstatsdata (`HuntWeapon.WeaponStatsData` _currentweapon))
  (`/Engine/EditorBlueprintResources/StandardMacros.IsValid` _currentweapon
    (:`Is Valid`
      (setmembers `WeaponStatsData` :`StructRef` _weaponstatsdata :`WeaponAmmoType` _newammotype)
      (if (`|EnumEquality` _newammotype "AT_Fire")
        (setmembers `WeaponStatsData` :`StructRef` _weaponstatsdata :`DamageModifierAmount` 1.5)))))

(fn `UserConstructionScript`
  (`parent.UserConstructionScript`))