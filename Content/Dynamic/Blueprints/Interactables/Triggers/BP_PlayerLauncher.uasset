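; BP_PlayerLauncher is a trigger interactable that launches the player character when activated.
; Its ActivateTrigger event calls LaunchCharacter on player 0 with a scaled LaunchVelocity variable, overriding both XY and Z velocity, then plays a 2D supercharger sound.
; It always targets the first player regardless of what activated it, and has no active overlap or tick logic of its own.
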(event `self.ActivateTrigger`
  (`Character.LaunchCharacter` (`GameplayStatics.GetPlayerCharacter` 0) (* (`self.LaunchVelocity`) 5.0) true true)
  (`GameplayStatics.PlaySound2D` "/Game/Static/Audio/SFX/Supercharger_Step.Supercharger_Step" 1.0 1.0 0.0 null null))

(fn `UserConstructionScript`
  (`parent.UserConstructionScript`))