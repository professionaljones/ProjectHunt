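; Debug trigger actor that switches the player's main ability to a configured choice when activated.
; On BeginPlay a text render component displays the DesiredMainAbility value as a label.
; ActivateTrigger switches on that value and sends player character 0 a set-main-ability message for Quicksilver, Showstopper or Overload.
; A leftover, unconnected node chain would turn the label toward the player's control rotation, but it never runs.
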(event `self.ReceiveBeginPlay`
  (`parent.ReceiveBeginPlay`)
  (`TextRenderComponent.K2_SetText` (`self.TextRender`) (`KismetTextLibrary.Conv_StringToText` (`self.DesiredMainAbility`))))

(event `self.ReceiveTick`
  (params (DeltaSeconds :type "Float (single-precision)"))
  (`parent.ReceiveTick` DeltaSeconds))

(event `self.ActivateTrigger`
  (bind _returnvalue (`GameplayStatics.GetPlayerCharacter` 0))
  (switch `string` (`self.DesiredMainAbility`)
    (:`Quicksilver`
      (message `/Game/Dynamic/Blueprints/Game/BPI_CheatsAndDebug.OnSetMainAbility` _returnvalue "MA_Quicksilver"))
    (:`Showstopper`
      (message `/Game/Dynamic/Blueprints/Game/BPI_CheatsAndDebug.OnSetMainAbility` _returnvalue "MA_Showstopper"))
    (:`Overload`
      (message `/Game/Dynamic/Blueprints/Game/BPI_CheatsAndDebug.OnSetMainAbility` _returnvalue "MA_Overload"))))

(fn `UserConstructionScript`
  (`parent.UserConstructionScript`))