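; Tutorial trigger that shows a gameplay message with action text and input text when activated.
; ActivateTrigger has GenerateNewText build two dialog entries, then passes them and the input action name to a WBP_GameplayMessage with a per-letter delay.
; It adds the widget to the viewport, clears the player controller's LastWBP and disables the box collision to prevent retriggering.
; Player movement and HUD toggling logic is left unconnected.
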(event `self.ReceiveBeginPlay`
  (`parent.ReceiveBeginPlay`))

(event `self.ActivateTrigger`
  (`/Engine/EditorBlueprintResources/StandardMacros.IsValid` (`self.MessageWBP`)
    (:`Is Not Valid`
      (`self.GenerateNewText`)
      (bind _returnvalue (`|CreateWidget` "/Game/Dynamic/UI/Gameplay/WBP_GameplayMessage.WBP_GameplayMessage_C" (`GameplayStatics.GetPlayerController` 0) 2.0 0.09 (`self.DialogTables`) 0 (`self.NewActionName`) null 1))
      (bind _output_get (set `self.MessageWBP` _returnvalue))
      (set `/Game/Dynamic/Blueprints/Player/BP_HuntPlayerController_Base.LastWBP` null (cast `/Game/Dynamic/Blueprints/Player/BP_HuntPlayerController_Base` (`GameplayStatics.GetPlayerController` 0) :!pure true))
      (`UserWidget.AddToViewport` _output_get 0)
      (`PrimitiveComponent.SetCollisionEnabled` (`self.Box`) "NoCollision"))))

(fn `GenerateNewText`
  (bind _dialogtables (`self.DialogTables`))
  (`KismetArrayLibrary.Array_AddUnique` _dialogtables (make `/Game/Examples/UC/-StorytellerObject/DialogTrees` 0 (`|MakeArray` (`KismetTextLibrary.Conv_StringToText` (`KismetTextLibrary.Conv_TextToString` (`self.ActionText`))))))
  (`KismetArrayLibrary.Array_AddUnique` _dialogtables (make `/Game/Examples/UC/-StorytellerObject/DialogTrees` 1 (`|MakeArray` (`self.InputActionText`)))))

(fn `UserConstructionScript`
  (`parent.UserConstructionScript`))