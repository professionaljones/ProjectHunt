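; BP_SubtitlesTrigger is an interactable trigger that shows a subtitle on screen when activated.
; ActivateTrigger creates a WBP_Subtitles widget from its dialog array, message index and speaker name, then adds it to the viewport.
; After a fixed delay it removes the widget and disables the Box collision.
; The MessageWBP validity check gates creation, but this graph never assigns that variable.
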(event `self.ActivateTrigger`
  (`/Engine/EditorBlueprintResources/StandardMacros.IsValid` (`self.MessageWBP`)
    (:`Is Not Valid`
      (bind _returnvalue (`|CreateWidget` "/Game/Dynamic/UI/Gameplay/WBP_Subtitles.WBP_Subtitles_C" null (`self.NewDialog`) (`self.MessageIndex`) 2.0 0.1 (`self.SpeakerName`)))
      (`UserWidget.AddToViewport` _returnvalue 0)
      (`KismetSystemLibrary.Delay` 3.0)
      (`Widget.RemoveFromParent` _returnvalue)
      (`PrimitiveComponent.SetCollisionEnabled` (`self.Box`) "NoCollision"))))

(fn `UserConstructionScript`
  (`parent.UserConstructionScript`))