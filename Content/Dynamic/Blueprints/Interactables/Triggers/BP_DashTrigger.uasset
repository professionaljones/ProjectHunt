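; BP_DashTrigger is an interactable trigger that activates when the player character hits its box while dashing.
; The hit handler checks BP_TrishPlayerCharacter's IsDashing, calls OnTriggerOverlap, sets IsActivated and starts a one-shot timer lasting TriggerTimeLimit.
; When the timer expires, ToggleActivateStatus clears IsActivated and calls OnDeactivated.
; Tick prints the remaining time while activated, and the hit also prints a debug string.
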(event `self.ReceiveTick`
  (params (DeltaSeconds :type "Float (single-precision)"))
  (`parent.ReceiveTick` DeltaSeconds)
  (if (`self.bIsActivated?`)
    (`KismetSystemLibrary.PrintString` (`KismetStringLibrary.TimeSecondsToString` (`KismetSystemLibrary.K2_GetTimerRemainingTimeHandle` (`self.TimerHandle`))))))

(event `self.Box.OnComponentHit`
  (params (HitComponent :type "PrimitiveComponent Object Reference") (OtherActor :type "Actor Object Reference") (OtherComp :type "PrimitiveComponent Object Reference") (NormalImpulse :type "Vector Structure") (Hit :type "HitResult Structure (by ref)"))
  (bind _returnvalue (`GameplayStatics.GetPlayerCharacter` 0))
  (if (== OtherActor _returnvalue)
    (if (`/Game/Dynamic/Blueprints/Player/BP_TrishPlayerCharacter.bIsDashing?` (cast `/Game/Dynamic/Blueprints/Player/BP_TrishPlayerCharacter` _returnvalue :!pure true))
      (`self.OnTriggerOverlap`)
      (`KismetSystemLibrary.PrintString` "Hello")
      (set `self.bIsActivated?` true)
      (bind _returnvalue_2 (`KismetSystemLibrary.K2_SetTimerDelegate` (delegate `ToggleActivateStatus`) (`self.TriggerTimeLimit`)))
      (set `self.TimerHandle` _returnvalue_2))))

(event `ToggleActivateStatus`
  (if (`self.bIsActivated?`)
    (set `self.bIsActivated?` false)
    (`self.OnDeactivated`)))

(fn `UserConstructionScript`
  (`parent.UserConstructionScript`))