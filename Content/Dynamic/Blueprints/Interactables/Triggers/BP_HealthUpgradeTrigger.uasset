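; BP_HealthUpgradeTrigger is a trigger that permanently upgrades the player's health and auto-saves the game.
; ActivateTrigger raises health stats through the player's StatsComponent, shows a temporary "energy increased" widget and saves asynchronously.
; It fades its audio and sets a short lifespan, disabling box collision only after the message delay.
; EndPlay spawns a healing-leaf particle effect when the actor is destroyed.
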(event `self.ReceiveBeginPlay`
  (`parent.ReceiveBeginPlay`))

(event `self.ActivateTrigger`
  (`HuntStatsComponent.UpgradeHealthStats` (`ProjectHuntCharacter.StatsComponent` (cast `ProjectHuntCharacter` (`GameplayStatics.GetPlayerCharacter` 0) :!pure true)) 100.0)
  (bind _returnvalue (`|CreateWidget` "/Game/Dynamic/UI/WBP_PickupMessage.WBP_PickupMessage_C" null "Your energy has been increased!"))
  (`UserWidget.AddToViewport` _returnvalue 0)
  (`/Game/Dynamic/Blueprints/Game/BP_ProjectHuntGameInstance.AsyncSaveSlot` (cast `/Game/Dynamic/Blueprints/Game/BP_ProjectHuntGameInstance` (`GameplayStatics.GetGameInstance`) :!pure true) "AutoSave")
  (`self.SetLifeSpan` 3.5)
  (`AudioComponent.FadeOut` (`self.Audio`) 3.2 0.0 "Linear")
  (`KismetSystemLibrary.Delay` 3.0)
  (`Widget.RemoveFromParent` _returnvalue)
  (`PrimitiveComponent.SetCollisionEnabled` (`self.Box`) "NoCollision"))

(event `self.ReceiveEndPlay`
  (params (EndPlayReason :type "EEndPlayReason Enum" :default "Destroyed"))
  (switch `EEndPlayReason` EndPlayReason
    (:`Destroyed`
      (`GameplayStatics.SpawnEmitterAtLocation` "/Game/Static/VFX_Toolkit_V1/ParticleSystems/356Days/Par_HealLeaf_01.Par_HealLeaf_01" (`self.K2_GetActorLocation`)))))

(fn `UserConstructionScript`
  (`parent.UserConstructionScript`))