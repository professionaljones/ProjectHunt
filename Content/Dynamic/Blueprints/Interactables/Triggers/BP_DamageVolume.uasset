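; BP_DamageVolume is an interactable trigger that hurts the player when ActivateTrigger fires.
; It applies fixed damage to the player character if that character can be damaged.
; A random coin flip then decides whether to start a looping timer, which is cleared after a delay; the timer's bound event is not shown.
; BeginPlay, overlap and Tick are disabled stubs.
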(event `self.ActivateTrigger`
  (bind _returnvalue (`GameplayStatics.GetPlayerCharacter` 0))
  (if (`Actor.bCanBeDamaged` _returnvalue)
    (`GameplayStatics.ApplyDamage` _returnvalue 15.0 null self)
    (if (`KismetMathLibrary.RandomBool`)
      (bind _returnvalue_2 (`KismetSystemLibrary.K2_SetTimerDelegate` (`|CreateDelegate` (cast `/Game/Dynamic/Blueprints/Player/BP_TrishPlayerCharacter` _returnvalue :!pure true) :!event `FireDamage_Player`) 1.0 true))
      (`KismetSystemLibrary.Delay` 10.0)
      (`KismetSystemLibrary.K2_ClearAndInvalidateTimerHandle` _returnvalue_2))))

(fn `UserConstructionScript`
  (`parent.UserConstructionScript`))