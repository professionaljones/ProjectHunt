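; BP_SaveStation is an interactable trigger that acts as a save point and restores the player's health.
; On BeginPlay it spawns a BP_ParticleHole actor at the transform of its Scene component.
; When activated, it adds a WBP_SaveScreen widget to the viewport, heals the HuntPlayerCharacter through its PlayerStatsComponent with a large fixed amount, and refreshes the stats UI.
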(event `self.ReceiveBeginPlay`
  (`parent.ReceiveBeginPlay`)
  (`|SpawnActorFromClass` "/Game/Wormholes/Blueprints/BP_ParticleHole.BP_ParticleHole_C" (`SceneComponent.K2_GetComponentToWorld` (`self.Scene`)) "Undefined" "OverrideRootScale" null null))

(event `self.ActivateTrigger`
  (bind _returnvalue (`GameplayStatics.GetPlayerCharacter` 0))
  (bind _returnvalue_2 (`|CreateWidget` "/Game/Dynamic/UI/SaveLoad/WBP_SaveScreen.WBP_SaveScreen_C"))
  (`UserWidget.AddToViewport` _returnvalue_2 0)
  (`HuntStatsComponent.RecoverHealth` (`HuntPlayerCharacter.PlayerStatsComponent` (cast `HuntPlayerCharacter` _returnvalue :!pure true)) 5000.0)
  (message `HuntCharacterInterface.UpdateStatsUI` _returnvalue))

(fn `UserConstructionScript`
  (`parent.UserConstructionScript`))