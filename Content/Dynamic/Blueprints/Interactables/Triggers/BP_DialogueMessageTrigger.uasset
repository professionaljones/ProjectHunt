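; Dialogue message trigger actor that shows an overridden dialogue widget on screen when activated.
; ActivateTrigger creates the widget for the first player controller with the new dialogue and NPC actor, adds it to the viewport and gives the trigger a short life span.
; The widget's display time is tied to the actor's lifetime, as the Destroyed event removes it from its parent.
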(event `self.ActivateTrigger`
  (bind _returnvalue (`|CreateWidget` "/DialoguePlugin/UI/OverridenDialogueWidget.OverridenDialogueWidget_C" (`GameplayStatics.GetPlayerController` 0) (`self.NewDialogue`) (`self.NPCActor`)))
  (set `self.WidgetReference` _returnvalue)
  (`UserWidget.AddToViewport` _returnvalue 0)
  (`self.SetLifeSpan` 5.0))

(event `self.ReceiveDestroyed`
  (`Widget.RemoveFromParent` (`self.WidgetReference`)))

(fn `UserConstructionScript`
  (`parent.UserConstructionScript`))