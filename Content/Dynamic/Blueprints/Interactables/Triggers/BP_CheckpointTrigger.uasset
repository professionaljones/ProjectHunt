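; BP_CheckpointTrigger is a checkpoint trigger that auto-saves the game when activated.
; Its ActivateTrigger event casts the game instance to BP_ProjectHuntUGC_GameInstance and calls AsyncAutoSave.
; The construction script runs the parent's script, then sizes the Box component from the NewBoxExtent variable.
; It has no active overlap or tick logic of its own.
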(event `self.ActivateTrigger`
  (`/Game/Dynamic/Blueprints/Game/BP_ProjectHuntUGC_GameInstance.AsyncAutoSave` (cast `/Game/Dynamic/Blueprints/Game/BP_ProjectHuntUGC_GameInstance` (`GameplayStatics.GetGameInstance`) :!pure true)))

(fn `UserConstructionScript`
  (`parent.UserConstructionScript`)
  (`BoxComponent.SetBoxExtent` (`self.Box`) (`self.NewBoxExtent`) true))