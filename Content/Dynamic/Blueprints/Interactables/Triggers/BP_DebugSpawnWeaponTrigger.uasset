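; Debug interactable trigger that displays a configured weapon class and gives it to the player when activated.
; On BeginPlay it spawns an instance of NewWeapon at its transform and snaps it to the root as a visible preview.
; ActivateTrigger has BP_TrishPlayerCharacter spawn the weapon, enables debug mode on it and refreshes the player's stats UI message.
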(event `self.ReceiveBeginPlay`
  (bind _newweapon (`self.NewWeapon`))
  (`parent.ReceiveBeginPlay`)
  (if (`KismetSystemLibrary.IsValidClass` _newweapon)
    (bind _returnvalue (`|SpawnActorFromClass` _newweapon (`self.GetTransform`) "Undefined" "OverrideRootScale" null null))
    (`self.K2_AttachToComponent` _returnvalue (`self.RootComponent`) "None" "SnapToTarget" "SnapToTarget" "SnapToTarget" true)))

(event `self.ActivateTrigger`
  (bind _returnvalue (`GameplayStatics.GetPlayerCharacter` 0))
  (bind _returnvalue_2 (`/Game/Dynamic/Blueprints/Player/BP_TrishPlayerCharacter.SpawnWeapon` (cast `/Game/Dynamic/Blueprints/Player/BP_TrishPlayerCharacter` _returnvalue :!pure true) (`self.NewWeapon`)))
  (`/Game/Dynamic/Blueprints/Weapons/BP_BaseWeapon.EnableDebugMode` _returnvalue_2)
  (message `HuntCharacterInterface.UpdateStatsUI` _returnvalue))

(fn `UserConstructionScript`
  (`parent.UserConstructionScript`))