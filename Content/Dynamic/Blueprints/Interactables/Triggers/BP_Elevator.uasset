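; Elevator interactable that carries the player along configurable control points when they enter its box while it is active.
; An InterpToMovement component makes a one-shot trip, with the particle system off and player movement input disabled via an interface message.
; On stop, input and particles return; after an outbound trip, a delay precedes an automatic reverse trip, with the HasMoved flag preventing retriggers until then.
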(event `self.ReceiveBeginPlay`
  (bind _interptomovement (`self.InterpToMovement`))
  (`parent.ReceiveBeginPlay`)
  (set `InterpToMovementComponent.ControlPoints` (`self.MyControlPoints`) _interptomovement)
  (set `InterpToMovementComponent.Duration` (`self.MyDuration`) _interptomovement)
  (`InterpToMovementComponent.FinaliseControlPoints` (`self.InterpToMovement`))
  (`MovementComponent.StopMovementImmediately` (`self.InterpToMovement`))
  (`MovementComponent.StopMovementImmediately` (`self.InterpToMovement`)))

(event `self.Box.OnComponentBeginOverlap`
  (params (OverlappedComponent :type "PrimitiveComponent Object Reference") (OtherActor :type "Actor Object Reference") (OtherComp :type "PrimitiveComponent Object Reference") (OtherBodyIndex :type Integer) (bFromSweep :type Boolean) (SweepResult :type "HitResult Structure (by ref)"))
  (bind _returnvalue (`GameplayStatics.GetPlayerCharacter` 0))
  (bind _interptomovement (`self.InterpToMovement`))
  (if (== OtherActor _returnvalue)
    (if (`self.bIsActive?`)
      (if (not (`self.bHasMoved`))
        (set `self.bHasMoved` true)
        (set `InterpToMovementComponent.BehaviourType` "OneShot" _interptomovement)
        (`ActorComponent.Deactivate` (`self.ParticleSystem`))
        (`InterpToMovementComponent.RestartMovement` _interptomovement 1.0)
        (message `HuntPlayerInterface.ToggleMovementInput` _returnvalue false)))))

(event `self.InterpToMovement.OnInterpToStop`
  (params (ImpactResult :type "HitResult Structure (by ref)") (Time :type "Float (single-precision)"))
  (bind _interptomovement (`self.InterpToMovement`))
  (message `HuntPlayerInterface.ToggleMovementInput` (`GameplayStatics.GetPlayerCharacter` 0) true)
  (`ActorComponent.Activate` (`self.ParticleSystem`) true)
  (if (`self.bHasMoved`)
    (`KismetSystemLibrary.Delay` 10.0)
    (set `InterpToMovementComponent.BehaviourType` "OneShot_Reverse" _interptomovement)
    (`InterpToMovementComponent.RestartMovement` _interptomovement 1.0)
    (set `self.bHasMoved` false)))

(event `self.Box.OnComponentEndOverlap`
  (params (OverlappedComponent :type "PrimitiveComponent Object Reference") (OtherActor :type "Actor Object Reference") (OtherComp :type "PrimitiveComponent Object Reference") (OtherBodyIndex :type Integer))
  (if (== OtherActor (`GameplayStatics.GetPlayerCharacter` 0))
    _))

(fn `UserConstructionScript`
  (`parent.UserConstructionScript`))