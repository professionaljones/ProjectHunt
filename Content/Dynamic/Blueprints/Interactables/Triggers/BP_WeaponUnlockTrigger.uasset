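; Interactable trigger that unlocks a new weapon for the player when activated.
; ActivateTrigger casts player 0 to BP_TrishPlayerCharacter and calls SpawnWeapon with the NewWeapon variable.
; It then spawns a BP_PickupMessageTrigger at its own location to announce the unlock, and sets a short life span to remove itself.
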(event `self.ActivateTrigger`
  (`/Game/Dynamic/Blueprints/Player/BP_TrishPlayerCharacter.SpawnWeapon` (cast `/Game/Dynamic/Blueprints/Player/BP_TrishPlayerCharacter` (`GameplayStatics.GetPlayerCharacter` 0) :!pure true) (`self.NewWeapon`))
  (`|SpawnActorFromClass` "/Game/Dynamic/Blueprints/Interactables/Triggers/BP_PickupMessageTrigger.BP_PickupMessageTrigger_C" (`KismetMathLibrary.MakeTransform` (`self.K2_GetActorLocation`)) "Undefined" "OverrideRootScale" null "You've unlocked a new weapon!" null)
  (`self.SetLifeSpan` 3.2))

(fn `UserConstructionScript`
  (`parent.UserConstructionScript`))