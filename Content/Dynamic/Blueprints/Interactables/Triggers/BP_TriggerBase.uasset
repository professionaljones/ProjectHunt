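; Base trigger volume that fires an event when player character 0 enters or leaves its Box.
; TriggerOnBeginOverlap selects entry or exit, and ActivateTrigger broadcasts OnTriggerOverlap.
; HideObject, not called within this graph, retires the trigger by hiding it, stopping audio and disabling collision.
; It then broadcasts OnObjectHide, async-saves to the AutoSave slot through the game instance, and sets a short lifespan for delayed destruction.
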(event `self.Box.OnComponentBeginOverlap`
  (params (OverlappedComponent :type "PrimitiveComponent Object Reference") (OtherActor :type "Actor Object Reference") (OtherComp :type "PrimitiveComponent Object Reference") (OtherBodyIndex :type Integer) (bFromSweep :type Boolean) (SweepResult :type "HitResult Structure (by ref)"))
  (if (== OtherActor (`GameplayStatics.GetPlayerCharacter` 0))
    (if (`self.bTriggerOnBeginOverlap?`)
      (`self.ActivateTrigger`))))

(event `self.Box.OnComponentEndOverlap`
  (params (OverlappedComponent :type "PrimitiveComponent Object Reference") (OtherActor :type "Actor Object Reference") (OtherComp :type "PrimitiveComponent Object Reference") (OtherBodyIndex :type Integer))
  (if (== OtherActor (`GameplayStatics.GetPlayerCharacter` 0))
    (if (not (`self.bTriggerOnBeginOverlap?`))
      (`self.ActivateTrigger`))))

(fn `ActivateTrigger`
  (`self.OnTriggerOverlap`))

(fn `HideObject`
  (`self.SetActorHiddenInGame` true)
  (`AudioComponent.Stop` (`self.Audio`))
  (`PrimitiveComponent.SetCollisionEnabled` (`self.Box`) "NoCollision")
  (`self.OnObjectHide`)
  (`/Game/Dynamic/Blueprints/Game/BP_ProjectHuntUGC_GameInstance.AsyncSaveSlot` (cast `/Game/Dynamic/Blueprints/Game/BP_ProjectHuntUGC_GameInstance` (`GameplayStatics.GetGameInstance`) :!pure true) "AutoSave")
  (`self.SetLifeSpan` 3.0))

(fn `UserConstructionScript`)