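; BP_TutorialMessageTrigger_New is a trigger actor that shows a tutorial message when activated.
; ActivateTrigger creates a WBP_GameplayMessage from TutorialMessageArray, registers it as the hunt controller's LastWBP, hides the HUD and stops Trish's movement.
; After fixed delays it removes the widget, restores HUD and movement, and disables Box collision so it cannot retrigger by overlap.
; A reverse-animation step is left unconnected.
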(event `self.ActivateTrigger`
  (bind _astrish_playercharacter (cast `/Game/Dynamic/Blueprints/Player/BP_TrishPlayerCharacter` (`GameplayStatics.GetPlayerCharacter` 0) :!pure true))
  (bind _asbp_hunt_player_controller_base (cast `/Game/Dynamic/Blueprints/Player/BP_HuntPlayerController_Base` (`GameplayStatics.GetPlayerController` 0) :!pure true))
  (`/Engine/EditorBlueprintResources/StandardMacros.IsValid` (`self.MessageWBP`)
    (:`Is Not Valid`
      (`|CreateWidget` "/Game/Dynamic/UI/Gameplay/WBP_GameplayMessage.WBP_GameplayMessage_C" null 2.0 0.1 (`self.TutorialMessageArray`))
      (bind _output_get (set `self.MessageWBP` null))
      (set `/Game/Dynamic/Blueprints/Player/BP_HuntPlayerController_Base.LastWBP` _output_get _asbp_hunt_player_controller_base)
      (`UserWidget.AddToViewport` _output_get 0)
      (`/Game/Dynamic/Blueprints/Player/BP_HuntPlayerController_Base.ToggleHUDVisibility` _asbp_hunt_player_controller_base false)
      (`/Game/Dynamic/Blueprints/Player/BP_TrishPlayerCharacter.StopPlayerMovement` _astrish_playercharacter)
      (`KismetSystemLibrary.Delay` 3.0)
      (`KismetSystemLibrary.Delay` 1.0)
      (`Widget.RemoveFromParent` (`self.MessageWBP`))
      (`/Game/Dynamic/Blueprints/Player/BP_HuntPlayerController_Base.ToggleHUDVisibility` _asbp_hunt_player_controller_base true)
      (`/Game/Dynamic/Blueprints/Player/BP_TrishPlayerCharacter.StartPlayerMovement` _astrish_playercharacter)
      (`PrimitiveComponent.SetCollisionEnabled` (`self.Box`) "NoCollision"))))

(fn `UserConstructionScript`
  (`parent.UserConstructionScript`))