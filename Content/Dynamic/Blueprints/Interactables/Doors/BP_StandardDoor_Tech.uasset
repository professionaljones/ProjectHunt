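; Tech variant of a standard interactable door, supplying its own opening motion and activation effect to the parent door logic.
; On BeginPlay it hands its two timelines to parent variables and sets an initial materialize value on the dynamic material.
; The door timeline drives the door's relative Z position and world Z scale, calling OnDoorLock on finish if locked.
; The activation timeline animates the materialize parameter.
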(event `self.ReceiveBeginPlay`
  (`parent.ReceiveBeginPlay`)
  (set `self.InputTimeline` (`self.TechDoorTimeline`))
  (set `self.InputActivationTimeline` (`self.TechDoorActivateTimeline`))
  (`MaterialInstanceDynamic.SetScalarParameterValue` (`self.DynMat`) (`self.MaterializeName`) 0.54))

(fn `UserConstructionScript`
  (`parent.UserConstructionScript`))