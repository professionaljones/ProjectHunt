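; Base door that opens when shot by the player's weapon, either as a standard door or only for matching Incendiary, Ice or Shock ammo.
; A one-second looping timer caches the player's current weapon, which damage events compare against the damage causer.
; Opening and closing play or reverse a supplied timeline with sounds; mismatched ammo plays a locked sound.
; The door closes when the player leaves its box trigger.
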(event `self.ReceiveBeginPlay`
  (bind _returnvalue (`KismetSystemLibrary.K2_SetTimerDelegate` (delegate `CheckForWeapon`) 1.0 true))
  (set `self.checkTimer` _returnvalue))

(event `CheckForWeapon`
  (bind _ashunt_player_character (cast `HuntPlayerCharacter` (`GameplayStatics.GetPlayerCharacter` 0) :!pure true))
  (`/Engine/EditorBlueprintResources/StandardMacros.IsValid` _ashunt_player_character
    (:`Is Valid`
      (set `self.PC_Weapon` (`ProjectHuntCharacter.CurrentWeapon` _ashunt_player_character)))
    (:`Is Not Valid`
      (`KismetSystemLibrary.K2_ClearAndInvalidateTimerHandle` (`self.checkTimer`)))))

(event `self.ReceiveAnyDamage`
  (params (Damage :type "Float (single-precision)") (DamageType :type "DamageType Object Reference") (InstigatedBy :type "Controller Object Reference") (DamageCauser :type "Actor Object Reference"))
  (if (== DamageCauser (`self.PC_Weapon`))
    (`self.ActivateDoor` (`self.InputTimeline`))))

(event `self.Box.OnComponentEndOverlap`
  (params (OverlappedComponent :type "PrimitiveComponent Object Reference") (OtherActor :type "Actor Object Reference") (OtherComp :type "PrimitiveComponent Object Reference") (OtherBodyIndex :type Integer))
  (if (== OtherActor (`GameplayStatics.GetPlayerPawn` 0))
    (if (`self.bShouldOpenDoor?`)
      (`self.CloseDoor` (`self.InputTimeline`)))))

(fn `ActivateDoor`
  (params (DoorTimeline :type "TimelineComponent Object Reference"))
  (bind _returnvalue (`HuntWeapon.GetWeaponAmmoType` (`self.PC_Weapon`)))
  (`self.CheckDoorStatus` _returnvalue DoorTimeline))

(fn `CheckDoorStatus`
  (params (AmmoUsed :type "EAmmoType Enum" :default "AT_Standard") (DoorTimeline :type "TimelineComponent Object Reference"))
  (bind _requireddoortype (`self.RequiredDoorType`))
  (if (`self.bIsStandardDoor?`)
    (`self.OpenDoor` DoorTimeline)
    (else
      (switch `EAmmoType` AmmoUsed
        (:`AT_Fire`
          (if (`|EnumEquality` AmmoUsed _requireddoortype)
            (`self.OpenDoor` DoorTimeline)
            (else
              (`self.OnDoorLock`))))
        (:`AT_Ice`
          (if (`|EnumEquality` AmmoUsed _requireddoortype)
            (`self.OpenDoor` DoorTimeline)
            (else
              (`self.OnDoorLock`))))
        (:`AT_Shock`
          (if (`|EnumEquality` AmmoUsed _requireddoortype)
            (`self.OpenDoor` DoorTimeline)
            (else
              (`self.OnDoorLock`))))))))

(fn `CloseDoor`
  (params (DoorTimeline :type "TimelineComponent Object Reference"))
  (set `self.bShouldOpenDoor?` false)
  (`TimelineComponent.ReverseFromEnd` DoorTimeline)
  (`GameplayStatics.PlaySoundAtLocation` (`self.DoorCloseSound`) (`self.K2_GetActorLocation`) (struct) 1.0 1.0 0.0 null null null))

(fn `OnDoorLock`
  (`GameplayStatics.PlaySoundAtLocation` (`self.DoorLockedSound`) (`self.K2_GetActorLocation`) (struct) 1.0 1.0 0.0 null null null))

(fn `OpenDoor`
  (params (DoorTimeline :type "TimelineComponent Object Reference"))
  (set `self.bShouldOpenDoor?` true)
  (`TimelineComponent.PlayFromStart` DoorTimeline)
  (`GameplayStatics.PlaySoundAtLocation` (`self.DoorOpenSound`) (`self.K2_GetActorLocation`) (struct) 1.0 1.0 0.0 null null null))

(fn `UserConstructionScript`)