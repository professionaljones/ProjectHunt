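; Test door Blueprint that reacts to damage by printing whether it would open, without actually opening.
; AnyDamage casts the damage type to BP_DT_Base and switches on its WeaponType.
; Explosives print an agreement to open, while pistol, rifle and shotgun share a refusal message.
; BeginPlay, overlap and Tick are disabled stubs, and the construction script only calls its parent.
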(event `/Game/Dynamic/Blueprints/Interactables/Doors/BP_DoorBase.ReceiveAnyDamage`
  (params (Damage :type "Float (single-precision)") (DamageType :type "DamageType Object Reference") (InstigatedBy :type "Controller Object Reference") (DamageCauser :type "Actor Object Reference"))
  (switch `EWeaponType` (`/Game/Dynamic/Blueprints/Weapons/BP_DT_Base.WeaponType` (cast `/Game/Dynamic/Blueprints/Weapons/BP_DT_Base` DamageType :!pure true))
    (:`WT_Explosive`
      (`KismetSystemLibrary.PrintString` "Okay, I will open for you!"))
    (:`WT_Pistol`
      (`KismetSystemLibrary.PrintString` "No, I refuse to open for you!" :!label _label))
    (:`WT_Rifle`
      (goto _label))
    (:`WT_Shotgun`
      (goto _label))))

(fn `UserConstructionScript`
  (`parent.UserConstructionScript`))