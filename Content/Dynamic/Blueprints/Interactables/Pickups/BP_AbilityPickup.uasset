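; Ability pickup that permanently unlocks one player upgrade: wallrun, dash, Aragon core or missile launcher.
; When triggered, it shows a pickup message, sets the matching flag in the player's saved stats, saves to the manual slot and hides itself.
; The missile launcher case also updates missile capacity.
; It exposes its GUID and picked-up state for saving, and destroys itself when told it was already collected.
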(event `self.ActivateTrigger`
  (bind _ashunt_player_character (cast `HuntPlayerCharacter` (`GameplayStatics.GetPlayerCharacter` 0) :!pure true))
  (bind _asbp_project_hunt_ugc_game_instance (cast `/Game/Dynamic/Blueprints/Game/BP_ProjectHuntUGC_GameInstance` (`GameplayStatics.GetGameInstance`) :!pure true))
  (bind _playersavedstats (`HuntPlayerCharacter.PlayerSavedStats` _ashunt_player_character))
  (switch `string` (`self.AbilityToModifiy`)
    (:`Wallrun Ability`
      (bind _returnvalue (`|CreateWidget` "/Game/Dynamic/UI/Gameplay/WBP_PickupMessage.WBP_PickupMessage_C" null "Wallrun upgrade: Acquired!"))
      (`UserWidget.AddToViewport` _returnvalue 0)
      (setmembers `PlayerSaveableStats` :`StructRef` _playersavedstats :`bUnlockedWallrun` true))
    (:`Dash Ability`
      (bind _returnvalue_2 (`|CreateWidget` "/Game/Dynamic/UI/Gameplay/WBP_PickupMessage.WBP_PickupMessage_C" null "Dash upgrade: Acquired!"))
      (`UserWidget.AddToViewport` _returnvalue_2 0)
      (setmembers `PlayerSaveableStats` :`StructRef` _playersavedstats :`bUnlockedDash` true))
    (:`Aragon`
      (bind _returnvalue_3 (`|CreateWidget` "/Game/Dynamic/UI/Gameplay/WBP_PickupMessage.WBP_PickupMessage_C" null "Aragon core:  Activated!"))
      (`UserWidget.AddToViewport` _returnvalue_3 0)
      (setmembers `PlayerSaveableStats` :`StructRef` _playersavedstats :`bUnlockedAragon` true))
    (:`Missile Launcher`
      (bind _returnvalue_4 (`|CreateWidget` "/Game/Dynamic/UI/Gameplay/WBP_PickupMessage.WBP_PickupMessage_C" null "Missile Launcher: Activated!"))
      (`UserWidget.AddToViewport` _returnvalue_4 0)
      (setmembers `PlayerSaveableStats` :`StructRef` _playersavedstats :`bHasMissileLauncher` true)
      (`HuntPlayerCharacter.UpdateMissileCapacity` _ashunt_player_character 5)))
  (message `/Game/Dynamic/Blueprints/Player/BPI_PlayerUserInterface.OnGameSave` (`GameplayStatics.GetPlayerController` 0))
  (`/Game/Dynamic/Blueprints/Game/BP_ProjectHuntUGC_GameInstance.AsyncSaveSlot` _asbp_project_hunt_ugc_game_instance (`/Game/Dynamic/Blueprints/Game/BP_ProjectHuntUGC_GameInstance.ManualSlotName` _asbp_project_hunt_ugc_game_instance))
  (`self.HideObject`))

(event `/Game/Examples/UC/-PersistentVariables/BPI_Saveable.DidInteractWith`
  (params (InteractedWith :type Boolean))
  (bind _output_get (set `self.bDidPlayerPickupItem?` InteractedWith))
  (if _output_get
    (`self.K2_DestroyActor`)))

(fn `GetSaveableValues`
  (returns (ID :type "Guid Structure") (InteractedWith :type Boolean))
  (return (`self.PickupGUID`) (`self.bDidPlayerPickupItem?`)))

(fn `UserConstructionScript`
  (`parent.UserConstructionScript`))