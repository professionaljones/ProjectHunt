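; Base Blueprint for a missile pickup that replenishes the player's missiles.
; When ActivateTrigger fires, it passes NewRecoverAmount to RecoverMissiles on player character 0, cast to HuntPlayerCharacter, then sends that character a stats UI update.
; It then plays the pickup sound at its own location and destroys itself.
; BeginPlay, overlap and Tick are disabled stubs, and the construction script only calls its parent.
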(event `self.ActivateTrigger`
  (bind _returnvalue (`GameplayStatics.GetPlayerCharacter` 0))
  (`HuntPlayerCharacter.RecoverMissiles` (cast `HuntPlayerCharacter` _returnvalue :!pure true) (`self.NewRecoverAmount`))
  (message `HuntCharacterInterface.UpdateStatsUI` _returnvalue)
  (`GameplayStatics.PlaySoundAtLocation` (`self.MissilePickupSFX`) (`self.K2_GetActorLocation`) (struct) 1.0 1.0 0.0 null null null)
  (`self.K2_DestroyActor`))

(fn `UserConstructionScript`
  (`parent.UserConstructionScript`))