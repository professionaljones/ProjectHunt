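; Base Blueprint for pickup interactables that remembers whether the player has picked up the item.
; An interaction event stores that flag and hides the object when it is true.
; A RamaSave component hides it again once the actor fully loads, if the flag is set.
; A setter and a saveable-values getter expose the flag, while construction-script GUID regeneration logic is left unconnected.
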(event `self.ReceiveBeginPlay`
  (`parent.ReceiveBeginPlay`))

(event `/Game/Examples/UC/-PersistentVariables/BPI_Saveable.DidInteractWith`
  (params (InteractedWith :type Boolean))
  (bind _output_get (set `self.bDidPlayerPickupItem?` InteractedWith))
  (if _output_get
    (`self.HideObject`)))

(event `self.RamaSave.RamaSaveEvent_ActorFullyLoaded`
  (params (RamaSaveComponent :type "RamaSaveComponent Object Reference") (LevelPackageName :type String))
  (if (`self.bDidPlayerPickupItem?`)
    (`self.HideObject`)))

(fn `GetSaveableValues`
  (returns (ID :type "Guid Structure") (InteractedWith :type Boolean))
  (return (struct) (`self.bDidPlayerPickupItem?`)))

(fn `SetPlayerPickupStatus`
  (params (`bDidPlayerPickupItem?` :type Boolean))
  (set `self.bDidPlayerPickupItem?` `bDidPlayerPickupItem?`))

(fn `UserConstructionScript`
  (`parent.UserConstructionScript`))