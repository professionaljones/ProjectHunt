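; Data-point pickup base that passes its DPModAmount to player zero and destroys itself when ActivateTrigger fires.
; BeginPlay starts a fast looping timer, though the function it binds is not shown.
; AttractToPlayer sphere-traces along the forward vector with debug drawing, then moves the pickup by sweep to a point interpolated from the impact point toward the hit actor, rather than from its own location.
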(event `self.ReceiveBeginPlay`
  (`parent.ReceiveBeginPlay`)
  (`KismetSystemLibrary.K2_SetTimerDelegate` (`|CreateDelegate` :!event `AttractToPlayer`) 0.01 true))

(event `self.ActivateTrigger`
  (message `HuntCharacterInterface.UpdatePlayerDataPoints` (`GameplayStatics.GetPlayerCharacter` 0) (`self.DPModAmount`))
  (`self.K2_DestroyActor`))

(fn `AttractToPlayer`
  (bind _returnvalue (`self.K2_GetActorLocation`))
  (bind _outhit (`KismetSystemLibrary.SphereTraceSingleForObjects` :`Start` _returnvalue :`End` (+ _returnvalue (* (`KismetMathLibrary.GetForwardVector` (`self.K2_GetActorRotation`)) 8000.0)) :`Radius` 360.0 :`ObjectTypes` (`|MakeArray` "ObjectTypeQuery9" :!type "EObjectTypeQuery Enum") :`bTraceComplex` true :`DrawDebugType` "ForDuration"))
  (bind (_bblockinghit _binitialoverlap _time _distance _location _impactpoint _normal _impactnormal _physmat _hitactor) (`GameplayStatics.BreakHitResult` _outhit))
  (if _bblockinghit
    (`/Engine/EditorBlueprintResources/StandardMacros.IsValid` _hitactor
      (:`Is Valid`
        (`self.K2_SetActorLocation` (`KismetMathLibrary.VInterpTo` _impactpoint (`self.K2_GetActorLocation` _hitactor) (`GameplayStatics.GetWorldDeltaSeconds`) 25.0) true)))))

(fn `UserConstructionScript`
  (`parent.UserConstructionScript`))