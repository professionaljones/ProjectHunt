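; Pickup that upgrades the player's Aragon stats and announces an energy increase.
; On trigger activation, it passes the upgrade amount to the player's stats component and refreshes the stats UI.
; It then fades out its audio, reports the pickup to the player, hides itself and shows a message widget.
; When destroyed, it spawns a healing-leaf particle effect at its location.
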(event `self.ActivateTrigger`
  (bind _returnvalue (`GameplayStatics.GetPlayerCharacter` 0))
  (`HuntStatsComponent.UpgradeAragonStats` (`HuntPlayerCharacter.PlayerStatsComponent` (cast `HuntPlayerCharacter` _returnvalue :!pure true)) (`self.NewUpgradeAmount`))
  (message `HuntCharacterInterface.UpdateStatsUI` _returnvalue)
  (`AudioComponent.FadeOut` (`self.Audio`) 3.2 0.0 "Linear")
  (message `HuntPlayerInterface.OnPlayerPickupItem` _returnvalue (`self.fPlayerCollectionMod`))
  (set `self.bDidPlayerPickupItem?` true)
  (`self.HideObject`)
  (bind _returnvalue_2 (`|CreateWidget` "/Game/Dynamic/UI/Gameplay/WBP_PickupMessage.WBP_PickupMessage_C" null "Your energy has been increased!"))
  (`UserWidget.AddToViewport` _returnvalue_2 0))

(event `self.ReceiveEndPlay`
  (params (EndPlayReason :type "EEndPlayReason Enum" :default "Destroyed"))
  (switch `EEndPlayReason` EndPlayReason
    (:`Destroyed`
      (`GameplayStatics.SpawnEmitterAtLocation` "/Game/Static/VFX_Toolkit_V1/ParticleSystems/356Days/Par_HealLeaf_01.Par_HealLeaf_01" (`self.K2_GetActorLocation`)))))

(fn `UserConstructionScript`
  (`parent.UserConstructionScript`))