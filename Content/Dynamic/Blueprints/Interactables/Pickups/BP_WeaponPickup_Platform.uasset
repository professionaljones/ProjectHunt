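; Weapon pickup platform that displays a rotating, firing preview of its configured weapon class.
; On BeginPlay it spawns the weapon, attaches it to a Scene component driven by RotatingMovement, and starts a looping timer, apparently meant for FireNewWeapon.
; FireNewWeapon assigns the player character as weapon owner and spawns a projectile.
; The graph holds no overlap or pickup logic.
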(event `self.ReceiveBeginPlay`
  (bind _scene (`self.Scene`))
  (bind _returnvalue (`|SpawnActorFromClass` (`self.WeaponToPickup`) (`SceneComponent.K2_GetComponentToWorld` _scene) "Undefined" "OverrideRootScale" null null))
  (set `self.PickupWeapon` _returnvalue)
  (`self.K2_AttachToComponent` _returnvalue _scene "None" "SnapToTarget" "SnapToTarget" "KeepRelative" true)
  (`MovementComponent.SetUpdatedComponent` (`self.RotatingMovement`) (`self.Scene`))
  (`KismetSystemLibrary.K2_SetTimerDelegate` (`|CreateDelegate` :!event `FireNewWeapon`) 2.0 true))

(event `FireNewWeapon`
  (bind _pickupweapon (`self.PickupWeapon`))
  (`HuntWeapon.SetWeaponOwner` _pickupweapon (cast `ProjectHuntCharacter` (`GameplayStatics.GetPlayerCharacter` 0) :!pure true))
  (`/Game/Dynamic/Blueprints/Weapons/BP_BaseWeapon.SpawnProjectile` _pickupweapon))

(fn `UserConstructionScript`)