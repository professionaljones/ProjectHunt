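; Base health pickup Blueprint that restores the player's health when its trigger is activated.
; ActivateTrigger casts player character 0 to HuntPlayerCharacter, recovers health through its StatsComponent and fires the HUD update delegate.
; It then plays the pickup sound at its location and destroys itself only if DidPlayerTriggerEvent is false.
; BeginPlay, overlap and Tick are disabled stubs, and this graph contains no trigger detection.
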(event `/Game/Dynamic/Blueprints/Interactables/Triggers/BP_TriggerBase.ActivateTrigger`
  (bind _ashunt_player_character (cast `HuntPlayerCharacter` (`GameplayStatics.GetPlayerCharacter` 0) :!pure true))
  (`HuntStatsComponent.RecoverHealth` (`ProjectHuntCharacter.StatsComponent` _ashunt_player_character) (`self.NewRecoverAmount`))
  (`HuntPlayerCharacter.UpdatePlayerHUD_Delegate` _ashunt_player_character)
  (`GameplayStatics.PlaySoundAtLocation` (`self.HealthPickupSFX`) (`self.K2_GetActorLocation`) (struct) 1.0 1.0 0.0 null null null)
  (if (not (`self.bDidPlayerTriggerEvent?`))
    (`self.K2_DestroyActor`)))

(fn `UserConstructionScript`
  (`parent.UserConstructionScript`))