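; Base pickup for data points, which pulls itself toward a nearby target and pays out when the player touches it.
; BeginPlay starts a fast looping timer, presumably for AttractToPlayer, which sphere-traces by object type and sweeps the pickup from the impact point toward the hit actor.
; When the player overlaps the Sphere, it passes DPModAmount to the player's data points update, plays a sound and destroys itself.
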(event `self.ReceiveBeginPlay`
  (`parent.ReceiveBeginPlay`)
  (`KismetSystemLibrary.K2_SetTimerDelegate` (`|CreateDelegate` :!event `AttractToPlayer`) 0.1 true))

(event `self.ActivateTrigger`)

(event `self.Sphere.OnComponentBeginOverlap`
  (params (OverlappedComponent :type "PrimitiveComponent Object Reference") (OtherActor :type "Actor Object Reference") (OtherComp :type "PrimitiveComponent Object Reference") (OtherBodyIndex :type Integer) (bFromSweep :type Boolean) (SweepResult :type "HitResult Structure (by ref)"))
  (bind _returnvalue (`GameplayStatics.GetPlayerCharacter` 0))
  (if (== OtherActor _returnvalue)
    (message `HuntCharacterInterface.UpdatePlayerDataPoints` _returnvalue (`self.DPModAmount`))
    (`GameplayStatics.PlaySound2D` "/Game/Static/Audio/SFX/Player/PM_FN_Objects_Items_Interactions_Menus_12.PM_FN_Objects_Items_Interactions_Menus_12" 1.0 1.0 0.0 null null)
    (`self.K2_DestroyActor`)))

(fn `AttractToPlayer`
  (bind _returnvalue (`self.K2_GetActorLocation`))
  (bind _outhit (`KismetSystemLibrary.SphereTraceSingleForObjects` _returnvalue (+ _returnvalue (* _returnvalue 2000.0)) 750.0 (`|MakeArray` "ObjectTypeQuery9" :!type "EObjectTypeQuery Enum") true))
  (bind (_bblockinghit _binitialoverlap _time _distance _location _impactpoint _normal _impactnormal _physmat _hitactor) (`GameplayStatics.BreakHitResult` _outhit))
  (if _bblockinghit
    (`/Engine/EditorBlueprintResources/StandardMacros.IsValid` _hitactor
      (:`Is Valid`
        (`self.K2_SetActorLocation` (`KismetMathLibrary.VInterpTo` _impactpoint (`self.K2_GetActorLocation` _hitactor) (`GameplayStatics.GetWorldDeltaSeconds`) 25.0) true)))))

(fn `UserConstructionScript`
  (`parent.UserConstructionScript`))