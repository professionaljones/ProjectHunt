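; Suit pickup interactable that gives the player a new suit when triggered.
; ActivateTrigger sets the suit on the player character and refreshes the stats UI.
; With a valid game state saveable manager, it records the interaction, hides itself and shows an energy-increase message; otherwise it only prints an unsaved-status error, leaving the pickup visible.
; Saveable values and interaction-state handling defer to the parent.
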(event `self.ActivateTrigger`
  (bind _returnvalue (`GameplayStatics.GetPlayerCharacter` 0))
  (bind _saveablemanagerreference (`/Game/Dynamic/Blueprints/Game/BP_ProjectHuntGameStateBase.SaveableManagerReference` (cast `/Game/Dynamic/Blueprints/Game/BP_ProjectHuntGameStateBase` (`GameplayStatics.GetGameState`) :!pure true)))
  (`HuntPlayerCharacter.SetPlayerSuit` (cast `HuntPlayerCharacter` _returnvalue :!pure true) (`self.NewPlayerSuit`))
  (message `HuntCharacterInterface.UpdateStatsUI` _returnvalue)
  (`/Engine/EditorBlueprintResources/StandardMacros.IsValid` _saveablemanagerreference
    (:`Is Valid`
      (`/Game/Examples/UC/-PersistentVariables/BP_SaveableObjectManager.UpdateSaveableObjectArray` _saveablemanagerreference self true)
      (`self.HideObject`)
      (bind _returnvalue_2 (`|CreateWidget` "/Game/Dynamic/UI/Gameplay/WBP_PickupMessage.WBP_PickupMessage_C" null "Your energy has been increased!" null))
      (`UserWidget.AddToViewport` _returnvalue_2 0))
    (:`Is Not Valid`
      (`KismetSystemLibrary.PrintString` "Saveable manager not valid; STATUS NOT SAVED" true true (struct :`R` 1.0 :`A` 1.0) 30.0))))

(event `/Game/Examples/UC/-PersistentVariables/BPI_Saveable.DidInteractWith`
  (params (InteractedWith :type Boolean))
  (`parent.DidInteractWith` InteractedWith))

(fn `GetSaveableValues`
  (returns (ID :type "Guid Structure") (InteractedWith :type Boolean))
  (bind (_id _interactedwith) (`parent.GetSaveableValues`))
  (return _id _interactedwith))

(fn `UserConstructionScript`
  (`parent.UserConstructionScript`))