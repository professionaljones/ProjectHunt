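; Missile launcher pickup that grants the player missile capacity when triggered, for players who cannot yet use missiles.
; ActivateTrigger checks the HuntPlayerCharacter, raises its missile capacity, calls the game instance's save-game message and flags the item as picked up.
; DidInteractwith sets that flag from its input and destroys the actor if true; ActivateTrigger itself does not destroy it.
; An UnlockAbility call is left unconnected.
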(event `/Game/Dynamic/Blueprints/Interactables/Triggers/BP_TriggerBase.ActivateTrigger`
  (bind _ashunt_player_character (cast `HuntPlayerCharacter` (`GameplayStatics.GetPlayerCharacter` 0) :!pure true))
  (if (not (`HuntPlayerCharacter.CanPlayerUseMissiles` _ashunt_player_character))
    (`HuntPlayerCharacter.UpdateMissileCapacity` _ashunt_player_character 5)
    (message `/Game/Dynamic/Blueprints/Game/BPI_GameData.OnPlayerSaveGame` (`GameplayStatics.GetGameInstance`))
    (set `self.bDidPlayerPickupItem?` true)))

(event `/Game/Examples/UC/-PersistentVariables/BPI_Saveable.DidInteractWith`
  (params (InteractedWith :type Boolean))
  (bind _output_get (set `self.bDidPlayerPickupItem?` InteractedWith))
  (if _output_get
    (`self.K2_DestroyActor`)))

(fn `UserConstructionScript`
  (`parent.UserConstructionScript`))