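; Weapon unlock pickup that grants the player a new weapon when its trigger activates.
; On activation it spawns the configured weapon on the Trish player character and shows an unlock message widget.
; It then records itself as interacted with in the game state's saveable manager and hides itself.
; Without a valid manager it prints a not-saved error and stays visible.
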(event `self.ActivateTrigger`
  (bind _saveablemanagerreference (`/Game/Dynamic/Blueprints/Game/BP_ProjectHuntGameStateBase.SaveableManagerReference` (cast `/Game/Dynamic/Blueprints/Game/BP_ProjectHuntGameStateBase` (`GameplayStatics.GetGameState`) :!pure true)))
  (`/Game/Dynamic/Blueprints/Player/BP_TrishPlayerCharacter.SpawnWeapon` (cast `/Game/Dynamic/Blueprints/Player/BP_TrishPlayerCharacter` (`GameplayStatics.GetPlayerCharacter` 0) :!pure true) (`self.NewWeapon`))
  (bind _returnvalue (`|CreateWidget` "/Game/Dynamic/UI/Gameplay/WBP_PickupMessage.WBP_PickupMessage_C" null "You've unlocked a new weapon!"))
  (`UserWidget.AddToViewport` _returnvalue 0)
  (`/Engine/EditorBlueprintResources/StandardMacros.IsValid` _saveablemanagerreference
    (:`Is Valid`
      (`/Game/Examples/UC/-PersistentVariables/BP_SaveableObjectManager.UpdateSaveableObjectArray` _saveablemanagerreference self true)
      (`self.HideObject`))
    (:`Is Not Valid`
      (`KismetSystemLibrary.PrintString` "Saveable manager not valid; STATUS NOT SAVED" true true (struct :`R` 1.0 :`A` 1.0) 30.0))))

(fn `UserConstructionScript`
  (`parent.UserConstructionScript`))