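; A health upgrade pickup that permanently raises the player's health stats when triggered.
; Activation upgrades the stats component, shows a timed message widget, autosaves, fades its audio, then destroys itself with a leaf particle burst.
; A construction-time GUID and interacted flag feed the saveable manager, so collected pickups remove themselves when their saved state is restored.
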(event `self.ReceiveBeginPlay`
  (`parent.ReceiveBeginPlay`))

(event `self.ActivateTrigger`
  (bind _returnvalue (`GameplayStatics.GetPlayerCharacter` 0))
  (bind _saveablemanagerreference (`/Game/Dynamic/Blueprints/Game/BP_ProjectHuntGameStateBase.SaveableManagerReference` (cast `/Game/Dynamic/Blueprints/Game/BP_ProjectHuntGameStateBase` (`GameplayStatics.GetGameState`) :!pure true)))
  (`HuntStatsComponent.UpgradeHealthStats` (`ProjectHuntCharacter.StatsComponent` (cast `ProjectHuntCharacter` _returnvalue :!pure true)) (`self.NewRecoverAmount`))
  (message `HuntCharacterInterface.UpdateStatsUI` _returnvalue)
  (bind _returnvalue_2 (`|CreateWidget` "/Game/Dynamic/UI/WBP_PickupMessage.WBP_PickupMessage_C" null "Your energy has been increased!"))
  (`UserWidget.AddToViewport` _returnvalue_2 0)
  (`/Game/Dynamic/Blueprints/Game/BP_ProjectHuntGameInstance.AsyncSaveSlot` (cast `/Game/Dynamic/Blueprints/Game/BP_ProjectHuntGameInstance` (`GameplayStatics.GetGameInstance`) :!pure true) "AutoSave")
  (`AudioComponent.FadeOut` (`self.Audio`) 3.2 0.0 "Linear")
  (`|ExecutionSequence`
    (:`then_0`
      (`/Engine/EditorBlueprintResources/StandardMacros.IsValid` _saveablemanagerreference
        (:`Is Valid`
          (`/Game/Examples/UC/-PersistentVariables/BP_SaveableObjectManager.UpdateSaveableObjectArray` _saveablemanagerreference self true))))
    (:`then_1`
      (`KismetSystemLibrary.Delay` 3.0)
      (`Widget.RemoveFromParent` _returnvalue_2)
      (`PrimitiveComponent.SetCollisionEnabled` (`self.Box`) "NoCollision")
      (`self.K2_DestroyActor`))))

(event `self.ReceiveEndPlay`
  (params (EndPlayReason :type "EEndPlayReason Enum" :default "Destroyed"))
  (switch `EEndPlayReason` EndPlayReason
    (:`Destroyed`
      (`GameplayStatics.SpawnEmitterAtLocation` "/Game/Static/VFX_Toolkit_V1/ParticleSystems/356Days/Par_HealLeaf_01.Par_HealLeaf_01" (`self.K2_GetActorLocation`)))))

(event `/Game/Examples/UC/-PersistentVariables/BPI_Saveable.DidInteractWith`
  (params (InteractedWith :type Boolean))
  (bind _output_get (set `self.bWasInteractedWith` InteractedWith))
  (if _output_get
    (`self.K2_DestroyActor`)))

(event `self.ReceiveDestroyed`
  (bind _saveablemanagerreference (`/Game/Dynamic/Blueprints/Game/BP_ProjectHuntGameStateBase.SaveableManagerReference` (cast `/Game/Dynamic/Blueprints/Game/BP_ProjectHuntGameStateBase` (`GameplayStatics.GetGameState`) :!pure true)))
  (`/Engine/EditorBlueprintResources/StandardMacros.IsValid` _saveablemanagerreference
    (:`Is Valid`
      (`/Game/Examples/UC/-PersistentVariables/BP_SaveableObjectManager.SaveAllTheThings` _saveablemanagerreference))))

(fn `GetSaveableValues`
  (returns (ID :type "Guid Structure") (InteractedWith :type Boolean))
  (return (`self.GUID`) (`self.bWasInteractedWith`)))

(fn `UserConstructionScript`
  (if (not (`KismetGuidLibrary.IsValid_Guid` (`self.GUID`)))
    (set `self.GUID` (`KismetGuidLibrary.NewGuid`))))