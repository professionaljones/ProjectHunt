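; Interactable powered wall that is solid when powered and has no collision when unpowered.
; DidInteractwith(true) powers it; CheckPowerStatus then enables collision and plays a timeline driving "Materialize Amount" on trim and base dynamic materials.
; It reports its state to the game state's saveable manager, with GetSaveableValues exposing GUID and interaction flag.
; Timeline completion re-runs CheckPowerStatus, restarting it while powered; the status timer setup is unconnected.
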(event `self.ReceiveBeginPlay`
  (bind _staticmesh (`self.StaticMesh`))
  (if (`self.bIsPowered?`)
    (`PrimitiveComponent.SetCollisionEnabled` _staticmesh "QueryAndPhysics")
    (else
      (`PrimitiveComponent.SetCollisionEnabled` _staticmesh "NoCollision"))))

(event `/Game/Examples/UC/-PersistentVariables/BPI_Saveable.DidInteractWith`
  (params (InteractedWith :type Boolean))
  (bind _output_get (set `self.InteractedWith` InteractedWith))
  (if _output_get
    (set `self.bIsPowered?` true)
    (`self.CheckPowerStatus`)))

(fn `CheckPowerStatus`
  (bind _staticmesh (`self.StaticMesh`))
  (bind _saveablemanagerreference (`/Game/Dynamic/Blueprints/Game/BP_ProjectHuntGameStateBase.SaveableManagerReference` (cast `/Game/Dynamic/Blueprints/Game/BP_ProjectHuntGameStateBase` (`GameplayStatics.GetGameState`) :!pure true)))
  (if (`self.bIsPowered?`)
    (`TimelineComponent.PlayFromStart` (`self.PoweredTimeline`))
    (`PrimitiveComponent.SetCollisionEnabled` _staticmesh "QueryAndPhysics")
    (`/Engine/EditorBlueprintResources/StandardMacros.IsValid` _saveablemanagerreference
      (:`Is Valid`
        (`/Game/Examples/UC/-PersistentVariables/BP_SaveableObjectManager.UpdateSaveableObjectArray` _saveablemanagerreference self (`self.bIsPowered?`))
        (`KismetSystemLibrary.K2_ClearAndInvalidateTimerHandle` (`self.StatusTimer`)))
      (:`Is Not Valid`
        (`KismetSystemLibrary.PrintString` "Game state not valid; STATUS NOT SAVED" true true (struct :`R` 1.0 :`A` 1.0) 30.0)))
    (else
      (`PrimitiveComponent.SetCollisionEnabled` _staticmesh "NoCollision"))))

(fn `GetSaveableValues`
  (returns (ID :type "Guid Structure") (InteractedWith :type Boolean))
  (return (`self.ActorGUID`) (`self.InteractedWith`)))

(fn `UserConstructionScript`
  (bind _staticmesh (`self.StaticMesh`))
  (bind _returnvalue (`PrimitiveComponent.CreateDynamicMaterialInstance` _staticmesh 0 (`PrimitiveComponent.GetMaterial` _staticmesh 0) "None"))
  (bind _output_get (set `self.DynMat_Trims` _returnvalue))
  (bind _returnvalue_2 (`PrimitiveComponent.CreateDynamicMaterialInstance` _staticmesh 1 (`PrimitiveComponent.GetMaterial` _staticmesh 1) "None"))
  (bind _output_get_2 (set `self.DynMat_Base` _returnvalue_2))
  (`MaterialInstanceDynamic.SetScalarParameterValue` _output_get "Materialize Amount" (`self.MatAmount_Trims`))
  (`MaterialInstanceDynamic.SetScalarParameterValue` _output_get_2 "Materialize Amount" (`self.MatAmount_Base`)))