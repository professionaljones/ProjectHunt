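; Explosive barrel hazard that takes damage through a HuntStats component, catches fire when low on health and explodes on death.
; AnyDamage ignores self-inflicted damage, spawns a fire emitter on every hit below half health, then calls Explode if dead.
; Explode applies radial damage with falloff, plays particles and sound, and sets a short lifespan.
; Construction script and Explode draw debug spheres for inner and outer damage radii.
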(event `self.ReceiveBeginPlay`
  (bind _huntstats (`self.HuntStats`))
  (`parent.ReceiveBeginPlay`)
  (set `HuntStatsComponent.CurrentHealth` (`HuntStatsComponent.GetMaxHealth` _huntstats) _huntstats))

(event `self.ReceiveAnyDamage`
  (params (Damage :type "Float (single-precision)") (DamageType :type "DamageType Object Reference") (InstigatedBy :type "Controller Object Reference") (DamageCauser :type "Actor Object Reference"))
  (bind _huntstats (`self.HuntStats`))
  (bind _returnvalue (`HuntStatsComponent.GetHealthPercentage` _huntstats))
  (if (!= DamageCauser self)
    (`HuntStatsComponent.DamageHealth` (`self.HuntStats`) Damage)
    (`KismetSystemLibrary.PrintString` (`KismetStringLibrary.Conv_DoubleToString` _returnvalue))
    (if (< _returnvalue 0.5)
      (`GameplayStatics.SpawnEmitterAtLocation` "/Game/Static/MobileStarterContent/Particles/P_Fire.P_Fire" (`SceneComponent.K2_GetComponentLocation` (`self.Scene`)) (struct) (1.0 1.0 1.0) true "AutoRelease")
      (if (`HuntStatsComponent.bIsDead` _huntstats)
        (`self.Explode` (`self.BaseDamage`) (`self.MinimumDamage`) (`self.DamageInnerRadius`) (`self.DamageOuterRadius`) (`self.DamageFalloff`))))))

(fn `Explode`
  (params (BaseDamage :type "Float (double-precision)") (MinimumDamage :type "Float (double-precision)") (DamageInnerRadius :type "Float (double-precision)") (DamageOuterRadius :type "Float (double-precision)") (DamageFalloff :type "Float (double-precision)"))
  (bind _returnvalue (`self.K2_GetActorLocation`))
  (bind _returnvalue_2 (`self.K2_GetActorLocation`))
  (`GameplayStatics.ApplyRadialDamageWithFalloff` :`BaseDamage` BaseDamage :`MinimumDamage` MinimumDamage :`Origin` _returnvalue_2 :`DamageInnerRadius` DamageInnerRadius :`DamageOuterRadius` DamageOuterRadius :`DamageFalloff` DamageFalloff :`DamageCauser` self :`InstigatedByController` null)
  (`GameplayStatics.SpawnEmitterAtLocation` "/Game/Static/MobileStarterContent/Particles/P_Explosion.P_Explosion" _returnvalue_2)
  (`GameplayStatics.PlaySoundAtLocation` "/Game/Static/MobileStarterContent/Audio/Explosion_Cue.Explosion_Cue" _returnvalue_2 (struct) 1.0 1.0 0.0 null null null)
  (`self.SetLifeSpan` 3.0)
  (`KismetSystemLibrary.DrawDebugSphere` _returnvalue DamageInnerRadius 12 (struct :`R` 1.0 :`A` 1.0) 15.0 4.0)
  (`KismetSystemLibrary.DrawDebugSphere` _returnvalue DamageOuterRadius 12 (struct :`G` 1.0 :`A` 1.0) 15.0 2.0))

(fn `UserConstructionScript`
  (bind _returnvalue (`self.K2_GetActorLocation`))
  (`parent.UserConstructionScript`)
  (`KismetSystemLibrary.DrawDebugSphere` _returnvalue (`self.DamageInnerRadius`) 12 (struct :`R` 1.0 :`A` 1.0) 15.0 4.0)
  (`KismetSystemLibrary.DrawDebugSphere` _returnvalue (`self.DamageOuterRadius`) 12 (struct :`G` 1.0 :`A` 1.0) 15.0 2.0))