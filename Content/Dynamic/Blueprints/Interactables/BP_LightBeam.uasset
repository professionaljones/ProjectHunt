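; BP_LightBeam is an interactable light beam actor that shows a colored Niagara beam with an adjustable charge length.
; AdjustBeamLength lerps the beam end between starting and charged lengths by Alpha, activating the beam and particle lifetime looping near full charge.
; An object line trace runs at BeginPlay and every Tick while active, drawing debug lines; its result is unused.
; The trace end scales location plus forward vector together, rather than only the direction.
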(event `self.ReceiveBeginPlay`
  (bind _returnvalue (`self.K2_GetActorLocation`))
  (`KismetSystemLibrary.LineTraceSingleForObjects` :`Start` _returnvalue :`End` (* (+ _returnvalue (`KismetMathLibrary.GetForwardVector` (`self.K2_GetActorRotation`))) 2000.0) :`ObjectTypes` (`self.ObjectTypes`) :`bTraceComplex` true :`DrawDebugType` "ForDuration" :!label _label))

(event `self.ReceiveTick`
  (params (DeltaSeconds :type "Float (single-precision)"))
  (if (`self.bIsActive?`)
    (goto _label)))

(fn `AdjustBeamLength`
  (params (Alpha :type "Float (double-precision)"))
  (bind _niagara (`self.Niagara`))
  (`NiagaraComponent.SetVariableVec3` (`self.Niagara`) "BeamEndLength" (`KismetMathLibrary.VLerp` (`self.StartingBeamLength`) (`self.ChargedBeamLength`) Alpha))
  (bind _output_get (set `self.bIsActive?` (>= Alpha 0.99)))
  (if _output_get
    (`NiagaraComponent.SetVariableBool` _niagara "bShouldLoopParticlesLifetime" true)
    (else
      (`NiagaraComponent.SetVariableBool` _niagara "bShouldLoopParticlesLifetime" false))))

(fn `UserConstructionScript`
  (`NiagaraComponent.SetVariableLinearColor` (`self.Niagara`) "BeamColor" (`self.BeamColor`)))