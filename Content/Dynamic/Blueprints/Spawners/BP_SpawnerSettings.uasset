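; Interactable settings actor that chooses which enemy class its connected spawner spawns.
; On BeginPlay it fills a unique list of valid enemy classes from GetEnemiesForSpawner.
; Interacting plays a fanfare and, on Normal Mode difficulty, sets ConnectedSpawner's ActorToSpawn to a random pick from the first three entries, or None if invalid.
; The validity check and the assignment roll separately, so the assigned class can differ from the checked one.
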(event `self.ReceiveBeginPlay`
  (bind _enemyarray (`/Game/Dynamic/Blueprints/Game/BPFL_GameData.GetEnemiesForSpawner`))
  (for _array_element _enemyarray
    (bind _output (`|ConvertAsset` _array_element))
    (if (`KismetSystemLibrary.IsValidClass` _output)
      (`KismetArrayLibrary.Array_AddUnique` (`self.Enemies`) _output))))

(event `HuntCharacterInterface.OnInteract`
  (bind _connectedspawner (`self.ConnectedSpawner`))
  (bind _output (`|GetArrayItem` (`self.Enemies`) (`KismetMathLibrary.RandomIntegerInRange` 0 2)))
  (`GameplayStatics.PlaySound2D` "/Game/Static/Audio/SFX/397353__plasterbrain__tada-fanfare-g.397353__plasterbrain__tada-fanfare-g" 1.0 1.0 0.0 null null)
  (switch `EGameDifficulty` (`self.SpawnerDifficulty`)
    (:`GD_Normal`
      (if (`KismetSystemLibrary.IsValidClass` _output)
        (set `/Game/Dynamic/Blueprints/Spawners/BP_BaseRespawner.ActorToSpawn` _output _connectedspawner)
        (else
          (set `/Game/Dynamic/Blueprints/Spawners/BP_BaseRespawner.ActorToSpawn` null _connectedspawner))))))

(fn `UserConstructionScript`)