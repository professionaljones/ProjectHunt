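; Trigger volume that sends the player back to a checkpoint position on overlap.
; It stores the player's location shortly after BeginPlay as the default return point.
; With LoadSavePosition set, it async-loads the AutoSave slot and uses the saved position, acting only if the saved level matches the current one.
; After moving the player it counts the use, plays a sound, and calls the Trish character's spawn and suit-power-deactivated handlers.
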(event `self.ReceiveBeginPlay`
  (bind _returnvalue (`GameplayStatics.GetPlayerCharacter` 0))
  (`KismetSystemLibrary.Delay` 0.2)
  (`/Engine/EditorBlueprintResources/StandardMacros.IsValid` _returnvalue
    (:`Is Valid`
      (set `self.StartLocation` (`self.K2_GetActorLocation` _returnvalue)))))

(event `self.Box.OnComponentBeginOverlap`
  (params (OverlappedComponent :type "PrimitiveComponent Object Reference") (OtherActor :type "Actor Object Reference") (OtherComp :type "PrimitiveComponent Object Reference") (OtherBodyIndex :type Integer) (bFromSweep :type Boolean) (SweepResult :type "HitResult Structure (by ref)"))
  (bind _returnvalue (`GameplayStatics.GetPlayerCharacter` 0))
  (bind _astrish_playercharacter (cast `/Game/Dynamic/Blueprints/Player/BP_TrishPlayerCharacter` _returnvalue :!pure true))
  (if (== OtherActor _returnvalue)
    (if (`self.bLoadSavePosition?`)
      (bind _returnvalue_2 (`GameplayStatics.DoesSaveGameExist` "AutoSave"))
      (if _returnvalue_2
        (bind _savegame (`AsyncActionHandleSaveGame.AsyncLoadGameFromSlot` "AutoSave")
          (:`Completed`
            (bind _asbp_project_hunt_save_game (cast `/Game/Dynamic/Blueprints/Game/Save_Load/BP_ProjectHuntSaveGame` _savegame))
            (bind _returnvalue_3 (`GameplayStatics.GetCurrentLevelName` true))
            (if (`KismetStringLibrary.EqualEqual_StrStr` _returnvalue_3 (`/Game/Dynamic/Blueprints/Game/Save_Load/BP_ProjectHuntSaveGame.Save_LevelName` _asbp_project_hunt_save_game))
              (bind _output_get (set `self.StartLocation` (.location (`/Game/Dynamic/Blueprints/Game/Save_Load/BP_ProjectHuntSaveGame.Save_PlayerTransform` _asbp_project_hunt_save_game))))
              (`self.K2_SetActorLocation` (`GameplayStatics.GetPlayerCharacter` 0) _output_get false false)
              (`/Engine/EditorBlueprintResources/StandardMacros.IncrementInt` (`self.TimesUsed`)
                (:`  `
                  (`GameplayStatics.PlaySound2D` "/Game/Static/Audio/SFX/QuicksilverSelectFX.QuicksilverSelectFX" 1.0 1.0 0.0 null null)
                  (`/Engine/EditorBlueprintResources/StandardMacros.IsValid` _astrish_playercharacter :!label _label
                    (:`Is Valid`
                      (`/Game/Dynamic/Blueprints/Player/BP_TrishPlayerCharacter.OnPlayerSpawn` _astrish_playercharacter)
                      (`/Game/Dynamic/Blueprints/Player/BP_TrishPlayerCharacter.OnSuitPowerDeactivated` _astrish_playercharacter)))))))))
      (else
        (`self.K2_SetActorLocation` _returnvalue (`self.StartLocation`) false false)
        (`/Engine/EditorBlueprintResources/StandardMacros.IncrementInt` (`self.TimesUsed`)
          (:`  `
            (`GameplayStatics.PlaySound2D` "/Game/Static/Audio/SFX/QuicksilverSelectFX.QuicksilverSelectFX" 1.0 1.0 0.0 null null)
            (goto _label)))))))

(fn `UserConstructionScript`)