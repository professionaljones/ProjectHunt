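; Base spawner actor that spawns a set class or a random enemy at its own transform, immediately or on a timer.
; On BeginPlay it caches the game instance's enemy array and optionally spawns at start, then schedules a delayed spawn.
; Random spawns fall back to the Grunt enemy when the picked class is invalid.
; A debug widget shows the timer countdown; without debugging, the widget and tick switch off.
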(event `self.ReceiveBeginPlay`
  (bind _widget (`self.Widget`))
  (set `self.EnemyArray` (`/Game/Dynamic/Blueprints/Game/BP_ProjectHuntUGC_GameInstance.EnemyArray` (cast `/Game/Dynamic/Blueprints/Game/BP_ProjectHuntUGC_GameInstance` (`GameplayStatics.GetGameInstance`) :!pure true)))
  (if (`self.bDebugSpawner?`)
    (bind _returnvalue (`|CreateWidget` "/Game/Dynamic/UI/Debug/WBP_SpawnerDetails.WBP_SpawnerDetails_C"))
    (bind _output_get (set `self.DetailsWBP` _returnvalue))
    (`WidgetComponent.SetWidget` _widget _output_get)
    (else
      (`ActorComponent.Deactivate` (`self.Widget`))
      (`WidgetComponent.SetWidget` _widget null)))
  (if (`self.bSpawnOnStart?`)
    (`self.SpawnActor`)
    (if (`self.bShouldSpawnOnDelay?`)
      (`self.SpawnOnDelay`))))

(event `self.ReceiveTick`
  (params (DeltaSeconds :type "Float (single-precision)"))
  (if (`self.bDebugSpawner?`)
    (`TextBlock.SetText` (`/Game/Dynamic/UI/Debug/WBP_SpawnerDetails.SpawnTimeText` (`self.DetailsWBP`)) (`KismetTextLibrary.Conv_StringToText` (`KismetStringLibrary.TimeSecondsToString` (`KismetSystemLibrary.K2_GetTimerRemainingTimeHandle` (`self.SpawnerHandle`)))))
    (else
      (`self.SetActorTickEnabled` false))))

(event `self.ReceiveDestroyed`
  (`KismetSystemLibrary.K2_ClearAndInvalidateTimerHandle` (`self.SpawnerHandle`)))

(fn `SpawnActor`
  (returns (ReturnValue :type "Actor Object Reference"))
  (bind _returnvalue (`|SpawnActorFromClass` (`self.ActorToSpawn`) (`self.GetTransform`) "AdjustIfPossibleButAlwaysSpawn" "OverrideRootScale" null null))
  (`/Engine/EditorBlueprintResources/StandardMacros.IsValid` _returnvalue
    (:`Is Valid`
      (`/Engine/EditorBlueprintResources/StandardMacros.IsValid` (`self.GetComponentByClass` _returnvalue "/Script/ProjectHunt.HuntStatsComponent")
        (:`Is Valid`
          (return _returnvalue))))
    (:`Is Not Valid`
      (return null))))

(fn `SpawnActor_Timer`
  (bind _returnvalue (`KismetSystemLibrary.IsValid` (`self.DetailsWBP`)))
  (bind _enemynametext (`/Game/Dynamic/UI/Debug/WBP_SpawnerDetails.EnemyNameText` (`self.DetailsWBP`)))
  (bind _returnvalue_2 (`|SpawnActorFromClass` (`self.ActorToSpawn`) (`self.GetTransform`) "AdjustIfPossibleButAlwaysSpawn" "OverrideRootScale" null null))
  (`/Engine/EditorBlueprintResources/StandardMacros.IsValid` (`self.GetComponentByClass` _returnvalue_2 "/Script/ProjectHunt.HuntStatsComponent")
    (:`Is Valid`
      (if _returnvalue
        (`TextBlock.SetText` _enemynametext (`KismetTextLibrary.Conv_StringToText` ""))))
    (:`Is Not Valid`
      (if _returnvalue
        (`TextBlock.SetText` _enemynametext (`KismetTextLibrary.Conv_StringToText` (`KismetSystemLibrary.GetDisplayName` _returnvalue_2)))))))

(fn `SpawnOnDelay`
  (bind _returnvalue (`KismetSystemLibrary.K2_SetTimerDelegate` (`|CreateDelegate` :!event `SpawnActor_Timer`) (`self.TimerDelay`) (`self.bLoopTimer`)))
  (set `self.SpawnerHandle` _returnvalue))

(fn `SpawnRandomActor`
  (bind _enemyarray (`self.EnemyArray`))
  (bind _output (`|ConvertAsset` (`|GetArrayItem` _enemyarray (`KismetMathLibrary.RandomIntegerInRange` 0 (`KismetArrayLibrary.Array_Length` _enemyarray)))))
  (if (`KismetSystemLibrary.IsValidClass` _output)
    (set `self.ActorToSpawn` _output)
    (`self.SpawnActor`)
    (else
      (set `self.ActorToSpawn` "/Game/Dynamic/Blueprints/Enemies/Humanoid/BP_EnemyCharacter_Grunt.BP_EnemyCharacter_Grunt_C")
      (`self.SpawnActor`)
      (`KismetSystemLibrary.PrintString` "INVALID ACTOR FROM ARRAY"))))

(fn `SpawnRandomActor_Timer`
  (bind _enemyarray (`self.EnemyArray`))
  (bind _output (`|ConvertAsset` (`|GetArrayItem` _enemyarray (`KismetMathLibrary.RandomIntegerInRange` 0 (`KismetArrayLibrary.Array_Length` _enemyarray)))))
  (if (`KismetSystemLibrary.IsValidClass` _output)
    (set `self.ActorToSpawn` _output)
    (`self.SpawnActor`)
    (else
      (set `self.ActorToSpawn` "/Game/Dynamic/Blueprints/Enemies/Humanoid/BP_EnemyCharacter_Grunt.BP_EnemyCharacter_Grunt_C")
      (`self.SpawnActor`)
      (`KismetSystemLibrary.PrintString` "INVALID ACTOR FROM ARRAY"))))

(fn `SpawnRandomOnDelay`
  (bind _returnvalue (`KismetSystemLibrary.K2_SetTimerDelegate` (`|CreateDelegate` :!event `SpawnRandomActor_Timer`) (`self.TimerDelay`) (`self.bLoopTimer`)))
  (set `self.SpawnerHandle` _returnvalue))

(fn `UserConstructionScript`)