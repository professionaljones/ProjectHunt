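; Base enemy respawner that spawns a configurable actor class at its own transform on a timer, optionally looping or spawning once immediately at start.
; BeginPlay creates a WBP_SpawnerDetails widget for its widget component and starts the timer, which is cleared on destruction.
; Tick writes the remaining time to the widget.
; SpawnActor labels it with the spawned actor's HuntStatsComponent character name, falling back to its display name.
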(event `self.ReceiveBeginPlay`
  (bind _returnvalue (`|CreateWidget` "/Game/Dynamic/UI/Debug/WBP_SpawnerDetails.WBP_SpawnerDetails_C"))
  (bind _output_get (set `self.DetailsWBP` _returnvalue))
  (`WidgetComponent.SetWidget` (`self.Widget`) _output_get)
  (bind _returnvalue_2 (`KismetSystemLibrary.K2_SetTimerDelegate` (`|CreateDelegate` :!event `SpawnActor`) (`self.TimerRate`) (`self.bLoopTimer`)))
  (set `self.SpawnerHandle` _returnvalue_2)
  (if (`self.bSpawnOnStart?`)
    (`self.SpawnActor`)))

(event `self.ReceiveTick`
  (params (DeltaSeconds :type "Float (single-precision)"))
  (`TextBlock.SetText` (`/Game/Dynamic/UI/Debug/WBP_SpawnerDetails.SpawnTimeText` (`self.DetailsWBP`)) (`KismetTextLibrary.Conv_StringToText` (`KismetStringLibrary.TimeSecondsToString` (`KismetSystemLibrary.K2_GetTimerRemainingTimeHandle` (`self.SpawnerHandle`))))))

(event `self.ReceiveDestroyed`
  (`KismetSystemLibrary.K2_ClearAndInvalidateTimerHandle` (`self.SpawnerHandle`)))

(fn `SpawnActor`
  (bind _returnvalue (`KismetSystemLibrary.IsValid` (`self.DetailsWBP`)))
  (bind _enemynametext (`/Game/Dynamic/UI/Debug/WBP_SpawnerDetails.EnemyNameText` (`self.DetailsWBP`)))
  (bind _returnvalue_2 (`|SpawnActorFromClass` (`self.ActorToSpawn`) (`self.GetTransform`) "AdjustIfPossibleButAlwaysSpawn" "OverrideRootScale" null null))
  (bind _returnvalue_3 (`self.GetComponentByClass` _returnvalue_2 "/Script/ProjectHunt.HuntStatsComponent"))
  (`/Engine/EditorBlueprintResources/StandardMacros.IsValid` _returnvalue_3
    (:`Is Valid`
      (if _returnvalue
        (`TextBlock.SetText` _enemynametext (`KismetTextLibrary.Conv_StringToText` (`HuntStatsComponent.CharacterName` _returnvalue_3)))))
    (:`Is Not Valid`
      (if _returnvalue
        (`TextBlock.SetText` _enemynametext (`KismetTextLibrary.Conv_StringToText` (`KismetSystemLibrary.GetDisplayName` _returnvalue_2)))))))

(fn `UserConstructionScript`)