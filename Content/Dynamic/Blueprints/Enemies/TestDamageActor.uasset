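; TestDamageActor is an enemy test actor that takes damage, explodes at zero health and responds to scanning.
; A HuntStats component holds health, death and scan state, with health filled from MaxHealth at BeginPlay and reduced by AnyDamage.
; Explode disables damage, plays an explosion effect and sound, then sets a short lifespan to remove the actor.
; OnTargetScanned records the first scan, and debug prints report damage and scans.
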(event `self.ReceiveBeginPlay`
  (set `HuntStatsComponent.CurrentHealth` (`self.MaxHealth`) (`self.HuntStats`)))

(event `self.ReceiveAnyDamage`
  (params (Damage :type "Float (single-precision)") (DamageType :type "DamageType Object Reference") (InstigatedBy :type "Controller Object Reference") (DamageCauser :type "Actor Object Reference"))
  (if (not (`HuntStatsComponent.bIsDead` (`self.HuntStats`)))
    (`|ExecutionSequence`
      (:`then_0`
        (`HuntStatsComponent.DamageHealth` (`self.HuntStats`) Damage)
        (`KismetSystemLibrary.PrintString` (`KismetStringLibrary.Concat_StrStr` "Damage taken: " " " (`KismetStringLibrary.Conv_DoubleToString` Damage)))
        (if (<= (`HuntStatsComponent.CurrentHealth` (`self.HuntStats`)) 0.0)
          (`self.Explode`))))))

(event `Explode`
  (bind _returnvalue (`self.K2_GetActorLocation`))
  (set `self.bCanBeDamaged` false)
  (`GameplayStatics.SpawnEmitterAtLocation` "/Game/Static/MobileStarterContent/Particles/P_Explosion.P_Explosion" _returnvalue)
  (`GameplayStatics.PlaySoundAtLocation` "/Game/Static/MobileStarterContent/Audio/Explosion_Cue.Explosion_Cue" _returnvalue (struct) 1.0 1.0 0.0 null null null)
  (`PrimitiveComponent.SetCollisionEnabled` (`self.StaticMesh`) "QueryAndPhysics")
  (`self.SetLifeSpan` 0.35))

(event `HuntCharacterInterface.OnTargetScanned`
  (params (bWasPreviouslyScanned :type Boolean))
  (bind _huntstats (`self.HuntStats`))
  (if (`HuntStatsComponent.bWasScanned` _huntstats)
    (`KismetSystemLibrary.PrintString` "I've been scanned before!")
    (else
      (`KismetSystemLibrary.PrintString` "I've been scanned!")
      (set `HuntStatsComponent.bWasScanned` true _huntstats))))

(fn `UserConstructionScript`)