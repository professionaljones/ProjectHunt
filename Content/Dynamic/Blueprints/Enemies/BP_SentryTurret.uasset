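; Sentry turret enemy that detects the player ahead, turns to face them and fires sentry projectiles.
; BeginPlay starts a fast looping timer, and SeekNewTarget sphere-traces forward with per-frame debug drawing, using a Delay to space out shots.
; Damage feeds the HuntStats health, and death triggers an explosion effect and sound before a short lifespan removes the actor.
; An idle-rotation timeline is left disconnected and never runs.
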(event `self.ReceiveBeginPlay`
  (`KismetSystemLibrary.K2_SetTimerDelegate` (`|CreateDelegate` :!event `SeekNewTarget`) 0.01 true)
  (set `HuntStatsComponent.CurrentHealth` (`self.MaxHealth`) (`self.HuntStats`)))

(event `SeekNewTarget`
  (bind _returnvalue (`self.K2_GetActorLocation`))
  (bind _returnvalue_2 (`GameplayStatics.GetPlayerCharacter` 0))
  (bind (_returnvalue_roll _returnvalue_pitch _returnvalue_yaw) (`KismetMathLibrary.BreakRotator` (`KismetMathLibrary.RInterpTo` (`self.K2_GetActorRotation`) (`KismetMathLibrary.FindLookAtRotation` (`self.K2_GetActorLocation`) (`self.K2_GetActorLocation` _returnvalue_2)) (`GameplayStatics.GetWorldDeltaSeconds`))))
  (bind (_outhit _returnvalue_3) (`KismetSystemLibrary.SphereTraceSingleForObjects` :`Start` _returnvalue :`End` (+ _returnvalue (* (`KismetMathLibrary.GetForwardVector` (`self.K2_GetActorRotation`)) 2000.0)) :`Radius` 90.0 :`ObjectTypes` (`|MakeArray` "ObjectTypeQuery9" :!type "EObjectTypeQuery Enum") :`bTraceComplex` true :`DrawDebugType` "ForOneFrame"))
  (if _returnvalue_3
    (`|ExecutionSequence`
      (:`then_1`
        (if (== (`.HitActor` (`GameplayStatics.BreakHitResult` _outhit)) _returnvalue_2)
          (`self.K2_SetActorRotation` (`KismetMathLibrary.MakeRotator` 0.0 _returnvalue_pitch _returnvalue_yaw))
          (`KismetSystemLibrary.Delay` 0.5)
          (`|SpawnActorFromClass` "/Game/Dynamic/Blueprints/Weapons/Projectiles/BP_SentryProjectile.BP_SentryProjectile_C" (`KismetMathLibrary.MakeTransform` (`self.K2_GetActorLocation`) (`self.K2_GetActorRotation`)) "Undefined" "OverrideRootScale" null 5.0 null))))))

(event `self.ReceiveAnyDamage`
  (params (Damage :type "Float (single-precision)") (DamageType :type "DamageType Object Reference") (InstigatedBy :type "Controller Object Reference") (DamageCauser :type "Actor Object Reference"))
  (bind _huntstats (`self.HuntStats`))
  (`HuntStatsComponent.DamageHealth` _huntstats Damage)
  (`KismetSystemLibrary.PrintString` (`KismetStringLibrary.Conv_DoubleToString` (`HuntStatsComponent.GetCurrentHealth` _huntstats)))
  (if (`HuntStatsComponent.bIsDead` _huntstats)
    (`self.Explode`)))

(event `Explode`
  (bind _returnvalue (`self.K2_GetActorLocation`))
  (`GameplayStatics.SpawnEmitterAtLocation` "/Game/Static/MobileStarterContent/Particles/P_Explosion.P_Explosion" _returnvalue)
  (`GameplayStatics.PlaySoundAtLocation` "/Game/Static/MobileStarterContent/Audio/Explosion_Cue.Explosion_Cue" _returnvalue (struct) 1.0 1.0 0.0 null null null)
  (`self.SetLifeSpan` 2.0))

(fn `UserConstructionScript`)