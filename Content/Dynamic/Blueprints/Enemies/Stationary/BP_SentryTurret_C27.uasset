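; BP_SentryTurret_C27 is a stationary enemy sentry turret, so far containing only an unfinished target-detection probe.
; Each Tick it sphere-traces from the turret mesh along the actor's forward vector out to TargetSearchRange, against one custom object type with per-frame debug drawing.
; The hit result is unused, so no targeting, aiming or firing follows, and the construction script only calls its parent.
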(event `self.ReceiveTick`
  (params (DeltaSeconds :type "Float (single-precision)"))
  (bind _returnvalue (`SceneComponent.K2_GetComponentLocation` (`self.ScifiTurret_SM_Turret_L`)))
  (bind _outhit (`KismetSystemLibrary.SphereTraceSingleForObjects` :`Start` _returnvalue :`End` (+ _returnvalue (* (`KismetMathLibrary.GetForwardVector` (`self.K2_GetActorRotation`)) (`self.TargetSearchRange`))) :`Radius` (`self.TraceRadius`) :`ObjectTypes` (`|MakeArray` "ObjectTypeQuery9" :!type "EObjectTypeQuery Enum") :`bTraceComplex` true :`DrawDebugType` "ForOneFrame" :`TraceColor` (struct :`R` 1.0 :`G` 0.873857 :`A` 1.0) :`TraceHitColor` (struct :`R` 0.510077 :`B` 1.0 :`A` 1.0))))

(fn `UserConstructionScript`
  (`parent.UserConstructionScript`))