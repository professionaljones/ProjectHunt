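; Base humanoid enemy character for arena combat, with a spawned weapon, lock-on widget and player-rank-based damage scaling.
; BeginPlay sets up health, dynamic material and weapon, then mirrors health into the AI blackboard, which also receives traced cover points.
; Damage reactions start timer-driven burning, freeze via time dilation and paused AI logic, or handle death.
; EndPlay awards arena points and, when destroyed, drops randomized pickups.
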(event `HuntCharacterInterface.OnFindCover`
  (bind (_outlocation _outrotation) (`self.GetActorEyesViewPoint`))
  (bind _outhit (`KismetSystemLibrary.LineTraceSingleForObjects` :`Start` _outlocation :`End` (+ _outlocation (* (`KismetMathLibrary.GetForwardVector` _outrotation) 1200.0)) :`ObjectTypes` (`|MakeArray` "ObjectTypeQuery2" :!type "EObjectTypeQuery Enum") :`bTraceComplex` true :`DrawDebugType` "ForDuration"))
  (bind (_bblockinghit _binitialoverlap _time _distance _location _impactpoint _normal _impactnormal _physmat _hitactor) (`GameplayStatics.BreakHitResult` _outhit))
  (`/Engine/EditorBlueprintResources/StandardMacros.IsValid` _hitactor
    (:`Is Valid`
      (if (and _bblockinghit (`self.ActorHasTag` _hitactor "Cover"))
        (`BlackboardComponent.SetValueAsVector` (`self.MyBlackboard`) "PatrolLocation" _impactpoint)))))

(event `self.ReceiveBeginPlay`
  (bind _statscomponent (`self.StatsComponent`))
  (bind _maxstarthealth (`self.MaxStartHealth`))
  (bind _mesh (`self.Mesh`))
  (bind _weapontospawn (`self.WeaponToSpawn`))
  (bind _returnvalue (`AIBlueprintHelperLibrary.GetAIController` self))
  (`HuntCharacterInterface.OnPlayerLockOn` false)
  (set `HuntStatsComponent.MaxHealth` _maxstarthealth _statscomponent)
  (set `HuntStatsComponent.CurrentHealth` _maxstarthealth _statscomponent)
  (add `self.UpdateHealthStats` (`|CreateDelegate` :!event `UpdatePlayerRankInfo`))
  (`self.UpdateDifficultyReference`)
  (`|ExecutionSequence`
    (:`then_0`
      (`/Engine/EditorBlueprintResources/StandardMacros.IsValid` _mesh
        (:`Is Valid`
          (bind _returnvalue_2 (`PrimitiveComponent.CreateDynamicMaterialInstance` _mesh 0 (`PrimitiveComponent.GetMaterial` _mesh 0) "None"))
          (set `self.Mesh_DynMat` _returnvalue_2)
          (`TimelineComponent.PlayFromStart` (`self.Timeline_0`)))))
    (:`then_1`
      (set `self.ArenaPointsToAdd` 10))
    (:`then_2`
      (if (`KismetSystemLibrary.IsValidClass` _weapontospawn)
        (bind _returnvalue_3 (`|SpawnActorFromClass` _weapontospawn (`KismetMathLibrary.MakeTransform` (0.0 0.0 0.0)) "Undefined" "OverrideRootScale" null (`Controller.K2_GetPawn` (`AIBlueprintHelperLibrary.GetAIController` self))))
        (bind _output_get (set `self.CurrentWeapon` _returnvalue_3))
        (`SceneComponent.K2_AttachToComponent` (`HuntWeapon.WeaponMeshTP` _output_get) (`self.Mesh`) "GripPoint" "KeepRelative" "KeepRelative" "KeepRelative" true)
        (`/Game/Dynamic/Blueprints/Weapons/BP_BaseWeapon.OnSpawn` (cast `/Game/Dynamic/Blueprints/Weapons/BP_BaseWeapon` _output_get :!pure true))
        (`HuntWeapon.SetWeaponOwner` _output_get (cast `ProjectHuntCharacter` (`self.GetInstigator`) :!pure true))))
    (:`then_3`
      (bind _returnvalue_4 (`KismetSystemLibrary.K2_SetTimerDelegate` (`|CreateDelegate` :!event `FireDamage`) 1.0 true))
      (bind _output_get_2 (set `self.FireTimer` _returnvalue_4))
      (`KismetSystemLibrary.K2_PauseTimerHandle` _output_get_2)
      (`/Engine/EditorBlueprintResources/StandardMacros.IsValid` _returnvalue
        (:`Is Valid`
          (bind _output_get_3 (set `self.MyAIController` _returnvalue))
          (bind _returnvalue_5 (`AIBlueprintHelperLibrary.GetBlackboard` _output_get_3))
          (bind _output_get_4 (set `self.MyBlackboard` _returnvalue_5))
          (`BlackboardComponent.SetValueAsFloat` _returnvalue_5 (`self.HealthKey`) (`HuntStatsComponent.GetCurrentHealth` (`self.StatsComponent`)))
          (`BlackboardComponent.SetValueAsFloat` _output_get_4 (`self.HealthKey`) (`HuntStatsComponent.GetCurrentHealth` (`self.StatsComponent`)))
          (`self.UpdateBlackboardStats`)
          (add `self.UpdateHealthStats` (`|CreateDelegate` :!event `UpdateBlackboardStats`))
          (if (== "/Game/Dynamic/Blueprints/Game/BP_ProjectHuntGameStateBase_Arena.BP_ProjectHuntGameStateBase_Arena" (`GameplayStatics.GetGameState`))
            _))))))

(event `self.ReceiveAnyDamage`
  (params (Damage :type "Float (single-precision)") (DamageType :type "DamageType Object Reference") (InstigatedBy :type "Controller Object Reference") (DamageCauser :type "Actor Object Reference"))
  (`parent.ReceiveAnyDamage` Damage DamageType InstigatedBy DamageCauser)
  (`AISense_Damage.ReportDamageEvent` DamageCauser InstigatedBy Damage (`self.K2_GetActorLocation` InstigatedBy) (`self.K2_GetActorLocation`)))

(event `self.ReactToDamage`
  (params (WeaponUsed :type "HuntWeapon Object Reference"))
  (`self.BP React To Damage` WeaponUsed))

(event `self.ReceiveEndPlay`
  (params (EndPlayReason :type "EEndPlayReason Enum" :default "Destroyed"))
  (bind _returnvalue (`self.K2_GetActorLocation`))
  (message `HuntGameInterface.OnPlayerArenaKill` (`GameplayStatics.GetGameState`) (`self.GetArenaPointsToAdd`))
  (switch `EEndPlayReason` EndPlayReason
    (:`Destroyed`
      (`|SpawnActorFromClass` "/Game/Dynamic/Blueprints/Interactables/Pickups/BP_DP_Pickup_Low.BP_DP_Pickup_Low_C" (`KismetMathLibrary.MakeTransform` (`self.K2_GetActorLocation`)) "Undefined" "OverrideRootScale" null null)
      (if (`KismetMathLibrary.RandomBool`)
        (if (`KismetMathLibrary.RandomBoolWithWeight` 0.65)
          (`|SpawnActorFromClass` "/Game/Dynamic/Blueprints/Interactables/Pickups/BP_HealthPickup_Low.BP_HealthPickup_Low_C" (`KismetMathLibrary.MakeTransform` _returnvalue) "Undefined" "OverrideRootScale" null null)
          (else
            (`|SpawnActorFromClass` "/Game/Dynamic/Blueprints/Interactables/Pickups/BP_HealthPickup_Medium.BP_HealthPickup_Medium_C" (`KismetMathLibrary.MakeTransform` _returnvalue) "Undefined" "OverrideRootScale" null null)))
        (elif (`KismetMathLibrary.RandomBoolWithWeight` 0.72)
          (`|SpawnActorFromClass` "/Game/Dynamic/Blueprints/Interactables/Pickups/BP_MissilePickup_Low.BP_MissilePickup_Low_C" (`KismetMathLibrary.MakeTransform` _returnvalue) "Undefined" "OverrideRootScale" null null)
          (else
            (`|SpawnActorFromClass` "/Game/Dynamic/Blueprints/Interactables/Pickups/BP_MissilePickup_Medium.BP_MissilePickup_Medium_C" (`KismetMathLibrary.MakeTransform` (0.0 0.0 0.0)) "Undefined" "OverrideRootScale" null null)))))))

(event `FireDamage`
  (`HuntStatsComponent.DamageHealth` (`self.StatsComponent`) 5.0))

(event `OnIceDamage`
  (if (`self.bIsFrozen?`)
    (set `self.bIsFrozen?` false)
    (set `self.CustomTimeDilation` 1.0)
    (`BrainComponent.RestartLogic` (`AIController.BrainComponent` (`AIBlueprintHelperLibrary.GetAIController` self)))
    (else
      (set `self.bIsFrozen?` true)
      (set `self.CustomTimeDilation` 0.0)
      (`BrainComponent.StopLogic` (`AIController.BrainComponent` (`AIBlueprintHelperLibrary.GetAIController` self)) "Actor Frozen")
      (`HuntWeapon.EndFire` (`self.GetCurrentWeapon`))
      (`KismetSystemLibrary.Delay` 10.0)
      (set `self.bIsFrozen?` false))))

(event `HuntCharacterInterface.OnAttackTarget`
  (bind _returnvalue (`self.GetCurrentWeapon`))
  (`/Engine/EditorBlueprintResources/StandardMacros.IsValid` _returnvalue
    (:`Is Valid`
      (set `HuntWeapon.WeaponProjectileState` "Projectile_Normal" _returnvalue)
      (`KismetSystemLibrary.K2_SetTimerDelegate` (delegate `EnemyFire`) (`.FireRate` (break `WeaponStatsData` (`HuntWeapon.WeaponStatsData` _returnvalue))) true))))

(event `EnemyFire`
  (bind _returnvalue (`self.GetCurrentWeapon`))
  (`/Engine/EditorBlueprintResources/StandardMacros.IsValid` _returnvalue
    (:`Is Valid`
      (message `HuntWeaponInterface.OnWeaponFire` _returnvalue))))

(event `UpdateBlackboardStats`
  (bind _statscomponent (`self.StatsComponent`))
  (bind _myblackboard (`self.MyBlackboard`))
  (`/Engine/EditorBlueprintResources/StandardMacros.IsValid` _myblackboard
    (:`Is Valid`
      (`BlackboardComponent.SetValueAsFloat` _myblackboard (`self.HealthKey`) (`HuntStatsComponent.GetCurrentHealth` _statscomponent))
      (`BlackboardComponent.SetValueAsFloat` _myblackboard (`self.HealthPercentKey`) (`HuntStatsComponent.GetHealthPercentage` _statscomponent)))))

(event `HuntCharacterInterface.OnPlayerLockOn`
  (params (bIsLockedOn :type Boolean))
  (bind _lockonwidget (`self.LockOnWidget`))
  (if bIsLockedOn
    (`SceneComponent.SetVisibility` _lockonwidget true false)
    (else
      (`SceneComponent.SetVisibility` _lockonwidget false false))))

(fn `BP React To Damage`
  (params (WeaponUsed :type "HuntWeapon Object Reference"))
  (bind _returnvalue (`self.GetCurrentWeapon`))
  (bind _firetimer (`self.FireTimer`))
  (bind _returnvalue_2 (`AIBlueprintHelperLibrary.GetBlackboard` (`self.MyAIController`)))
  (`|ExecutionSequence`
    (:`then_0`
      (`/Engine/EditorBlueprintResources/StandardMacros.IsValid` _returnvalue_2
        (:`Is Valid`
          (`BlackboardComponent.SetValueAsFloat` _returnvalue_2 (`self.HealthKey`) (`HuntStatsComponent.GetCurrentHealth` (`self.StatsComponent`))))))
    (:`then_1`
      (`self.UpdateHealthStats`)
      (if (`HuntStatsComponent.bIsDead` (`self.StatsComponent`))
        (`self.SetLifeSpan` 3.0)
        (`GameplayStatics.PlaySoundAtLocation` "/Game/Static/Audio/SFX/Enemy/Damage/A_EnemyDeath_Cue.A_EnemyDeath_Cue" (`self.K2_GetActorLocation`) (struct) 1.0 1.0 0.0 null null null)
        (set `self.bCanBeDamaged` false)
        (`/Engine/EditorBlueprintResources/StandardMacros.IsValid` (`AIBlueprintHelperLibrary.GetAIController` self)
          (:`Is Valid`
            (`self.DetachFromControllerPendingDestroy`)
            (`TimelineComponent.ReverseFromEnd` (`self.Timeline_0`))
            (`/Engine/EditorBlueprintResources/StandardMacros.IsValid` _returnvalue
              (:`Is Valid`
                (`HuntWeapon.EndFire` _returnvalue)
                (`self.K2_DestroyActor` (`self.GetCurrentWeapon`))))))
        (else
          (`GameplayStatics.PlaySoundAtLocation` "/Game/Static/Audio/SFX/Enemy/Damage/A_EnemyDamage_Cue.A_EnemyDamage_Cue" (`self.K2_GetActorLocation`) (struct) 1.0 1.0 0.0 null null null)
          (`/Engine/EditorBlueprintResources/StandardMacros.IsValid` WeaponUsed
            (:`Is Valid`
              (switch `EAmmoType` (`HuntWeapon.GetWeaponAmmoType` WeaponUsed)
                (:`AT_Fire`
                  (if (`KismetSystemLibrary.K2_IsTimerPausedHandle` _firetimer)
                    (`KismetSystemLibrary.K2_UnPauseTimerHandle` _firetimer)
                    (`GameplayStatics.SpawnEmitterAttached` "/Game/Static/MobileStarterContent/Particles/P_Fire.P_Fire" (`self.Mesh`) "pelvis" (0.0 0.0 0.0) (struct) (1.0 1.0 1.0) "SnapToTarget")))
                (:`AT_Ice`
                  (`self.OnIceDamage`))))))))))

(fn `UpdateDifficultyReference`
  (bind _returnvalue (`GameplayStatics.GetGameMode`))
  (bind _returnvalue_2 (message `HuntDifficultyInterface.GetDifficultyRankMin` _returnvalue))
  (set `self.DifficultyRankMin` _returnvalue_2)
  (bind _returnvalue_3 (message `HuntDifficultyInterface.GetDifficultyRankMax` _returnvalue))
  (set `self.DifficultyRankMax` _returnvalue_3))

(fn `UpdatePlayerRankInfo`
  (bind _returnvalue (`GameplayStatics.GetGameMode`))
  (bind _returnvalue_2 (`self.GetCurrentWeapon`))
  (bind _returnvalue_3 (`GameplayStatics.GetGlobalTimeDilation`))
  (bind _returnvalue_4 (message `HuntDifficultyInterface.GetPlayerRankPercentage` _returnvalue))
  (bind _output_get (set `self.PlayerRankPercentage` _returnvalue_4))
  (bind _returnvalue_5 (message `HuntDifficultyInterface.GetPlayerRank` _returnvalue))
  (set `self.PlayerCurrentRank` _returnvalue_5)
  (`/Engine/EditorBlueprintResources/StandardMacros.IsValid` _returnvalue_2
    (:`Is Valid`
      (set `Actor.CustomTimeDilation` _returnvalue_3 _returnvalue_2)
      (set `self.CustomTimeDilation` _returnvalue_3)
      (setmembers `WeaponStatsData` :`StructRef` (`HuntWeapon.WeaponStatsData` _returnvalue_2) :`DamageModifierAmount` _output_get)
      (`HuntWeapon.CalculateDamage` _returnvalue_2))))

(fn `UpdateWalkSpeed`
  (params (NewWalkSpeed :type "Float (double-precision)"))
  (set `CharacterMovementComponent.MaxWalkSpeed` NewWalkSpeed (`self.CharacterMovement`)))

(fn `UserConstructionScript`)