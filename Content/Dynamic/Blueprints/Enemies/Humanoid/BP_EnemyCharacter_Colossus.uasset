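; Colossus boss enemy character that drives the player's on-screen boss health bar and attacks with projectiles.
; On BeginPlay it links itself to the boss widget and binds health updates, which set a dynamic material's progress and show damage taken.
; Activation reveals the widget and starts a looping timer.
; Box overlap knocks back and damages the player and fires a Chrono projectile, while a debug event randomly spawns Chrono or delayed laser projectiles.
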(event `self.ReceiveBeginPlay`
  (bind _wbp_bosshealth (`/Game/Dynamic/UI/WBP_GameplayHUD.WBP_BossHealth` (`/Game/Dynamic/Blueprints/Player/BP_HuntPlayerController_Base.GameplayWBP` (cast `/Game/Dynamic/Blueprints/Player/BP_Gameplay_PlayerController` (`GameplayStatics.GetPlayerController` 0) :!pure true))))
  (`parent.ReceiveBeginPlay`)
  (set `/Game/Dynamic/UI/WBP_BossHealth.EnemyReference` (`|ConvertAsset` self) _wbp_bosshealth)
  (`TextBlock.SetText` (`/Game/Dynamic/UI/WBP_BossHealth.EnemyName` _wbp_bosshealth) (`KismetTextLibrary.Conv_StringToText` (`HuntStatsComponent.CharacterName` (`self.StatsComponent`))))
  (bind _returnvalue (`Image.GetDynamicMaterial` (`/Game/Dynamic/UI/WBP_BossHealth.HealthBarImage` _wbp_bosshealth)))
  (set `self.HealthBarImage_DynMat` _returnvalue)
  (add `self.UpdateHealthStats` (`|CreateDelegate` :!event `UpdateBossUI`))
  (`self.UpdateBossUI`))

(event `self.ReceivePointDamage`
  (params (Damage :type "Float (single-precision)") (DamageType :type "DamageType Object Reference") (HitLocation :type "Vector Structure") (HitNormal :type "Vector Structure") (HitComponent :type "PrimitiveComponent Object Reference") (BoneName :type Name) (ShotFromDirection :type "Vector Structure") (InstigatedBy :type "Controller Object Reference") (DamageCauser :type "Actor Object Reference") (HitInfo :type "HitResult Structure (by ref)"))
  (`parent.ReceiveAnyDamage` Damage DamageType InstigatedBy DamageCauser))

(event `UpdateBossUI`
  (bind _statscomponent (`self.StatsComponent`))
  (bind _wbp_bosshealth (`/Game/Dynamic/UI/WBP_GameplayHUD.WBP_BossHealth` (`/Game/Dynamic/Blueprints/Player/BP_HuntPlayerController_Base.GameplayWBP` (cast `/Game/Dynamic/Blueprints/Player/BP_Gameplay_PlayerController` (`GameplayStatics.GetPlayerController` 0) :!pure true))))
  (if (not (`HuntStatsComponent.bIsDead` _statscomponent))
    (`MaterialInstanceDynamic.SetScalarParameterValue` (`self.HealthBarImage_DynMat`) "Progress" (/ (`HuntStatsComponent.GetCurrentHealth` _statscomponent) (`HuntStatsComponent.GetMaxHealth` _statscomponent)))
    (`TextBlock.SetText` (`/Game/Dynamic/UI/WBP_BossHealth.DmgTakenText` _wbp_bosshealth) (`KismetTextLibrary.Conv_DoubleToText` (`self.DamageTaken`) "HalfToEven"))
    (if (`self.bIsActive?`)
      (`UserWidget.PlayAnimationForward` _wbp_bosshealth (`/Game/Dynamic/UI/WBP_BossHealth.DamageAnimation` _wbp_bosshealth) 2.0 false))))

(event `self.Box.OnComponentBeginOverlap`
  (params (OverlappedComponent :type "PrimitiveComponent Object Reference") (OtherActor :type "Actor Object Reference") (OtherComp :type "PrimitiveComponent Object Reference") (OtherBodyIndex :type Integer) (bFromSweep :type Boolean) (SweepResult :type "HitResult Structure (by ref)"))
  (bind _returnvalue (`GameplayStatics.GetPlayerCharacter` 0))
  (if (== OtherActor _returnvalue)
    (`CharacterMovementComponent.AddImpulse` (`Character.CharacterMovement` _returnvalue) (`self.PlayerKnockbackVector`) true)
    (`GameplayStatics.ApplyDamage` OtherActor 4.0)
    (`|SpawnActorFromClass` "/Game/Dynamic/Blueprints/Weapons/Projectiles/BP_HuntProjectile_Chrono_AI.BP_HuntProjectile_Chrono_AI_C" (`KismetMathLibrary.MakeTransform` (`SceneComponent.K2_GetComponentLocation` (`self.Scene`)) (`self.GetControlRotation`) (2.0 2.0 2.0)) "Undefined" "OverrideRootScale" null 0.0 null)))

(event `DebugSpawnProjectie`
  (bind _returnvalue (`self.GetControlRotation`))
  (bind _returnvalue_2 (`SceneComponent.K2_GetComponentLocation` (`self.Scene`)))
  (switch `int` (`KismetMathLibrary.RandomIntegerInRange` 0 2)
    (:`0`
      (`|SpawnActorFromClass` "/Game/Dynamic/Blueprints/Weapons/Projectiles/BP_HuntProjectile_Chrono_AI.BP_HuntProjectile_Chrono_AI_C" (`KismetMathLibrary.MakeTransform` _returnvalue_2 _returnvalue (2.0 2.0 2.0)) "Undefined" "OverrideRootScale" null 0.0 null :!label _label))
    (:`1`
      (goto _label))
    (:`2`
      (`KismetSystemLibrary.Delay` 2.0)
      (`|SpawnActorFromClass` "/Game/Dynamic/Blueprints/Weapons/Projectiles/BP_HuntProject_C_Laser.BP_HuntProject_C_Laser_C" (`KismetMathLibrary.MakeTransform` _returnvalue_2 _returnvalue (2.0 2.0 2.0)) "Undefined" "OverrideRootScale" null 0.0 null))))

(event `self.ReceiveAnyDamage`
  (params (Damage :type "Float (single-precision)") (DamageType :type "DamageType Object Reference") (InstigatedBy :type "Controller Object Reference") (DamageCauser :type "Actor Object Reference"))
  (`parent.ReceiveAnyDamage` Damage DamageType InstigatedBy DamageCauser)
  (set `self.DamageTaken` Damage))

(fn `OnActivateEnemy`
  (bind _wbp_bosshealth (`/Game/Dynamic/UI/WBP_GameplayHUD.WBP_BossHealth` (`/Game/Dynamic/Blueprints/Player/BP_HuntPlayerController_Base.GameplayWBP` (cast `/Game/Dynamic/Blueprints/Player/BP_Gameplay_PlayerController` (`GameplayStatics.GetPlayerController` 0) :!pure true))))
  (set `self.bIsActive?` true)
  (`Widget.SetVisibility` _wbp_bosshealth "HitTestInvisible")
  (`UserWidget.PlayAnimationForward` _wbp_bosshealth (`/Game/Dynamic/UI/WBP_BossHealth.StartAnimation` _wbp_bosshealth) 1.0 false)
  (`KismetSystemLibrary.K2_SetTimerDelegate` (`|CreateDelegate` :!event `DebugSpawnProjectie`) 1.0 true))

(fn `UserConstructionScript`
  (`parent.UserConstructionScript`))