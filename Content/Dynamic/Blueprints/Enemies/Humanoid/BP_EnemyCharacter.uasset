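; Humanoid AI enemy base that spawns with an attached weapon, fights, and drops pickups when destroyed.
; It mirrors health into its Blackboard and traces for "Cover"-tagged actors to set the patrol location.
; Weapon ammo type drives damage reactions: incendiary unpauses a looping burn timer, while ice toggles a freeze through time dilation and brain logic.
; A timeline plays on spawn and reverses on death, when the AI unpossesses and firing stops.
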(event `HuntCharacterInterface.OnFindCover`
  (bind (_outlocation _outrotation) (`self.GetActorEyesViewPoint`))
  (bind _outhit (`KismetSystemLibrary.LineTraceSingleForObjects` :`Start` _outlocation :`End` (+ _outlocation (* (`KismetMathLibrary.GetForwardVector` _outrotation) 1200.0)) :`ObjectTypes` (`|MakeArray` "ObjectTypeQuery2" :!type "EObjectTypeQuery Enum") :`bTraceComplex` true :`DrawDebugType` "ForDuration"))
  (bind (_bblockinghit _binitialoverlap _time _distance _location _impactpoint _normal _impactnormal _physmat _hitactor) (`GameplayStatics.BreakHitResult` _outhit))
  (`/Engine/EditorBlueprintResources/StandardMacros.IsValid` _hitactor
    (:`Is Valid`
      (if (and _bblockinghit (`self.ActorHasTag` _hitactor "Cover"))
        (`BlackboardComponent.SetValueAsVector` (`self.MyBlackboard`) "PatrolLocation" _impactpoint)))))

(event `self.ReceiveBeginPlay`
  (bind _statscomponent (`self.StatsComponent`))
  (bind _maxstarthealth (`self.MaxStartHealth`))
  (bind _mesh (`self.Mesh`))
  (bind _weapontospawn (`self.WeaponToSpawn`))
  (bind _returnvalue (`AIBlueprintHelperLibrary.GetAIController` self))
  (set `HuntStatsComponent.MaxHealth` _maxstarthealth _statscomponent)
  (set `HuntStatsComponent.CurrentHealth` _maxstarthealth _statscomponent)
  (bind _returnvalue_2 (`PrimitiveComponent.CreateDynamicMaterialInstance` _mesh 0 (`PrimitiveComponent.GetMaterial` _mesh 0) "None"))
  (set `self.Mesh_DynMat` _returnvalue_2)
  (`TimelineComponent.PlayFromStart` (`self.Timeline_0`))
  (`|ExecutionSequence`
    (:`then_0`
      (if (`KismetSystemLibrary.IsValidClass` _weapontospawn)
        (bind _returnvalue_3 (`|SpawnActorFromClass` _weapontospawn (`KismetMathLibrary.MakeTransform` (0.0 0.0 0.0)) "Undefined" "OverrideRootScale" self null))
        (bind _output_get (set `self.CurrentWeapon` _returnvalue_3))
        (`SceneComponent.K2_AttachToComponent` (`HuntWeapon.WeaponMeshTP` _output_get) (`self.Mesh`) "GripPoint" "KeepRelative" "KeepRelative" "KeepRelative" true)
        (`/Game/Dynamic/Blueprints/Weapons/BP_BaseWeapon.OnSpawn` (cast `/Game/Dynamic/Blueprints/Weapons/BP_BaseWeapon` _output_get :!pure true))
        (`HuntWeapon.SetWeaponOwner` _output_get self)))
    (:`then_1`
      (bind _returnvalue_4 (`KismetSystemLibrary.K2_SetTimerDelegate` (`|CreateDelegate` :!event `FireDamage`) 1.0 true))
      (bind _output_get_2 (set `self.FireTimer` _returnvalue_4))
      (`KismetSystemLibrary.K2_PauseTimerHandle` _output_get_2)
      (`/Engine/EditorBlueprintResources/StandardMacros.IsValid` _returnvalue
        (:`Is Valid`
          (bind _output_get_3 (set `self.MyAIController` _returnvalue))
          (bind _returnvalue_5 (`AIBlueprintHelperLibrary.GetBlackboard` _output_get_3))
          (bind _output_get_4 (set `self.MyBlackboard` _returnvalue_5))
          (`BlackboardComponent.SetValueAsFloat` _returnvalue_5 (`self.HealthKey`) (`HuntStatsComponent.GetCurrentHealth` (`self.StatsComponent`)))
          (`BlackboardComponent.SetValueAsFloat` _output_get_4 (`self.HealthKey`) (`HuntStatsComponent.GetCurrentHealth` (`self.StatsComponent`)))
          (`self.UpdateBlackboardStats`)
          (add `self.UpdateHealthStats` (`|CreateDelegate` :!event `UpdateBlackboardStats`)))))))

(event `self.ReceiveAnyDamage`
  (params (Damage :type "Float (single-precision)") (DamageType :type "DamageType Object Reference") (InstigatedBy :type "Controller Object Reference") (DamageCauser :type "Actor Object Reference"))
  (bind _returnvalue (`self.GetCurrentWeapon`))
  (bind _returnvalue_2 (`AIBlueprintHelperLibrary.GetAIController` self))
  (`parent.ReceiveAnyDamage` Damage DamageType InstigatedBy DamageCauser)
  (`GameplayStatics.PlaySoundAtLocation` "/Game/Static/Audio/SFX/Enemy/Damage/A_EnemyDamage_Cue.A_EnemyDamage_Cue" (`self.K2_GetActorLocation`) (struct) 1.0 1.0 0.0 null null null)
  (`self.ReactToDamage` (cast `HuntWeapon` DamageCauser :!pure true))
  (if (`HuntStatsComponent.bIsDead` (`self.StatsComponent`))
    (`self.SetLifeSpan` 3.0)
    (`GameplayStatics.PlaySoundAtLocation` "/Game/Static/Audio/SFX/Enemy/Damage/A_EnemyDeath_Cue.A_EnemyDeath_Cue" (`self.K2_GetActorLocation`) (struct) 1.0 1.0 0.0 null null null)
    (set `self.bCanBeDamaged` false)
    (`|ExecutionSequence`
      (:`then_0`
        (`/Engine/EditorBlueprintResources/StandardMacros.IsValid` _returnvalue_2
          (:`Is Valid`
            (`Controller.UnPossess` _returnvalue_2)
            (`TimelineComponent.ReverseFromEnd` (`self.Timeline_0`)))))
      (:`then_1`
        (`/Engine/EditorBlueprintResources/StandardMacros.IsValid` _returnvalue
          (:`Is Valid`
            (`HuntWeapon.EndFire` _returnvalue)))))))

(event `Key|G`
  (params (Key :type "Key Structure"))
  (:`Pressed`
    (`Controller.Possess` (`GameplayStatics.GetPlayerController` 0) (`/Game/Dynamic/Blueprints/Game/BP_ProjectHuntGameMode_Gameplay.PlayerRef` (cast `/Game/Dynamic/Blueprints/Game/BP_ProjectHuntGameMode_Gameplay` (`GameplayStatics.GetGameMode`) :!pure true)))))

(event `self.ReceiveEndPlay`
  (params (EndPlayReason :type "EEndPlayReason Enum" :default "Destroyed"))
  (bind _returnvalue (`self.K2_GetActorLocation`))
  (switch `EEndPlayReason` EndPlayReason
    (:`Destroyed`
      (`self.K2_DestroyActor` (`self.GetCurrentWeapon`))
      (`|SpawnActorFromClass` "/Game/Dynamic/Blueprints/Interactables/Pickups/BP_DP_Pickup_Low.BP_DP_Pickup_Low_C" (`KismetMathLibrary.MakeTransform` (`self.K2_GetActorLocation`)) "Undefined" "OverrideRootScale" null null)
      (if (`KismetMathLibrary.RandomBool`)
        (`|SpawnActorFromClass` "/Game/Dynamic/Blueprints/Interactables/Pickups/BP_HealthPickup_Low.BP_HealthPickup_Low_C" (`KismetMathLibrary.MakeTransform` _returnvalue) "Undefined" "OverrideRootScale" null null)
        (else
          (`|SpawnActorFromClass` "/Game/Dynamic/Blueprints/Interactables/Pickups/BP_MissilePickupBase_Low.BP_MissilePickupBase_Low_C" (`KismetMathLibrary.MakeTransform` _returnvalue) "Undefined" "OverrideRootScale" null null))))))

(event `FireDamage`
  (`HuntStatsComponent.DamageHealth` (`self.StatsComponent`) 5.0))

(event `OnIceDamage`
  (if (`self.bIsFrozen?`)
    (set `self.bIsFrozen?` false)
    (set `self.CustomTimeDilation` 1.0)
    (`BrainComponent.RestartLogic` (`AIController.BrainComponent` (`AIBlueprintHelperLibrary.GetAIController` self)))
    (else
      (set `self.bIsFrozen?` true)
      (set `self.CustomTimeDilation` 0.0)
      (`BrainComponent.StopLogic` (`AIController.BrainComponent` (`AIBlueprintHelperLibrary.GetAIController` self)) "Actor Frozen")
      (`HuntWeapon.EndFire` (`self.GetCurrentWeapon`))
      (`KismetSystemLibrary.Delay` 10.0)
      (set `self.bIsFrozen?` false))))

(event `HuntCharacterInterface.OnAttackTarget`
  (bind _returnvalue (`self.GetCurrentWeapon`))
  (`/Engine/EditorBlueprintResources/StandardMacros.IsValid` _returnvalue
    (:`Is Valid`
      (`HuntWeapon.StartFire` _returnvalue))))

(event `UpdateBlackboardStats`
  (bind _statscomponent (`self.StatsComponent`))
  (bind _myblackboard (`self.MyBlackboard`))
  (`/Engine/EditorBlueprintResources/StandardMacros.IsValid` _myblackboard
    (:`Is Valid`
      (`BlackboardComponent.SetValueAsFloat` _myblackboard (`self.HealthKey`) (`HuntStatsComponent.GetCurrentHealth` _statscomponent))
      (`BlackboardComponent.SetValueAsFloat` _myblackboard (`self.HealthPercentKey`) (`HuntStatsComponent.GetHealthPercentage` _statscomponent)))))

(fn `ReactToDamage`
  (params (WeaponUsed :type "HuntWeapon Object Reference"))
  (bind _firetimer (`self.FireTimer`))
  (`/Engine/EditorBlueprintResources/StandardMacros.IsValid` WeaponUsed
    (:`Is Valid`
      (`BlackboardComponent.SetValueAsFloat` (`AIBlueprintHelperLibrary.GetBlackboard` (`self.MyAIController`)) (`self.HealthKey`) (`HuntStatsComponent.GetCurrentHealth` (`self.StatsComponent`)))
      (`self.UpdateHealthStats`)
      (switch `EAmmoType` (`HuntWeapon.GetWeaponAmmoType` WeaponUsed)
        (:`AT_Fire`
          (if (`KismetSystemLibrary.K2_IsTimerPausedHandle` _firetimer)
            (`KismetSystemLibrary.K2_UnPauseTimerHandle` _firetimer)
            (`GameplayStatics.SpawnEmitterAttached` "/Game/Static/MobileStarterContent/Particles/P_Fire.P_Fire" (`self.Mesh`) "pelvis" (0.0 0.0 0.0) (struct) (1.0 1.0 1.0) "SnapToTarget")))
        (:`AT_Ice`
          (`self.OnIceDamage`))))))

(fn `UpdateWalkSpeed`
  (params (NewWalkSpeed :type "Float (double-precision)"))
  (set `CharacterMovementComponent.MaxWalkSpeed` NewWalkSpeed (`self.CharacterMovement`)))

(fn `UserConstructionScript`)