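; BP_MusicPlayer is an actor that plays music through its Audio component.
; On BeginPlay it sets the NextTrack sound and fades it in, with the target volume read from a music volume console variable.
; Playback percent updates store the elapsed seconds, though the print of that value is unconnected.
; PageUp and PageDown restart playback from a fixed offset or the beginning, apparently as debug keys.
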(event `self.ReceiveBeginPlay`
  (`self.PlayNextTrack` (`self.NextTrack`)))

(event `self.ReceiveTick`
  (params (DeltaSeconds :type "Float (single-precision)")))

(event `self.Audio.OnAudioPlaybackPercent`
  (params (PlayingSoundWave :type "SoundWave Object Reference") (PlaybackPercent :type "Float (single-precision)"))
  (set `self.NewVar_0` (* PlaybackPercent (`SoundBase.Duration` (`AudioComponent.Sound` (`self.Audio`))))))

(event `Key|PageUp`
  (params (Key :type "Key Structure"))
  (:`Pressed`
    (`AudioComponent.Play` (`self.Audio`) 30.0)))

(event `Key|PageDown`
  (params (Key :type "Key Structure"))
  (:`Pressed`
    (`AudioComponent.Play` (`self.Audio`) 0.0)))

(fn `PlayNextTrack`
  (params (NewSound :type "SoundBase Object Reference"))
  (`AudioComponent.SetSound` (`self.Audio`) NewSound)
  (`AudioComponent.FadeIn` (`self.Audio`) 2.0 (`ConsoleUtils.GetFloatCVar` "GameAudio MusicVolume") 0.0 "Linear"))

(fn `UserConstructionScript`)