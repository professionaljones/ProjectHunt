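; Gameplay game state Blueprint for Project Hunt that spawns the supporting manager actors for a session.
; BeginPlay spawns the music player, global-vars save actor and hunt chameleon at the world origin and stores references to them.
; AudioManagerSpawn creates a HuntAudioManager at a given transform and registers it with the audio manager subsystem.
; On level transition, EndPlay only prints the player location held by the save component.
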(event `self.ReceiveBeginPlay`
  (bind _returnvalue (`KismetMathLibrary.MakeTransform` (0.0 0.0 0.0)))
  (`parent.ReceiveBeginPlay`)
  (bind _returnvalue_2 (`|SpawnActorFromClass` "/Game/Dynamic/Blueprints/BP_MusicPlayer.BP_MusicPlayer_C" _returnvalue "Undefined" "OverrideRootScale" null null))
  (set `self.CurrentMusicPlayer` _returnvalue_2)
  (bind _returnvalue_3 (`|SpawnActorFromClass` "/Game/Dynamic/Blueprints/BP_GlobalVars_SaveActor.BP_GlobalVars_SaveActor_C" (`KismetMathLibrary.MakeTransform` (0.0 0.0 0.0)) "Undefined" "OverrideRootScale" null null))
  (set `self.GlobalVarsActor` _returnvalue_3)
  (bind _returnvalue_4 (`|SpawnActorFromClass` "/Game/Chameleon/BP_HuntChameleon.BP_HuntChameleon_C" _returnvalue "Undefined" "OverrideRootScale" null null))
  (set `self.ChameleonReference` _returnvalue_4))

(event `self.ReceiveEndPlay`
  (params (EndPlayReason :type "EEndPlayReason Enum" :default "Destroyed"))
  (switch `EEndPlayReason` EndPlayReason
    (:`LevelTransition`
      (`KismetSystemLibrary.PrintString` (`KismetStringLibrary.Conv_TransformToString` (`/Game/Dynamic/Blueprints/BP_GlobalVarsComponent.PlayerLocation` (`/Game/Dynamic/Blueprints/BP_GlobalVars_SaveActor.GlobalSaveComponent` (`self.GlobalVarsActor`))))))))

(fn `AudioManagerSpawn`
  (params (SpawnTransform :type "Transform Structure"))
  (bind _returnvalue (subsystem `AudioManagerSubsystem`))
  (bind _returnvalue_2 (`|SpawnActorFromClass` "/Script/ProjectHunt.HuntAudioManager" SpawnTransform "Undefined" "OverrideRootScale" null null))
  (bind _output_get (set `AudioManagerSubsystem.CurrentAudioManager` _returnvalue_2 _returnvalue))
  (`AudioManagerSubsystem.SetNewAudioManager` _returnvalue _output_get))

(fn `UserConstructionScript`
  (`parent.UserConstructionScript`))