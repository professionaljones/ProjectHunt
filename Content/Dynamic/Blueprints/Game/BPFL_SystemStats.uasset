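; BPFL_SystemStats is a function library of helpers that report platform and device status.
; IsRunningOnDesktop switches on the platform name, returning true for Windows, Linux and Mac and false for IOS and Android.
; GetMobileBatteryTemp reads the device battery temperature and converts it from Celsius to Fahrenheit when requested.
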(fn `GetMobileBatteryTemp`
  (params (bWantFahrenheit :type Boolean))
  (returns (ReturnValue :type "Float (double-precision)"))
  (if bWantFahrenheit
    (bind _returnvalue (`OptionalMobileFeaturesBPLibrary.GetBatteryTemperature`))
    (return (+ (* _returnvalue (/ 9.0 5.0)) 32.0))
    (else
      (bind _returnvalue_2 (`OptionalMobileFeaturesBPLibrary.GetBatteryTemperature`))
      (return _returnvalue_2))))

(fn `IsRunningOnDesktop`
  (returns (`bIsDesktop?` :type Boolean))
  (switch `string` (`GameplayStatics.GetPlatformName`)
    (:`Windows`
      _)
    (:`Linux`
      _)
    (:`Mac`
      _)
    (:`IOS`
      (return false))
    (:`Android`
      (return false)))
  (return true))