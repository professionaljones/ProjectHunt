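; Game instance for Project Hunt that handles save slots, checkpoint respawn and player settings.
; Save events snapshot player stats, weapons, ammo types, transform and level into a ProjectHuntSaveGame, synchronously or async; load events reopen the saved level.
; SetPlayerToCheckpoint reloads the AutoSave slot and moves the player to its saved location.
; Init registers CVar callbacks for sound-class volumes, look sensitivity and player style; a helper sets global time dilation.
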(event `AsyncSaveSlot`
  (params (SaveSlotName :type String))
  (bind (_current_health _max_health _current_aragon _max_aragon _weaponinventory _playertransform _pat _rat _sat _pistol_chargelimit _rifle_chargelimit _shotgun_chargelimit _currentsuitpower _maxmissiles) (`self.GetPlayerData`))
  (if (`self.bIsLoadingSave?`)
    (set `self.bIsLoadingSave?` false))
  (bind _returnvalue (`GameplayStatics.CreateSaveGameObject` "/Game/Dynamic/Blueprints/Game/Save_Load/ProjectHuntSaveGame.ProjectHuntSaveGame_C"))
  (bind _output_get (set `self.SaveGameReference` _returnvalue))
  (bind _returnvalue_2 (`GameplayStatics.GetCurrentLevelName` true))
  (bind _desiredsavename (`/Game/Dynamic/Blueprints/Game/Save_Load/ProjectHuntSaveGame.SetSaveData` _output_get _current_health _max_health _current_aragon _max_aragon _weaponinventory _returnvalue_2 _playertransform SaveSlotName _pat _rat _sat _currentsuitpower _maxmissiles))
  (bind (_savegame _bsuccess) (`AsyncActionHandleSaveGame.AsyncSaveGameToSlot` _output_get _desiredsavename (`/Game/Dynamic/Blueprints/Game/Save_Load/ProjectHuntSaveGame.UserIndex` _output_get))
    (:`Completed`
      (`/Engine/EditorBlueprintResources/StandardMacros.IsValid` _savegame
        (:`Is Valid`
          (if _bsuccess
            (`GameplayStatics.PlaySound2D` "/Game/Static/Audio/SFX/PM_FSSF2_TONAL_ACHIEVEMENT_POWERUP_EVENT_19.PM_FSSF2_TONAL_ACHIEVEMENT_POWERUP_EVENT_19" 1.0 1.0 0.0 null null)))))))

(event `AsyncLoadSlot`
  (params (SlotName :type String))
  (bind _returnvalue (`GameplayStatics.DoesSaveGameExist` SlotName))
  (if _returnvalue
    (bind _savegame (`AsyncActionHandleSaveGame.AsyncLoadGameFromSlot` SlotName)
      (:`Completed`
        (bind _asproject_hunt_save_game (cast `/Game/Dynamic/Blueprints/Game/Save_Load/ProjectHuntSaveGame` _savegame :!pure true))
        (set `self.SaveGameReference` _asproject_hunt_save_game)
        (set `self.bIsLoadingSave?` true)
        (bind _save_levelname (`/Game/Dynamic/Blueprints/Game/Save_Load/ProjectHuntSaveGame.Save_LevelName` _asproject_hunt_save_game))
        (`GameplayStatics.OpenLevel` (`KismetStringLibrary.Conv_StringToName` _save_levelname))
        (`KismetSystemLibrary.PrintString` _save_levelname)))
    (else
      (`KismetSystemLibrary.PrintString` "Save does not exist!" true true (struct :`R` 1.0 :`A` 1.0) 5.0))))

(event `LoadPlayerStats`
  (params (SlotName :type String))
  (bind _returnvalue (`GameplayStatics.DoesSaveGameExist` SlotName))
  (if _returnvalue
    (bind _returnvalue_2 (`GameplayStatics.LoadGameFromSlot` SlotName))
    (set `self.SaveGameReference` (cast `/Game/Dynamic/Blueprints/Game/Save_Load/ProjectHuntSaveGame` _returnvalue_2 :!pure true))
    (else
      (`KismetSystemLibrary.PrintString` "Save does not exist!" true true (struct :`R` 1.0 :`A` 1.0) 5.0))))

(event `MenuSaveSlot`
  (params (SaveSlotName :type String))
  (bind (_current_health _max_health _current_aragon _max_aragon _weaponinventory _playertransform _pat _rat _sat _pistol_chargelimit _rifle_chargelimit _shotgun_chargelimit _currentsuitpower _maxmissiles) (`self.GetPlayerData`))
  (if (`self.bIsLoadingSave?`)
    (set `self.bIsLoadingSave?` false))
  (bind _returnvalue (`GameplayStatics.CreateSaveGameObject` "/Game/Dynamic/Blueprints/Game/Save_Load/ProjectHuntSaveGame.ProjectHuntSaveGame_C"))
  (bind _output_get (set `self.SaveGameReference` _returnvalue))
  (bind _returnvalue_2 (`GameplayStatics.GetCurrentLevelName` true))
  (bind _desiredsavename (`/Game/Dynamic/Blueprints/Game/Save_Load/ProjectHuntSaveGame.SetSaveData` _output_get _current_health _max_health _current_aragon _max_aragon _weaponinventory _returnvalue_2 _playertransform SaveSlotName _pat _rat _sat _currentsuitpower _maxmissiles))
  (bind _returnvalue_3 (`GameplayStatics.SaveGameToSlot` _output_get _desiredsavename))
  (if _returnvalue_3
    (`GameplayStatics.PlaySound2D` "/Game/Static/Audio/SFX/PM_FSSF2_TONAL_ACHIEVEMENT_POWERUP_EVENT_19.PM_FSSF2_TONAL_ACHIEVEMENT_POWERUP_EVENT_19" 1.0 1.0 0.0 null null)))

(event `MenuLoadSlot`
  (params (SlotName :type String))
  (bind _returnvalue (`GameplayStatics.DoesSaveGameExist` SlotName))
  (if _returnvalue
    (bind _returnvalue_2 (`GameplayStatics.LoadGameFromSlot` SlotName))
    (bind _asproject_hunt_save_game (cast `/Game/Dynamic/Blueprints/Game/Save_Load/ProjectHuntSaveGame` _returnvalue_2))
    (bind _output_get (set `self.SaveGameReference` _asproject_hunt_save_game))
    (set `self.bIsLoadingSave?` true)
    (`GameplayStatics.OpenLevel` (`KismetStringLibrary.Conv_StringToName` (`/Game/Dynamic/Blueprints/Game/Save_Load/ProjectHuntSaveGame.Save_LevelName` _output_get)))
    (`/Game/Dynamic/Blueprints/Player/BP_TrishPlayerCharacter.InitSaveStats` (cast `/Game/Dynamic/Blueprints/Player/BP_TrishPlayerCharacter` (`GameplayStatics.GetPlayerCharacter` 0) :!pure true))
    (else
      (`KismetSystemLibrary.PrintString` "Save does not exist!" true true (struct :`R` 1.0 :`A` 1.0) 5.0))))

(event `self.ReceiveInit`
  (`/Game/Dialog/DialogSystem.Set dialogue language` "There's no need to setting up a language if \nthe \"Get the savegame language\" is checked, \nsince it only refreshes your game instance language \nvariable. Otherwise, we should put \"English\", \"Spanish\",\"German\", etc in order to set up those languages." true)
  (`|ExecutionSequence`
    (:`then_0`
      (`SettingsManager.RegisterFloatCVarSettingWithCallback` "GameAudio MasterVolume" 0.75 "This value adjusts the loudness of all sound classes." (`|CreateDelegate` :!event `UpdateMasterVolume`) true)
      (`SettingsManager.RegisterFloatCVarSettingWithCallback` "GameAudio MusicVolume" 0.75 "This value adjusts the loudness of the Music sound class." (`|CreateDelegate` :!event `UpdateMusicVolume`) true)
      (`SettingsManager.RegisterFloatCVarSettingWithCallback` "GameAudio VoiceVolume" 0.75 "This value adjusts the loudness of the Voice sound class." (`|CreateDelegate` :!event `UpdateVoiceVolume`) true)
      (`SettingsManager.RegisterFloatCVarSettingWithCallback` "GameAudio EffectsVolume" 0.75 "This value adjusts the loudness of the Effects sound class" (`|CreateDelegate` :!event `UpdateEffectsVolume`) true)
      (`SettingsManager.RegisterFloatCVarSettingWithCallback` "GameAudio InterfaceVolume" 0.75 "This value adjusts the loudness of the Interface sound class" (`|CreateDelegate` :!event `UpdateInterfaceVolume`) true)
      (`SettingsManager.RegisterFloatCVarSettingWithCallback` "GameAudio WeaponsVolume" 0.75 "This value adjusts the loudness of the Weapons sound class" (`|CreateDelegate` :!event `UpdateWeaponsVolume`) true)
      (`SettingsManager.RegisterFloatCVarSettingWithCallback` "CameraSensitivity MouseX" 1.0 "This value adjusts the multiplier for the Mouse X axis adjuster" (`|CreateDelegate` :!event `UpdateMouseXSensitivity`) true)
      (`SettingsManager.RegisterFloatCVarSettingWithCallback` "CameraSensitivity MouseY" 1.0 "This value adjusts the multiplier for the Mouse Y axis adjuster" (`|CreateDelegate` :!event `UpdateMouseYSensitivity`) true)
      (`SettingsManager.RegisterFloatCVarSettingWithCallback` "CameraSensitivity GamepadX" 50.0 "This value adjusts the multiplier for the Gamepad X axis adjuster" (`|CreateDelegate` :!event `UpdateGamepadXSensitivity`) true)
      (`SettingsManager.RegisterFloatCVarSettingWithCallback` "CameraSensitivity GamepadY" 50.0 "This value adjusts the multiplier for the Gamepad Y axis adjuster" (`|CreateDelegate` :!event `UpdateGamepadYSensitivity`) true)
      (`SettingsManager.RegisterFloatCVarSettingWithCallback` "Cheat ModifyStyle" 0.02 "This will modify the players current style by the @param amount" (`|CreateDelegate` :!event `UpdatePlayerStyle`) true))))

(event `UpdateMasterVolume`
  (params (NewValue :type "Float (double-precision)"))
  (`GameplayStatics.PushSoundMixModifier` "/Game/Dynamic/Sound/SM_Master.SM_Master")
  (`GameplayStatics.SetSoundMixClassOverride` "/Game/Dynamic/Sound/SM_Master.SM_Master" "/Game/Dynamic/Sound/Master.Master" NewValue 1.0 0.25))

(event `UpdatePlayerStyle`
  (params (NewValue :type "Float (double-precision)"))
  (`ProjectHuntCharacter.ModifyStyle` (cast `ProjectHuntCharacter` (`GameplayStatics.GetPlayerCharacter` 0) :!pure true) NewValue))

(event `UpdateMouseXSensitivity`
  (params (NewValue :type "Float (double-precision)"))
  (bind _output_get (set `self.MouseXSensitivity` NewValue))
  (set `HuntPlayerController.LookXSensitivity_PC` _output_get (cast `HuntPlayerController` (`GameplayStatics.GetPlayerController` 0) :!pure true)))

(event `UpdateMusicVolume`
  (params (NewValue :type "Float (double-precision)"))
  (`GameplayStatics.PushSoundMixModifier` "/Game/Dynamic/Sound/SM_Master.SM_Master")
  (`GameplayStatics.SetSoundMixClassOverride` "/Game/Dynamic/Sound/SM_Master.SM_Master" "/Game/Dynamic/Sound/Music.Music" NewValue 1.0 0.25))

(event `UpdateMouseYSensitivity`
  (params (NewValue :type "Float (double-precision)"))
  (bind _output_get (set `self.MouseYSensitivity` NewValue))
  (set `HuntPlayerController.LookYSensitivity_PC` _output_get (cast `HuntPlayerController` (`GameplayStatics.GetPlayerController` 0) :!pure true)))

(event `UpdateEffectsVolume`
  (params (NewValue :type "Float (double-precision)"))
  (`GameplayStatics.PushSoundMixModifier` "/Game/Dynamic/Sound/SM_Master.SM_Master")
  (`GameplayStatics.SetSoundMixClassOverride` "/Game/Dynamic/Sound/SM_Master.SM_Master" "/Game/Dynamic/Sound/Effects.Effects" NewValue 1.0 0.25))

(event `UpdateGamepadXSensitivity`
  (params (NewValue :type "Float (double-precision)"))
  (bind _output_get (set `self.GamepadXSensitivity` NewValue))
  (set `HuntPlayerController.LookXSensitivity_GP` _output_get (cast `HuntPlayerController` (`GameplayStatics.GetPlayerController` 0) :!pure true)))

(event `UpdateInterfaceVolume`
  (params (NewValue :type "Float (double-precision)"))
  (`GameplayStatics.PushSoundMixModifier` "/Game/Dynamic/Sound/SM_Master.SM_Master")
  (`GameplayStatics.SetSoundMixClassOverride` "/Game/Dynamic/Sound/SM_Master.SM_Master" "/Game/Dynamic/Sound/Interface.Interface" NewValue 1.0 0.25))

(event `UpdateGamepadYSensitivity`
  (params (NewValue :type "Float (double-precision)"))
  (bind _output_get (set `self.GamepadYSensitivity` NewValue))
  (set `HuntPlayerController.LookYSensitivity_GP` _output_get (cast `HuntPlayerController` (`GameplayStatics.GetPlayerController` 0) :!pure true)))

(event `UpdateWeaponsVolume`
  (params (NewValue :type "Float (double-precision)"))
  (`GameplayStatics.PushSoundMixModifier` "/Game/Dynamic/Sound/SM_Master.SM_Master")
  (`GameplayStatics.SetSoundMixClassOverride` "/Game/Dynamic/Sound/SM_Master.SM_Master" "/Game/Dynamic/Sound/Weapons.Weapons" NewValue 1.0 0.25))

(event `UpdateVoiceVolume`
  (params (NewValue :type "Float (double-precision)"))
  (`GameplayStatics.PushSoundMixModifier` "/Game/Dynamic/Sound/SM_Master.SM_Master")
  (`GameplayStatics.SetSoundMixClassOverride` "/Game/Dynamic/Sound/SM_Master.SM_Master" "/Game/Dynamic/Sound/Voice.Voice" NewValue 1.0 0.25))

(fn `AdjustGlobalTimeDilation`
  (params (CurrentTimeDilation :type "Float (double-precision)"))
  (bind _output_get (set `self.CurrentTimeDilation` CurrentTimeDilation))
  (`GameplayStatics.SetGlobalTimeDilation` _output_get))

(fn `GetPlayerData`
  (returns (`Current Health` :type "Float (double-precision)") (`Max Health` :type "Float (double-precision)") (`Current Aragon` :type "Float (double-precision)") (`Max Aragon` :type "Float (double-precision)") (WeaponInventory :type "Map of EWeaponType Enum to HuntWeapon Object Reference") (PlayerTransform :type "Transform Structure (by ref)") (PAT :type "EAmmoType Enum") (RAT :type "EAmmoType Enum") (SAT :type "EAmmoType Enum") (Pistol_ChargeLimit :type "Float (double-precision)") (Rifle_ChargeLimit :type "Float (double-precision)") (Shotgun_ChargeLimit :type "Float (double-precision)") (CurrentSuitPower :type "ESuitMainAbilities Enum") (MaxMissiles :type Integer))
  (locals (L_SavePAT :type "EAmmoType Enum") (L_SaveRAT :type "EAmmoType Enum" :default "AT_Standard") (L_SaveSAT :type "EAmmoType Enum" :default "AT_Standard"))
  (bind _returnvalue (`GameplayStatics.GetPlayerCharacter` 0))
  (bind _ashunt_player_character (cast `HuntPlayerCharacter` _returnvalue :!pure true))
  (bind _statscomponent (`ProjectHuntCharacter.StatsComponent` _ashunt_player_character))
  (bind _weaponinventory (`HuntPlayerCharacter.WeaponInventory` _ashunt_player_character))
  (bind (_value _returnvalue_2) (`BlueprintMapLibrary.Map_Find` _weaponinventory "WT_Shotgun"))
  (bind (_value_2 _returnvalue_3) (`BlueprintMapLibrary.Map_Find` _weaponinventory "WT_Rifle"))
  (bind (_value_3 _returnvalue_4) (`BlueprintMapLibrary.Map_Find` _weaponinventory "WT_Pistol"))
  (bind ((`WeaponAmmoType` _weaponammotype) (`WeaponChargeLimit` _weaponchargelimit)) (break `WeaponStatsData` (`HuntWeapon.WeaponStatsData` _value_3)))
  (`|ExecutionSequence`
    (:`then_0`
      (if _returnvalue_4
        (set `local.L_SavePAT` _weaponammotype)))
    (:`then_1`
      (if _returnvalue_3
        (set `local.L_SaveRAT` (`.WeaponAmmoType` (break `WeaponStatsData` (`HuntWeapon.WeaponStatsData` _value_2))))))
    (:`then_2`
      (if _returnvalue_2
        (set `local.L_SaveSAT` (`.WeaponAmmoType` (break `WeaponStatsData` (`HuntWeapon.WeaponStatsData` _value))))))
    (:`then_3`
      (return (`HuntStatsComponent.GetCurrentHealth` _statscomponent) (`HuntStatsComponent.GetMaxHealth` _statscomponent) (`HuntStatsComponent.GetCurrentAragon` _statscomponent) (`HuntStatsComponent.GetMaxAragon` _statscomponent) _weaponinventory (`Actor.GetTransform` _returnvalue) (`local.L_SavePAT`) (`local.L_SaveRAT`) (`local.L_SaveSAT`) _weaponchargelimit 0.0 0.0 (`HuntStatsComponent.CurrentSuitPower` _statscomponent) (`HuntPlayerCharacter.GetMaxMissiles` _ashunt_player_character)))))

(fn `SetPlayerToCheckpoint`
  (bind _returnvalue (`GameplayStatics.DoesSaveGameExist` "AutoSave"))
  (if _returnvalue
    (`self.MenuLoadSlot` "AutoSave")
    (`Actor.K2_SetActorLocation` (`GameplayStatics.GetPlayerCharacter` 0) (.location (`/Game/Dynamic/Blueprints/Game/Save_Load/ProjectHuntSaveGame.Save_PlayerTransform` (`self.SaveGameReference`))) false false)))