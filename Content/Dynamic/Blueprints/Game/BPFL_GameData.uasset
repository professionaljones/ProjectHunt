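; Blueprint function library of static getters for shared game data in the Hunt project.
; It returns the enemy array for spawners from the UGC game instance and the gamepad-usage state from player controller 0.
; It also builds a save path to a hardcoded TestSave.sav under My Games/Aragon The Hunt in the Documents folder.
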(fn `GetEnemiesForSpawner`
  (returns (EnemyArray :type "Array of Actor Class Reference"))
  (return (`/Game/Dynamic/Blueprints/Game/BP_ProjectHuntUGC_GameInstance.EnemyArray` (cast `/Game/Dynamic/Blueprints/Game/BP_ProjectHuntUGC_GameInstance` (`GameplayStatics.GetGameInstance` null) :!pure true))))

(fn `GetSaveLocation`
  (returns (ReturnValue :type String))
  (return (`KismetStringLibrary.Concat_StrStr` (`RamaSaveLibrary.GetDocumentsFolder`) "My Games/" "Aragon The Hunt/" "TestSave.sav")))

(fn `IsPlayerUsingGamepad?`
  (returns (`bIsUsingGamepad?` :type Boolean))
  (return (`/Game/Dynamic/Blueprints/Player/BP_HuntPlayerController_Base.IsPlayerUsingGamepad?` (cast `/Game/Dynamic/Blueprints/Player/BP_HuntPlayerController_Base` (`GameplayStatics.GetPlayerController` null) :!pure true))))