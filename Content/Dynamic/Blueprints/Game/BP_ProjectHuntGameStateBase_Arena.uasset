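; Arena mode game state that runs endless enemy waves and passes kill score to the player state and stats UI.
; Wave start triggers every level BP_ArenaSpawner and, inside that loop, starts random music and a looping timer for enemy checks.
; When no "Enemy"-tagged actors remain, it increments the wave, resets the modifier and restarts after a delay.
; From wave five onward, each completion also picks a random modifier.
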(event `HuntGameInterface.OnPlayerArenaKill`
  (params (ScoreModAmount :type Integer))
  (bind _returnvalue (`GameplayStatics.GetPlayerController` 0))
  (bind _returnvalue_2 (`self.UpdatePlayerScore` ScoreModAmount))
  (`/Engine/EditorBlueprintResources/StandardMacros.IsValid` _returnvalue
    (:`Is Valid`
      (message `HuntPlayerInterface.OnModifyArenaScore` (`Controller.PlayerState` _returnvalue) _returnvalue_2)
      (message `HuntCharacterInterface.UpdateStatsUI` (`GameplayStatics.GetPlayerCharacter` 0)))))

(event `self.ReceiveBeginPlay`
  (`parent.ReceiveBeginPlay`)
  (bind _outactors (`GameplayStatics.GetAllActorsOfClass` "/Game/Dynamic/Blueprints/Spawners/BP_ArenaSpawner.BP_ArenaSpawner_C"))
  (set `self.LevelEnemySpawners` _outactors)
  (`self.ResetModifierOne`))

(event `HuntGameInterface.OnArenaWaveStart`
  (bind _currentmusicplayer (`self.CurrentMusicPlayer`))
  (for _array_element (`self.LevelEnemySpawners`)
    (`/Game/Dynamic/Blueprints/Spawners/BP_BaseRespawner.SpawnRandomOnDelay` _array_element)
    (`/Engine/EditorBlueprintResources/StandardMacros.IsValid` _currentmusicplayer
      (:`Is Valid`
        (`/Game/Dynamic/Blueprints/BP_MusicPlayer.PlayRandomTrack` _currentmusicplayer false true)
        (bind _returnvalue (`KismetSystemLibrary.K2_SetTimerDelegate` (`|CreateDelegate` :!event `CheckForEnemies`) 0.5 true 5.0))
        (set `self.EnemyCheckHandle` _returnvalue)))))

(event `CheckForEnemies`
  (bind _outactors (`GameplayStatics.GetAllActorsWithTag` "Enemy"))
  (bind _output_get (set `self.CurrentWaveEnemies` _outactors))
  (bind _output_get_2 (set `self.CurrentNumEnemies` (`KismetArrayLibrary.Array_Length` _output_get)))
  (`KismetSystemLibrary.PrintString` (`KismetStringLibrary.Conv_IntToString` _output_get_2))
  (if (<= _output_get_2 0)
    (`HuntGameInterface.OnArenaWaveComplete`)))

(event `HuntGameInterface.OnArenaWaveComplete`
  (bind _currentwave (`self.CurrentWave`))
  (`self.ResetModifierOne`)
  (set `self.LastArenaWave` _currentwave)
  (bind _result (`/Engine/EditorBlueprintResources/StandardMacros.IncrementInt` _currentwave)
    (:`  `
      (bind _output_get (set `self.CurrentWave` _result))
      (`|ExecutionSequence`
        (:`then_0`
          (message `HuntCharacterInterface.UpdateStatsUI` (`GameplayStatics.GetPlayerCharacter` 0))
          (`KismetSystemLibrary.K2_ClearAndInvalidateTimerHandle` (`self.EnemyCheckHandle`))
          (`KismetSystemLibrary.PrintString` "Wave is complete!")
          (`KismetSystemLibrary.Delay` 5.0)
          (`HuntGameInterface.OnArenaWaveStart`))
        (:`then_1`
          (if (>= _output_get 5)
            (bind _output_get_2 (set `self.bUseModifiers?` true))
            (if _output_get_2
              (`self.FindRandomModifier`))))))))

(fn `UserConstructionScript`
  (`parent.UserConstructionScript`))