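; Game instance for Project Hunt that handles saving and loading, settings, in-app purchases, pause and time dilation.
; Profile saves store prologue completion, while slot saves snapshot player stats, weapons, abilities, transform and level objects.
; Async and blocking (menu) variants write and read slots, with loads reopening the saved level.
; Init registers CVar settings with callbacks for sound class volumes and look sensitivity, and requests Android permissions.
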(event `AsyncSaveProfile`
  (bind _returnvalue (`GameplayStatics.CreateSaveGameObject` "/Game/Dynamic/Blueprints/Game/Save_Load/ProjectHuntProfileSaveGame.ProjectHuntProfileSaveGame_C"))
  (bind _output_get (set `self.ProfileSaveReference` _returnvalue))
  (`/Game/Dynamic/Blueprints/Game/Save_Load/ProjectHuntProfileSaveGame.SetProfileData` _output_get (`self.GetProfileData`) false)
  (bind (_savegame _bsuccess) (`AsyncActionHandleSaveGame.AsyncSaveGameToSlot` _output_get "Profile01")
    (:`Completed`
      (set `self.ProfileSaveReference` (cast `/Game/Dynamic/Blueprints/Game/Save_Load/ProjectHuntProfileSaveGame` _savegame :!pure true))
      (if _bsuccess
        (`GameplayStatics.PlaySound2D` "/Game/Static/Audio/SFX/PM_FSSF2_TONAL_ACHIEVEMENT_POWERUP_EVENT_19.PM_FSSF2_TONAL_ACHIEVEMENT_POWERUP_EVENT_19" 1.0 1.0 0.0 null null)))))

(event `MakeIAP`
  (params (`Product Identifier` :type String) (`Is Consumable` :type Boolean))
  (bind _inapppurchaseproductrequest (make `InAppPurchaseProductRequest` `Product Identifier` `Is Consumable`))
  (bind _returnvalue (`/Game/Dynamic/Blueprints/Game/BPFL_SystemStats.GetOnlineStatus`))
  (if _returnvalue
    (bind (_purchasestatus _inapppurchasereceipts) (`|InAppPurchase` (`GameplayStatics.GetPlayerController` 0) _inapppurchaseproductrequest)
      (:`OnSuccess`
        _)
      (:`OnFailure`
        _))
    (switch `EInAppPurchaseState` _purchasestatus
      (:`Success`
        (`KismetSystemLibrary.PrintString` "You have purchased new content!"))
      (:`Failed`
        (`KismetSystemLibrary.PrintString` "Purchase failed, please try again" :!label _label))
      (:`NotAllowed`
        (goto _label)))
    (else
      (bind _playercontroller (`ShowLoginUICallbackProxy.ShowExternalLoginUI` (`GameplayStatics.GetPlayerController` 0))
        (:`OnSuccess`
          (`InAppPurchaseCallbackProxy.CreateProxyObjectForInAppPurchase` _playercontroller _inapppurchaseproductrequest))))))

(event `AsyncLoadProfile`
  (bind _returnvalue (`GameplayStatics.DoesSaveGameExist` "Profile01"))
  (if _returnvalue
    (bind (_savegame _bsuccess) (`AsyncActionHandleSaveGame.AsyncLoadGameFromSlot` "Profile01")
      (:`then`
        (`KismetSystemLibrary.PrintString` "Loading"))
      (:`Completed`
        (if _bsuccess
          (bind _output_get (set `self.ProfileSaveReference` (cast `/Game/Dynamic/Blueprints/Game/Save_Load/ProjectHuntProfileSaveGame` _savegame :!pure true)))
          (set `/Game/Dynamic/Blueprints/Game/BP_ProjectHuntGameStateBase.bIsPrologueComplete?` (`.bHasCompletedPrologue?` (`/Game/Dynamic/Blueprints/Game/Save_Load/ProjectHuntProfileSaveGame.GetProfileData` _output_get)) (cast `/Game/Dynamic/Blueprints/Game/BP_ProjectHuntGameStateBase` (`GameplayStatics.GetGameState`) :!pure true)))))))

(event `AsyncSaveSlot`
  (params (SaveSlotName :type String))
  (bind (_current_health _max_health _current_aragon _max_aragon _weaponinventory _playertransform _currentsuitpower _maxmissiles _pistolstatsdata _riflestatsdata _shotgunstatsdata _currentitempercentage _currentdatapoints _bcanusemissiles _bcandash _bcanwallrun) (`self.GetPlayerData`))
  (set `self.SaveSlotName` SaveSlotName)
  (if (`self.bIsLoadingSave?`)
    (set `self.bIsLoadingSave?` false))
  (bind _returnvalue (`GameplayStatics.CreateSaveGameObject` "/Game/Dynamic/Blueprints/Game/Save_Load/ProjectHuntSaveGame.ProjectHuntSaveGame_C"))
  (bind _output_get (set `self.SaveGameReference` _returnvalue))
  (bind _returnvalue_2 (`GameplayStatics.GetCurrentLevelName` true))
  (bind _desiredsavename (`/Game/Dynamic/Blueprints/Game/Save_Load/ProjectHuntSaveGame.SetSaveData` _output_get _current_health _max_health _current_aragon _max_aragon _weaponinventory _returnvalue_2 _playertransform SaveSlotName _currentsuitpower _maxmissiles _pistolstatsdata _riflestatsdata _shotgunstatsdata _currentitempercentage (`self.LevelSaveableObjectsArray`) (`self.ManualSlotName`) _currentdatapoints _bcanusemissiles _bcandash _bcanwallrun (`KismetMathLibrary.Now`)))
  (bind (_savegame _bsuccess) (`AsyncActionHandleSaveGame.AsyncSaveGameToSlot` _output_get _desiredsavename (`/Game/Dynamic/Blueprints/Game/Save_Load/ProjectHuntSaveGame.UserIndex` _output_get))
    (:`Completed`
      (if _bsuccess
        (set `self.SaveGameReference` (cast `/Game/Dynamic/Blueprints/Game/Save_Load/ProjectHuntSaveGame` _savegame :!pure true))
        (`GameplayStatics.PlaySound2D` "/Game/Static/Audio/SFX/PM_FSSF2_TONAL_ACHIEVEMENT_POWERUP_EVENT_19.PM_FSSF2_TONAL_ACHIEVEMENT_POWERUP_EVENT_19" 1.0 1.0 0.0 null null)))))

(event `LoadPlayerStats`
  (params (SlotName :type String))
  (bind _returnvalue (`GameplayStatics.DoesSaveGameExist` SlotName))
  (if _returnvalue
    (bind _returnvalue_2 (`GameplayStatics.LoadGameFromSlot` SlotName))
    (set `self.SaveGameReference` (cast `/Game/Dynamic/Blueprints/Game/Save_Load/ProjectHuntSaveGame` _returnvalue_2 :!pure true))
    (else
      (`KismetSystemLibrary.PrintString` "Save does not exist!" true true (struct :`R` 1.0 :`A` 1.0) 5.0))))

(event `AsyncLoadSlot`
  (params (SlotName :type String))
  (bind _returnvalue (`GameplayStatics.DoesSaveGameExist` SlotName))
  (set `self.bIsLoadingSave?` _returnvalue)
  (bind _output_get (set `self.SaveSlotName` SlotName))
  (if _returnvalue
    (bind (_savegame _bsuccess) (`AsyncActionHandleSaveGame.AsyncLoadGameFromSlot` _output_get)
      (:`then`
        (`KismetSystemLibrary.PrintString` "Loading"))
      (:`Completed`
        (if _bsuccess
          (bind _asproject_hunt_save_game (cast `/Game/Dynamic/Blueprints/Game/Save_Load/ProjectHuntSaveGame` _savegame :!pure true))
          (set `self.SaveGameReference` _asproject_hunt_save_game)
          (`GameplayStatics.OpenLevel` (`KismetStringLibrary.Conv_StringToName` (`/Game/Dynamic/Blueprints/Game/Save_Load/ProjectHuntSaveGame.Save_LevelName` _asproject_hunt_save_game))))))
    (else
      (`KismetSystemLibrary.PrintString` "Save does not exist!" true true (struct :`R` 1.0 :`A` 1.0) 5.0))))

(event `MenuSaveSlot`
  (params (SaveSlotName :type String))
  (bind (_current_health _max_health _current_aragon _max_aragon _weaponinventory _playertransform _currentsuitpower _maxmissiles _pistolstatsdata _riflestatsdata _shotgunstatsdata _currentitempercentage _currentdatapoints _bcanusemissiles _bcandash _bcanwallrun) (`self.GetPlayerData`))
  (bind _returnvalue (`GameplayStatics.CreateSaveGameObject` "/Game/Dynamic/Blueprints/Game/Save_Load/ProjectHuntSaveGame.ProjectHuntSaveGame_C"))
  (bind _output_get (set `self.SaveGameReference` _returnvalue))
  (bind _returnvalue_2 (`GameplayStatics.GetCurrentLevelName` true))
  (bind _desiredsavename (`/Game/Dynamic/Blueprints/Game/Save_Load/ProjectHuntSaveGame.SetSaveData` :`self` _output_get :`Save_CurrentHealth` _current_health :`Save_MaxHealth` _max_health :`Save_CurrentAragon` _current_aragon :`Save_MaxAragon` _max_aragon :`Save_WeaponInventory` _weaponinventory :`Save_LevelName` _returnvalue_2 :`Save_PlayerTransform` _playertransform :`SaveSlotName` SaveSlotName :`Save_CurrentSuitPower` _currentsuitpower :`SaveMaxMissiles` _maxmissiles :`SavePistolStats` _pistolstatsdata :`SaveRifleStats` _riflestatsdata :`SaveSGStats` _shotgunstatsdata :`ItemPercentage` _currentitempercentage :`SaveableObjectArray` (`self.LevelSaveableObjectsArray`) :`Save_ManualSlotName` (`self.ManualSlotName`) :`Save_CurrentDP` _currentdatapoints :`Save_HasMissileLauncher` _bcanusemissiles :`Save_CanWallrun` _bcandash :`Save_CanDash` _bcanwallrun))
  (bind _returnvalue_3 (`GameplayStatics.SaveGameToSlot` _output_get _desiredsavename))
  (if _returnvalue_3
    (`GameplayStatics.PlaySound2D` "/Game/Static/Audio/SFX/PM_FSSF2_TONAL_ACHIEVEMENT_POWERUP_EVENT_19.PM_FSSF2_TONAL_ACHIEVEMENT_POWERUP_EVENT_19" 1.0 1.0 0.0 null null)))

(event `MenuLoadSlot`
  (params (SlotName :type String))
  (bind _output_get (set `self.SaveSlotName` SlotName))
  (bind _returnvalue (`GameplayStatics.DoesSaveGameExist` _output_get))
  (if _returnvalue
    (bind _returnvalue_2 (`GameplayStatics.LoadGameFromSlot` SlotName))
    (bind _asproject_hunt_save_game (cast `/Game/Dynamic/Blueprints/Game/Save_Load/ProjectHuntSaveGame` _returnvalue_2))
    (bind _output_get_2 (set `self.SaveGameReference` _asproject_hunt_save_game))
    (set `self.bIsLoadingSave?` true)
    (`GameplayStatics.OpenLevel` (`KismetStringLibrary.Conv_StringToName` (`/Game/Dynamic/Blueprints/Game/Save_Load/ProjectHuntSaveGame.Save_LevelName` _output_get_2)))
    (else
      (`KismetSystemLibrary.PrintString` "Save does not exist!" true true (struct :`R` 1.0 :`A` 1.0) 5.0))))

(event `self.ReceiveInit`
  (`|ExecutionSequence`
    (:`then_0`
      (`SettingsManager.RegisterFloatCVarSettingWithCallback` "GameAudio MasterVolume" 0.75 "This value adjusts the loudness of all sound classes." (`|CreateDelegate` :!event `UpdateMasterVolume`) true)
      (`SettingsManager.RegisterFloatCVarSettingWithCallback` "GameAudio MusicVolume" 0.75 "This value adjusts the loudness of the Music sound class." (`|CreateDelegate` :!event `UpdateMusicVolume`) true)
      (`SettingsManager.RegisterFloatCVarSettingWithCallback` "GameAudio VoiceVolume" 0.75 "This value adjusts the loudness of the Voice sound class." (`|CreateDelegate` :!event `UpdateVoiceVolume`) true)
      (`SettingsManager.RegisterFloatCVarSettingWithCallback` "GameAudio EffectsVolume" 0.75 "This value adjusts the loudness of the Effects sound class" (`|CreateDelegate` :!event `UpdateEffectsVolume`) true)
      (`SettingsManager.RegisterFloatCVarSettingWithCallback` "GameAudio InterfaceVolume" 0.75 "This value adjusts the loudness of the Interface sound class" (`|CreateDelegate` :!event `UpdateInterfaceVolume`) true)
      (`SettingsManager.RegisterFloatCVarSettingWithCallback` "GameAudio WeaponsVolume" 0.75 "This value adjusts the loudness of the Weapons sound class" (`|CreateDelegate` :!event `UpdateWeaponsVolume`) true)
      (`SettingsManager.RegisterFloatCVarSettingWithCallback` "CameraSensitivity MouseX" 1.0 "This value adjusts the multiplier for the Mouse X axis adjuster" (`|CreateDelegate` :!event `UpdateMouseXSensitivity`) true)
      (`SettingsManager.RegisterFloatCVarSettingWithCallback` "CameraSensitivity MouseY" 1.0 "This value adjusts the multiplier for the Mouse Y axis adjuster" (`|CreateDelegate` :!event `UpdateMouseYSensitivity`) true)
      (`SettingsManager.RegisterFloatCVarSettingWithCallback` "CameraSensitivity GamepadX" 50.0 "This value adjusts the multiplier for the Gamepad X axis adjuster" (`|CreateDelegate` :!event `UpdateGamepadXSensitivity`) true)
      (`SettingsManager.RegisterFloatCVarSettingWithCallback` "CameraSensitivity GamepadY" 50.0 "This value adjusts the multiplier for the Gamepad Y axis adjuster" (`|CreateDelegate` :!event `UpdateGamepadYSensitivity`) true))
    (:`then_2`
      (`AndroidPermissionFunctionLibrary.AcquirePermissions` (`self.AndroidPermissions`)))))

(event `UpdateMasterVolume`
  (params (NewValue :type "Float (double-precision)"))
  (`GameplayStatics.PushSoundMixModifier` "/Game/Dynamic/Sound/SM_Master.SM_Master")
  (`GameplayStatics.SetSoundMixClassOverride` "/Game/Dynamic/Sound/SM_Master.SM_Master" "/Game/Dynamic/Sound/Master.Master" NewValue 1.0 0.25))

(event `UpdateMouseXSensitivity`
  (params (NewValue :type "Float (double-precision)"))
  (bind _output_get (set `self.MouseXSensitivity` NewValue))
  (set `HuntPlayerController.LookXSensitivity_PC` _output_get (cast `HuntPlayerController` (`GameplayStatics.GetPlayerController` 0) :!pure true)))

(event `UpdateMusicVolume`
  (params (NewValue :type "Float (double-precision)"))
  (`GameplayStatics.PushSoundMixModifier` "/Game/Dynamic/Sound/SM_Master.SM_Master")
  (`GameplayStatics.SetSoundMixClassOverride` "/Game/Dynamic/Sound/SM_Master.SM_Master" "/Game/Dynamic/Sound/Music.Music" NewValue 1.0 0.25))

(event `UpdateMouseYSensitivity`
  (params (NewValue :type "Float (double-precision)"))
  (bind _output_get (set `self.MouseYSensitivity` NewValue))
  (set `HuntPlayerController.LookYSensitivity_PC` _output_get (cast `HuntPlayerController` (`GameplayStatics.GetPlayerController` 0) :!pure true)))

(event `UpdateEffectsVolume`
  (params (NewValue :type "Float (double-precision)"))
  (`GameplayStatics.PushSoundMixModifier` "/Game/Dynamic/Sound/SM_Master.SM_Master")
  (`GameplayStatics.SetSoundMixClassOverride` "/Game/Dynamic/Sound/SM_Master.SM_Master" "/Game/Dynamic/Sound/Effects.Effects" NewValue 1.0 0.25))

(event `UpdateGamepadXSensitivity`
  (params (NewValue :type "Float (double-precision)"))
  (bind _output_get (set `self.GamepadXSensitivity` NewValue))
  (set `HuntPlayerController.LookXSensitivity_GP` _output_get (cast `HuntPlayerController` (`GameplayStatics.GetPlayerController` 0) :!pure true)))

(event `UpdateInterfaceVolume`
  (params (NewValue :type "Float (double-precision)"))
  (`GameplayStatics.PushSoundMixModifier` "/Game/Dynamic/Sound/SM_Master.SM_Master")
  (`GameplayStatics.SetSoundMixClassOverride` "/Game/Dynamic/Sound/SM_Master.SM_Master" "/Game/Dynamic/Sound/Interface.Interface" NewValue 1.0 0.25))

(event `UpdateGamepadYSensitivity`
  (params (NewValue :type "Float (double-precision)"))
  (bind _output_get (set `self.GamepadYSensitivity` NewValue))
  (set `HuntPlayerController.LookYSensitivity_GP` _output_get (cast `HuntPlayerController` (`GameplayStatics.GetPlayerController` 0) :!pure true)))

(event `UpdateWeaponsVolume`
  (params (NewValue :type "Float (double-precision)"))
  (`GameplayStatics.PushSoundMixModifier` "/Game/Dynamic/Sound/SM_Master.SM_Master")
  (`GameplayStatics.SetSoundMixClassOverride` "/Game/Dynamic/Sound/SM_Master.SM_Master" "/Game/Dynamic/Sound/Weapons.Weapons" NewValue 1.0 0.25))

(event `UpdateVoiceVolume`
  (params (NewValue :type "Float (double-precision)"))
  (`GameplayStatics.PushSoundMixModifier` "/Game/Dynamic/Sound/SM_Master.SM_Master")
  (`GameplayStatics.SetSoundMixClassOverride` "/Game/Dynamic/Sound/SM_Master.SM_Master" "/Game/Dynamic/Sound/Voice.Voice" NewValue 1.0 0.25))

(fn `AdjustGlobalTimeDilation`
  (params (CurrentTimeDilation :type "Float (double-precision)"))
  (bind _output_get (set `self.CurrentTimeDilation` CurrentTimeDilation))
  (`GameplayStatics.SetGlobalTimeDilation` _output_get))

(fn `CreateEmptySave`
  (returns (ReturnValue :type "/Game/Dynamic/Blueprints/Game/Save_Load/ProjectHuntSaveGame Object Reference"))
  (bind _returnvalue (`GameplayStatics.CreateSaveGameObject` "/Game/Dynamic/Blueprints/Game/Save_Load/ProjectHuntSaveGame.ProjectHuntSaveGame_C"))
  (`/Engine/EditorBlueprintResources/StandardMacros.IsValid` _returnvalue
    (:`Is Valid`
      (bind _output_get (set `self.SaveGameReference` _returnvalue))
      (return _output_get))))

(fn `DoesPlayerHavePoints?`
  (params (StorePrice :type Integer))
  (returns (ReturnValue :type Boolean))
  (return (>= (`ProjectHuntCharacter.GetDataPoints` (cast `HuntPlayerCharacter` (`GameplayStatics.GetPlayerCharacter` 0) :!pure true)) StorePrice)))

(fn `DoManualSavesExist?`
  (returns (ReturnValue :type Boolean))
  (for _array_element (`self.SaveSlotNameArray`)
    (bind _returnvalue (`GameplayStatics.DoesSaveGameExist` _array_element))
    (if _returnvalue
      (return true)
      (else
        (return false)))))

(fn `GetPlayerData`
  (returns (`Current Health` :type "Float (double-precision)") (`Max Health` :type "Float (double-precision)") (`Current Aragon` :type "Float (double-precision)") (`Max Aragon` :type "Float (double-precision)") (WeaponInventory :type "Map of EWeaponType Enum to HuntWeapon Object Reference") (PlayerTransform :type "Transform Structure (by ref)") (CurrentSuitPower :type "ESuitMainAbilities Enum") (MaxMissiles :type Integer) (PistolStatsData :type "WeaponStatsData Structure") (RifleStatsData :type "WeaponStatsData Structure") (ShotgunStatsData :type "WeaponStatsData Structure") (CurrentItemPercentage :type "Float (double-precision)") (CurrentDataPoints :type Integer) (bCanUseMissiles :type Boolean) (bCanDash :type Boolean) (bCanWallrun :type Boolean))
  (locals (L_SavePAT :type "EAmmoType Enum") (L_SaveRAT :type "EAmmoType Enum" :default "AT_Standard") (L_SaveSAT :type "EAmmoType Enum" :default "AT_Standard") (L_SavePistolChargeLimit :type "Float (double-precision)") (L_SaveRifleChargeLimit :type "Float (double-precision)") (L_SaveSGChargeLimit :type "Float (double-precision)") (L_PistolStats :type "WeaponStatsData Structure") (L_RifleStats :type "WeaponStatsData Structure") (L_ShotgunStats :type "WeaponStatsData Structure"))
  (bind _returnvalue (`GameplayStatics.GetPlayerCharacter` 0))
  (bind _ashunt_player_character (cast `HuntPlayerCharacter` _returnvalue :!pure true))
  (bind _statscomponent (`ProjectHuntCharacter.StatsComponent` _ashunt_player_character))
  (bind _weaponinventory (`HuntPlayerCharacter.WeaponInventory` _ashunt_player_character))
  (bind (_value _returnvalue_2) (`BlueprintMapLibrary.Map_Find` _weaponinventory "WT_Shotgun"))
  (bind (_value_2 _returnvalue_3) (`BlueprintMapLibrary.Map_Find` _weaponinventory "WT_Rifle"))
  (bind (_value_3 _returnvalue_4) (`BlueprintMapLibrary.Map_Find` _weaponinventory "WT_Pistol"))
  (`/Engine/EditorBlueprintResources/StandardMacros.IsValid` _ashunt_player_character
    (:`Is Valid`
      (if _returnvalue_4
        (set `local.L_PistolStats` (`HuntWeapon.WeaponStatsData` _value_3))
        (if _returnvalue_3
          (set `local.L_RifleStats` (`HuntWeapon.WeaponStatsData` _value_2))
          (if _returnvalue_2
            (set `local.L_ShotgunStats` (`HuntWeapon.WeaponStatsData` _value)))))
      (return (`HuntStatsComponent.GetCurrentHealth` _statscomponent) (`HuntStatsComponent.GetMaxHealth` _statscomponent) (`HuntStatsComponent.GetCurrentAragon` _statscomponent) (`HuntStatsComponent.GetMaxAragon` _statscomponent) _weaponinventory (`Actor.GetTransform` _returnvalue) (`HuntStatsComponent.CurrentSuitPower` _statscomponent) (`HuntPlayerCharacter.GetMaxMissiles` _ashunt_player_character) (`local.L_PistolStats`) (`local.L_RifleStats`) (`local.L_ShotgunStats`) (`HuntPlayerController.CurrentItemPercentage` (cast `HuntPlayerController` (`GameplayStatics.GetPlayerController` 0) :!pure true)) (`ProjectHuntCharacter.CurrentDataPoints` _ashunt_player_character) (`HuntPlayerCharacter.CanPlayerUseMissiles` _ashunt_player_character) (`HuntPlayerCharacter.bCanDash` _ashunt_player_character) (`HuntPlayerCharacter.bCanWallrun` _ashunt_player_character)))))

(fn `GetProfileData`
  (returns (`bIsPrologueComplete?` :type Boolean))
  (return (`/Game/Dynamic/Blueprints/Game/BP_ProjectHuntGameStateBase.bIsPrologueComplete?` (cast `/Game/Dynamic/Blueprints/Game/BP_ProjectHuntGameStateBase` (`GameplayStatics.GetGameState`) :!pure true))))

(fn `IsSaveRecent?`
  (params (SlotName :type String))
  (locals (LocalSaveReference :type "/Game/Dynamic/Blueprints/Game/Save_Load/ProjectHuntSaveGame Object Reference"))
  (bind _returnvalue (`GameplayStatics.LoadGameFromSlot` SlotName))
  (bind _asproject_hunt_save_game (cast `/Game/Dynamic/Blueprints/Game/Save_Load/ProjectHuntSaveGame` _returnvalue))
  (bind _output_get (set `local.LocalSaveReference` _asproject_hunt_save_game))
  (bind _returnvalue_2 (`GameplayStatics.LoadGameFromSlot` "AutoSave"))
  (if (>= (`/Game/Dynamic/Blueprints/Game/Save_Load/ProjectHuntSaveGame.SaveDateTime` _output_get) (`/Game/Dynamic/Blueprints/Game/Save_Load/ProjectHuntSaveGame.SaveDateTime` (cast `/Game/Dynamic/Blueprints/Game/Save_Load/ProjectHuntSaveGame` _returnvalue_2 :!pure true)))
    (`KismetSystemLibrary.PrintString` "Manual Save is more recent")
    (else
      (`KismetSystemLibrary.PrintString` "Auto Save is more recent"))))

(fn `OnPauseGame`
  (params (bPaused :type Boolean))
  (`GameplayStatics.SetGamePaused` bPaused))

(fn `SetPlayerToCheckpoint`
  (bind _returnvalue (`GameplayStatics.DoesSaveGameExist` "AutoSave"))
  (if _returnvalue
    (`self.MenuLoadSlot` "AutoSave")
    (`Actor.K2_SetActorLocation` (`GameplayStatics.GetPlayerCharacter` 0) (.location (`/Game/Dynamic/Blueprints/Game/Save_Load/ProjectHuntSaveGame.Save_PlayerTransform` (`self.SaveGameReference`))) false false)))

(fn `StartNewGame`
  (params (SaveSlotName :type String) (LevelName :type Name))
  (bind _output_get (set `self.ManualSlotName` SaveSlotName))
  (set `self.SaveSlotName` _output_get)
  (`GameplayStatics.OpenLevel` LevelName))