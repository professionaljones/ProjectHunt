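; Gameplay game mode for Project Hunt that decides where the player pawn spawns, including when resuming from a save.
; SpawnDefaultPawnAtTransform finds the PlayerStart tagged "OriginStart", then substitutes the game instance's saved transform if loading a save made in the current level.
; A level mismatch keeps the supplied transform, while spawns without a valid save require it to match the origin start.
; InitStartSpot prints the chosen start's tag.
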(event `self.ReceiveBeginPlay`
  (set `self.PlayerRef` (cast `HuntPlayerCharacter` (`GameplayStatics.GetPlayerCharacter` 0) :!pure true))
  (`parent.ReceiveBeginPlay`))

(event `self.InitStartSpot`
  (params (StartSpot :type "Actor Object Reference") (NewPlayer :type "Controller Object Reference"))
  (bind _asplayer_start (cast `PlayerStart` StartSpot))
  (`KismetSystemLibrary.PrintString` (`KismetStringLibrary.Conv_NameToString` (`PlayerStart.PlayerStartTag` _asplayer_start))))

(fn `SpawnDefaultPawnAtTransform`
  (params (NewPlayer :type "Controller Object Reference") (SpawnTransform :type "Transform Structure (by ref)"))
  (returns (ReturnValue :type "Pawn Object Reference"))
  (bind _asbp_project_hunt_ugc_game_instance (cast `/Game/Dynamic/Blueprints/Game/BP_ProjectHuntUGC_GameInstance` (`GameplayStatics.GetGameInstance`) :!pure true))
  (bind _savegamereference (`/Game/Dynamic/Blueprints/Game/BP_ProjectHuntUGC_GameInstance.SaveGameReference` _asbp_project_hunt_ugc_game_instance))
  (bind _outactors (`GameplayStatics.GetAllActorsOfClass` "/Script/Engine.PlayerStart"))
  (for _array_element _outactors
    (if (== (`PlayerStart.PlayerStartTag` _array_element) "OriginStart")
      (set `self.OriginPlayerStart` _array_element)
      (if (`/Game/Dynamic/Blueprints/Game/BP_ProjectHuntUGC_GameInstance.bIsLoadingSave?` _asbp_project_hunt_ugc_game_instance)
        (`/Engine/EditorBlueprintResources/StandardMacros.IsValid` _savegamereference
          (:`Is Valid`
            (bind _returnvalue (`GameplayStatics.GetCurrentLevelName` true))
            (if (`KismetStringLibrary.EqualEqual_StrStr` _returnvalue (`/Game/Dynamic/Blueprints/Game/Save_Load/ProjectHuntSaveGame.Save_LevelName` _savegamereference))
              (bind _returnvalue_2 (`parent.SpawnDefaultPawnAtTransform` NewPlayer (`/Game/Dynamic/Blueprints/Game/Save_Load/ProjectHuntSaveGame.Save_PlayerTransform` _savegamereference)))
              (return _returnvalue_2)
              (else
                (bind _returnvalue_3 (`parent.SpawnDefaultPawnAtTransform` NewPlayer SpawnTransform))
                (return _returnvalue_3))))
          (:`Is Not Valid`
            _)))
      (if (== SpawnTransform (`self.GetTransform` (`self.OriginPlayerStart`)))
        (bind _returnvalue_4 (`parent.SpawnDefaultPawnAtTransform` NewPlayer SpawnTransform))
        (return _returnvalue_4)))))

(fn `UserConstructionScript`
  (`parent.UserConstructionScript`))