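; Base game mode for Project Hunt that tracks a player rank reference and runs the level time limit.
; BeginPlay sets starting difficulty and starts a fast looping timer, while damage dealt or received events raise or lower the rank reference.
; SetLevelTimer starts a one-second looping timer; LevelTimerCountdown decrements the limit, flags expiry, and turns on the Chameleon's camera shake through the GameState in the final quarter.
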(event `self.ReceiveBeginPlay`
  (`self.SetStartingDifficulty`)
  (`KismetSystemLibrary.K2_SetTimerDelegate` (`|CreateDelegate` :!event `MeasureRank`) 0.1 true))

(event `HuntDifficultyInterface.PlayerDealtDamage`
  (params (RankModiferAmount :type "Float (single-precision)"))
  (bind _output_get (set `self.CurrentRankReference` (+ RankModiferAmount (`self.CurrentRankReference`)))))

(event `HuntDifficultyInterface.PlayerReceivedDamage`
  (params (RankModiferAmount :type "Float (single-precision)"))
  (bind _output_get (set `self.CurrentRankReference` (- (`self.CurrentRankReference`) RankModiferAmount))))

(fn `GetGameRank`
  (returns (ReturnValue :type "Float (double-precision)"))
  (return (`self.PlayerRank`)))

(fn `LevelTimerCountdown`
  (bind _output_get (set `self.TimeLimit` (- (`self.TimeLimit`) 1.0)))
  (`|ExecutionSequence`
    (:`then_0`
      (if (<= _output_get 0.0)
        (set `self.bHasTimerElapsed?` true)))
    (:`then_1`
      (if (<= (/ (`self.TimeLimit`) (`self.StartingTimeLimit`)) 0.25)
        (`/Engine/EditorBlueprintResources/StandardMacros.DoOnce` false :!label _label
          (:`Completed`
            (set `/Game/Chameleon/Chameleon.Camera Shake` true (`/Game/Dynamic/Blueprints/Game/BP_ProjectHuntGameStateBase.ChameleonReference` (cast `/Game/Dynamic/Blueprints/Game/BP_ProjectHuntGameStateBase` (`GameplayStatics.GetGameState`) :!pure true)))))
        (else
          (goto _label :!via `Reset`))))))

(fn `SetLevelTimer`
  (params (StartingTimeLimit :type "Float (double-precision)"))
  (bind _output_get (set `self.StartingTimeLimit` StartingTimeLimit))
  (set `self.TimeLimit` _output_get)
  (`KismetSystemLibrary.K2_SetTimerDelegate` (`|CreateDelegate` :!event `LevelTimerCountdown`) 1.0 true))

(fn `UserConstructionScript`)