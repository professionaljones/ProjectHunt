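; Save game object for Project Hunt that stores player progress: vitals, weapons, suit, modifiers, level and transform, teleport points, saveable objects and slot metadata.
; SetSaveData writes all fields in one call, increments TimesSaved and returns the slot name.
; GetSaveData returns most fields in one call, leaving out slot name, date-time and save count.
; It only holds data, with no disk read or write logic.
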(fn `GetSaveData`
  (returns (Save_CurrentHealth :type "Float (double-precision)") (Save_MaxHealth :type "Float (double-precision)") (Save_CurrentAragon :type "Float (double-precision)") (Save_MaxAragon :type "Float (double-precision)") (Save_WeaponInventory :type "Map of Integer to HuntWeapon Object Reference") (Save_LevelName :type String) (Save_PlayerTransform :type "Transform Structure") (CurrentSuitPower :type "ESuitMainAbilities Enum") (SaveMaxMissiles :type Integer) (SavePistolStats :type "WeaponStatsData Structure") (SaveRifleStats :type "WeaponStatsData Structure") (SaveSGStats :type "WeaponStatsData Structure") (ItemPercentage :type "Float (double-precision)") (SaveableObjectArray :type "Array of /Game/Examples/UC/-PersistentVariables/Struct_SaveableObjects Structure") (Save_ManualSlotName :type String) (Save_CurrentDP :type Integer) (Save_PlayTime :type "Timespan Structure") (Save_TeleportPoints :type "Map of Name to /Game/Dynamic/Blueprints/LevelTeleporterDataStruct Structure") (Save_CurrentSuit :type "EPlayerSuit Enum") (Save_PlayerUnlockedStats :type "PlayerSaveableStats Structure") (Save_PowerModifierOne :type "ESuitPowerModifiers Enum") (Save_PowerModifierTwo :type "ESuitPowerModifiers Enum") (Save_ScreenShot :type "TextureRenderTarget2D Object Reference"))
  (return (`self.Save_CurrentHealth`) (`self.Save_MaxHealth`) (`self.Save_CurrentAragon`) (`self.Save_MaxAragon`) (`self.Save_WeaponInventory`) (`self.Save_LevelName`) (`self.Save_PlayerTransform`) (`self.Save_CurrentSuitPower`) (`self.SaveMaxMissiles`) (`self.Save_PistolStatsStruct`) (`self.Save_RifleStatsStruct`) (`self.Save_SGStatsStruct`) (`self.ItemPercentage`) (`self.SaveableObjectArray`) (`self.Save_ManualSlotName`) (`self.Save_CurrentDP`) (`self.Save_PlayTime`) (`self.Save_TeleportPoints`) (`self.Save_CurrentSuit`) (`self.Save_PlayerUnlockedStats`) (`self.Save_PowerModifierOne`) (`self.Save_PowerModifierTwo`) (`self.Save_ScreenShot`)))

(fn `SetSaveData`
  (params (Save_CurrentHealth :type "Float (double-precision)") (Save_MaxHealth :type "Float (double-precision)") (Save_CurrentAragon :type "Float (double-precision)") (Save_MaxAragon :type "Float (double-precision)") (Save_WeaponInventory :type "Map of Integer to HuntWeapon Object Reference") (Save_LevelName :type String) (Save_PlayerTransform :type "Transform Structure") (SaveSlotName :type String) (Save_CurrentSuitPower :type "ESuitMainAbilities Enum" :default "MA_None") (SaveMaxMissiles :type Integer) (SavePistolStats :type "WeaponStatsData Structure") (SaveRifleStats :type "WeaponStatsData Structure") (SaveSGStats :type "WeaponStatsData Structure") (ItemPercentage :type "Float (double-precision)") (SaveableObjectArray :type "Array of /Game/Examples/UC/-PersistentVariables/Struct_SaveableObjects Structure") (Save_ManualSlotName :type String) (Save_CurrentDP :type Integer) (SaveDateTime :type "DateTime Structure") (Save_PlayTime :type "Timespan Structure") (Save_TeleportPoints :type "Map of Name to /Game/Dynamic/Blueprints/LevelTeleporterDataStruct Structure") (Save_CurrentSuit :type "EPlayerSuit Enum" :default "Suit_Standard") (Save_PlayerUnlockedStats :type "PlayerSaveableStats Structure") (Save_PowerModifierOne :type "ESuitPowerModifiers Enum" :default "PM_None") (Save_PowerModifierTwo :type "ESuitPowerModifiers Enum" :default "PM_None") (Save_ScreenShot :type "TextureRenderTarget2D Object Reference"))
  (returns (DesiredSaveName :type String))
  (set `self.Save_CurrentHealth` Save_CurrentHealth)
  (set `self.Save_MaxHealth` Save_MaxHealth)
  (set `self.Save_CurrentAragon` Save_CurrentAragon)
  (set `self.Save_MaxAragon` Save_MaxAragon)
  (set `self.Save_WeaponInventory` Save_WeaponInventory)
  (set `self.Save_LevelName` Save_LevelName)
  (set `self.Save_PlayerTransform` Save_PlayerTransform)
  (set `self.SaveSlotName` SaveSlotName)
  (set `self.Save_CurrentSuitPower` Save_CurrentSuitPower)
  (set `self.SaveMaxMissiles` SaveMaxMissiles)
  (set `self.Save_PistolStatsStruct` SavePistolStats)
  (set `self.Save_RifleStatsStruct` SaveRifleStats)
  (set `self.Save_SGStatsStruct` SaveSGStats)
  (`/Engine/EditorBlueprintResources/StandardMacros.IncrementInt` (`self.TimesSaved`)
    (:`  `
      (set `self.ItemPercentage` ItemPercentage)
      (set `self.SaveableObjectArray` SaveableObjectArray)
      (set `self.Save_ManualSlotName` Save_ManualSlotName)
      (set `self.Save_CurrentDP` Save_CurrentDP)
      (set `self.Save_PlayerUnlockedStats` Save_PlayerUnlockedStats)
      (set `self.Save_PowerModifierOne` Save_PowerModifierOne)
      (set `self.Save_PowerModifierTwo` Save_PowerModifierTwo)
      (set `self.SaveDateTime` SaveDateTime)
      (set `self.Save_PlayTime` Save_PlayTime)
      (set `self.Save_TeleportPoints` Save_TeleportPoints)
      (set `self.Save_CurrentSuit` Save_CurrentSuit)
      (set `self.Save_ScreenShot` Save_ScreenShot)
      (return (`self.SaveSlotName`)))))