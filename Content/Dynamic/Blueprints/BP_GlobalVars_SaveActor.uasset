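; Save actor that carries global game state (current level, player transform, teleporter points) through Rama Save System events on its GlobalSaveComponent.
; BeginPlay records the level name; pre-save captures the pawn transform and the GameInstance's refreshed teleporter map.
; Pre-load-destroy reopens the saved level, then after a short Delay passes the transform to the player controller and teleporter points to the GameInstance.
; Both save and load print teleporter keys for debugging.
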(event `self.ReceiveBeginPlay`
  (bind _returnvalue (`GameplayStatics.GetCurrentLevelName` true))
  (set `/Game/Dynamic/Blueprints/BP_GlobalVarsComponent.CurrentLevel` _returnvalue (`self.GlobalSaveComponent`)))

(event `self.GlobalSaveComponent.RamaSaveEvent_PreLoadDestroy`
  (params (RamaSaveComponent :type "RamaSaveComponent Object Reference"))
  (bind _globalsavecomponent (`self.GlobalSaveComponent`))
  (`GameplayStatics.OpenLevel` (`KismetStringLibrary.Conv_StringToName` (`/Game/Dynamic/Blueprints/BP_GlobalVarsComponent.CurrentLevel` _globalsavecomponent)))
  (`KismetSystemLibrary.Delay` 0.2)
  (set `/Game/Dynamic/Blueprints/Player/BP_Gameplay_PlayerController.NewVar_1` (`/Game/Dynamic/Blueprints/BP_GlobalVarsComponent.PlayerLocation` _globalsavecomponent) (cast `/Game/Dynamic/Blueprints/Player/BP_Gameplay_PlayerController` (`GameplayStatics.GetPlayerController` 0) :!pure true))
  (bind _output_get (set `/Game/Dynamic/Blueprints/Game/BP_ProjectHuntUGC_GameInstance.SavedTeleporterPoints` (`/Game/Dynamic/Blueprints/BP_GlobalVarsComponent.TeleportPoints` _globalsavecomponent) (cast `/Game/Dynamic/Blueprints/Game/BP_ProjectHuntUGC_GameInstance` (`GameplayStatics.GetGameInstance`) :!pure true)))
  (bind _keys (`BlueprintMapLibrary.Map_Keys` _output_get))
  (for _array_element _keys
    (`KismetSystemLibrary.PrintString` (`KismetStringLibrary.Conv_NameToString` _array_element) true true (struct :`R` 1.0 :`G` 0.091858 :`A` 1.0))))

(event `self.GlobalSaveComponent.RamaSaveEvent_PreSave`
  (params (RamaSaveComponent :type "RamaSaveComponent Object Reference"))
  (bind _asbp_project_hunt_ugc_game_instance (cast `/Game/Dynamic/Blueprints/Game/BP_ProjectHuntUGC_GameInstance` (`GameplayStatics.GetGameInstance`) :!pure true))
  (bind _output_get (set `/Game/Dynamic/Blueprints/BP_GlobalVarsComponent.PlayerLocation` (`self.GetTransform` (`GameplayStatics.GetPlayerPawn` 0)) (`self.GlobalSaveComponent`)))
  (`/Game/Dynamic/Blueprints/Game/BP_ProjectHuntUGC_GameInstance.SaveTeleportPoints` _asbp_project_hunt_ugc_game_instance)
  (bind _output_get_2 (set `/Game/Dynamic/Blueprints/BP_GlobalVarsComponent.TeleportPoints` (`/Game/Dynamic/Blueprints/Game/BP_ProjectHuntUGC_GameInstance.SavedTeleporterPoints` _asbp_project_hunt_ugc_game_instance) (`self.GlobalSaveComponent`)))
  (bind _keys (`BlueprintMapLibrary.Map_Keys` _output_get_2))
  (for _array_element _keys
    (`KismetSystemLibrary.PrintString` (`KismetStringLibrary.Conv_NameToString` _array_element))))

(fn `UserConstructionScript`)