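; BP_ShieldPylon is a damageable pylon that goes down when its health runs out and then recovers over time.
; It passes damage to its HuntStats only when the damage causer matches BP_SentryProjectile.
; Once dead, a looping one-second timer, apparently driving RegenHealth, restores health in steps until full, then clears the dead flag and timer.
; BeginPlay stores a dynamic material for ShapeSphere, which this file never changes.
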(event `self.ReceiveBeginPlay`
  (bind _shape_sphere (`self.Shape_Sphere`))
  (bind _returnvalue (`PrimitiveComponent.CreateDynamicMaterialInstance` _shape_sphere 0 (`PrimitiveComponent.GetMaterial` _shape_sphere 0) "None"))
  (set `self.Shield_DynMat` _returnvalue))

(event `self.ReceiveAnyDamage`
  (params (Damage :type "Float (single-precision)") (DamageType :type "DamageType Object Reference") (InstigatedBy :type "Controller Object Reference") (DamageCauser :type "Actor Object Reference"))
  (if (== DamageCauser "/Game/Dynamic/Blueprints/Weapons/Projectiles/BP_SentryProjectile.BP_SentryProjectile")
    (`HuntStatsComponent.DamageHealth` (`self.HuntStats`) Damage)
    (if (`HuntStatsComponent.bIsDead` (`self.HuntStats`))
      (bind _returnvalue (`KismetSystemLibrary.K2_SetTimerDelegate` (`|CreateDelegate` :!event `RegenHealth`) 1.0 true))
      (set `self.RegenHealthTimer` _returnvalue))))

(event `RegenHealth`
  (bind _huntstats (`self.HuntStats`))
  (if (`HuntStatsComponent.bIsDead` _huntstats)
    (`HuntStatsComponent.RecoverHealth` (`self.HuntStats`) 5.0)
    (if (>= (`HuntStatsComponent.GetPlayerCurrentHealth` _huntstats) (`HuntStatsComponent.GetPlayerMaxHealth` _huntstats))
      (set `HuntStatsComponent.bIsDead` false _huntstats)
      (`KismetSystemLibrary.K2_ClearAndInvalidateTimerHandle` (`self.RegenHealthTimer`)))))

(fn `UserConstructionScript`)