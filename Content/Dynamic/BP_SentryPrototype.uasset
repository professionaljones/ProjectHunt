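; BP_SentryPrototype is a prototype sentry actor with a shield and health.
; BeginPlay creates a dynamic shield material and starts a rotation timeline meant to sweep the actor's yaw.
; Incoming damage makes the causer's projectile bounce while the shield is active, otherwise it reduces health through HuntStats.
; Unconnected draft logic covers sphere-trace detection that pauses rotation to spawn a projectile at the hit point, and timeline-driven shield materialization.
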(event `self.ReceiveBeginPlay`
  (bind _shape_cylinder (`self.Shape_Cylinder`))
  (bind _returnvalue (`PrimitiveComponent.CreateDynamicMaterialInstance` _shape_cylinder 0 (`PrimitiveComponent.GetMaterial` _shape_cylinder 0) "None"))
  (set `self.Shield_DynMat` _returnvalue)
  (`TimelineComponent.PlayFromStart` (`self.RotateTimeline`)))

(event `self.ReceiveAnyDamage`
  (params (Damage :type "Float (single-precision)") (DamageType :type "DamageType Object Reference") (InstigatedBy :type "Controller Object Reference") (DamageCauser :type "Actor Object Reference"))
  (if (`self.bIsShieldActive?`)
    (set `ProjectileMovementComponent.bShouldBounce` true (`self.GetComponentByClass` DamageCauser "/Script/Engine.ProjectileMovementComponent"))
    (else
      (`HuntStatsComponent.DamageHealth` (`self.HuntStats`) Damage))))

(event `self.ReceiveTick`
  (params (DeltaSeconds :type "Float (single-precision)")))

(fn `UserConstructionScript`)