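; BP_SentryTurret is a sentry turret actor that constantly faces the first player character and fires projectiles at it.
; Each Tick snaps the whole actor to a look-at rotation, with no range or line-of-sight check.
; A half-second Delay on Tick throttles fire, spawning BP_SentryProjectile with a fixed damage output at the actor's location and rotation.
; A gun socket rotation lookup is present but unused.
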(event `self.ReceiveTick`
  (params (DeltaSeconds :type "Float (single-precision)"))
  (`self.K2_SetActorRotation` (`KismetMathLibrary.FindLookAtRotation` (`self.K2_GetActorLocation`) (`self.K2_GetActorLocation` (`GameplayStatics.GetPlayerCharacter` 0))))
  (`KismetSystemLibrary.Delay` 0.5)
  (`|SpawnActorFromClass` "/Game/Dynamic/Blueprints/Weapons/Projectiles/BP_SentryProjectile.BP_SentryProjectile_C" (`KismetMathLibrary.MakeTransform` (`self.K2_GetActorLocation`) (`self.K2_GetActorRotation`)) "Undefined" "OverrideRootScale" null 5.0 null))

(fn `UserConstructionScript`)