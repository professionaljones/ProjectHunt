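; Test player controller for the MTS tutorial system, linking player input, tutorial stage progress and the HUD.
; Fire_Weapon and Jump presses record the current input type and send a key ID, directly on authority or through a server call on remotes.
; Next-stage calls pass to the MTSListener component, whose new-stage event triggers a local HUD stage message.
; Getters expose the current input type and stage ID.
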(event `/Game/FILab/MTS/BPI_MTSListener.HandleNextStage`
  (params (StageID :type Name))
  ;[1 1 1] Push to our component and hud
  (`/Game/FILab/MTS/BPC_MTSListener.HandleNextStage` (`self.MTSListener`) StageID))

(event `InputAction|Fire_Weapon`
  (params (Key :type "Key Structure"))
  (:`Pressed`
    (`self.Template_ProcessKey` Key "Fire_Weapon")))

(event `InputAction|Jump`
  (params (Key :type "Key Structure"))
  (:`Pressed`
    (`self.Template_ProcessKey` Key "Jump")))

(event `self.MTSListener.NewTutorialStage`
  (params (Component :type "/Game/FILab/MTS/BPC_MTSListener Object Reference"))
  ;[1 1 1] Wait for listener to tell us it's okay to show next stage
  (`self.Local_UpdateStage` Component))

(event `Server_SendInputKey`
  (params (KeyID :type Name))
  (`/Game/FILab/MTS/BPFL_MTS.SendInputKey` self KeyID))

(event `Local_UpdateStage`
  (params (Component :type "/Game/FILab/MTS/BPI_MTSListener Interface"))
  ;[1 1 1] Wait for listener to tell us it's okay to show next stage
  (bind _currentstage (`/Game/FILab/MTS/BPI_MTSListener.GetCurrentStageID` Component))
  (message `/Game/FILab/MTS/BPI_MTSHUD.SendTutorialStage` (`self.GetHUD`) _currentstage))

(fn `GetCurrentInputType`
  (returns (InputType :type "/Game/FILab/MTS/EInputType Enum"))
  ;[1 1 1] You can also push this to the component if you want, but there's no need to
  (return (`self.CurrentInputType`)))

(fn `GetCurrentStageID`
  (returns (CurrentStage :type Name))
  (bind _currentstage (`/Game/FILab/MTS/BPC_MTSListener.GetCurrentStageID` (`self.MTSListener`)))
  (return _currentstage))

(fn `Template_ProcessKey`
  (params (Key :type "Key Structure" :default "None") (KeyID :type Name))
  (set `self.CurrentInputType` (`/Game/FILab/MTS/BPFL_MTS.ProcessInputKey` Key))
  (`/Engine/EditorBlueprintResources/ActorMacros.Switch Has Authority`
    (:`Authority`
      (`/Game/FILab/MTS/BPFL_MTS.SendInputKey` self KeyID))
    (:`Remote`
      (`self.Server_SendInputKey` KeyID))))

(fn `UserConstructionScript`)