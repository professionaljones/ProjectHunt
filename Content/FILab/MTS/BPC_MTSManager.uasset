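; Manager component for a multiplayer tutorial system (MTS) that tracks each client's current stage and advances it along a data-table-defined sequence.
; After a BeginPlay delay, it loads TutorialTable and, as a demo kickoff, starts every BPI_MTSListener actor on the first stage.
; Stage requests succeed only when matching the client's recorded stage; the client then receives the next stage via HandleNextStageMessage.
; Server events update progress, and a multicast replicates the client-to-stage map.
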(event `self.ReceiveBeginPlay`
  ;[1 0.38 0] Load the data from the default table
  (`KismetSystemLibrary.Delay` 2.0)
  (if (`KismetSystemLibrary.IsServer`)
    (`self.Default_Initialize` :!label _label)
    (else
      (`self.Server_Play`))))

(event `Server_Play`
  ;[1 0.38 0] Load the data from the default table
  (goto _label))

(event `Multicast_UpdateClientTutorialProgress`
  (params (ClientTutorialProgress :type "Map of Object Object Reference to Name"))
  ;[0 0 0] Set tutorial progress
  (set `self.ClientTutorialProgress` ClientTutorialProgress))

(event `Server_UpdateClientTutorialProgress`
  (params (Key :type "Object Object Reference (by ref)") (Value :type "Name (by ref)"))
  ;[0 0 0] Set tutorial progress
  (`self.UpdateClientTutorialProgress` Key Value))

(event `Server_TryProcessNextStage`
  (params (Key :type "Object Object Reference (by ref)") (Value :type "Name (by ref)"))
  (`self.TryProcessTutorialStage` Key Value))

(fn `AddClient`
  (params (Key :type "Object Object Reference (by ref)") (InputPin :type Name))
  (message `/Game/FILab/MTS/BPI_MTSListener.HandleNextStage` Key InputPin)
  (`self.UpdateClientTutorialProgress` Key InputPin))

(fn `CanClientRunNextStage`
  (params (Client :type "Object Object Reference") (StageID :type Name))
  (returns (bSuccess :type Boolean))
  (locals (L_FoundStage :type Name))
  (bind (_bfound _nextstage) (`self.GetNextStage` (`local.StageID`)))
  ;[1 0.38 0] Try to set stage for client. Client can only move to stage if the current stage their on == the stage that was passed to the client.
  (`/Engine/EditorBlueprintResources/StandardMacros.IsValid` (`local.Client`)
    (:`Is Valid`
      (set `local.L_FoundStage` (`BlueprintMapLibrary.Map_Find` (`self.ClientTutorialProgress`) (`local.Client`)))
      (if (== (`local.L_FoundStage`) (`local.StageID`))
        (if _bfound
          (`self.Server_UpdateClientTutorialProgress` (`local.Client`) _nextstage)
          (return true)
          (else
            (`KismetSystemLibrary.PrintString` (`KismetStringLibrary.Concat_StrStr` "MTSManager : Failed to find next stage for " (`KismetStringLibrary.Conv_NameToString` (`local.StageID`))) true true (struct :`R` 1.0 :`A` 1.0))
            (return false)))
        (else
          (`KismetSystemLibrary.PrintString` (`KismetStringLibrary.Concat_StrStr` "MTSManager :" " Client - " (`KismetSystemLibrary.GetDisplayName` (`local.Client`)) " tried to go to stage " (`KismetStringLibrary.Conv_NameToString` (`local.StageID`)) " but is at stage " (`KismetStringLibrary.Conv_NameToString` (`local.L_FoundStage`))) true true (struct :`R` 1.0 :`A` 1.0))
          (return false))))
    (:`Is Not Valid`
      (`KismetSystemLibrary.PrintString` "MTSManager : Invalid Client!" true true (struct :`R` 1.0 :`A` 1.0))
      (return false))))

(fn `Default_Initialize`
  ;[0 0 0] Load the tutorial data from the default table.
  (bind _outrownames (`DataTableFunctionLibrary.GetDataTableRowNames` (`self.TutorialTable`)))
  (for _array_element _outrownames
    (bind _returnvalue (`|GetDataTableRow` (`self.TutorialTable`) _array_element)
      (:`then`
        (`KismetArrayLibrary.Array_Add` (`self.TutorialMap`) _returnvalue))))
  ;[1 1 1] This is a demo implementation.
  ; If you are running this in a real scenario you will want to have a second mathod to kick off the tutorial for the connected client
  (bind _outactors (`GameplayStatics.GetAllActorsWithInterface` "/Game/FILab/MTS/BPI_MTSListener.BPI_MTSListener_C"))
  (for _array_element_2 _outactors
    (`self.AddClient` _array_element_2 (`.StageID_17_8F9D3C5B426A5F9D9E377BA79DE1FFF9` (break `/Game/FILab/MTS/FMTSStage` (`|GetArrayItem` (`self.TutorialMap`)))))))

(fn `GetClientTutorialStage`
  (params (Client :type "Object Object Reference"))
  (returns (StageID :type Name))
  (return (`BlueprintMapLibrary.Map_Find` (`self.ClientTutorialProgress`) Client)))

(fn `GetNextStage`
  (params (StageID :type Name))
  (returns (bFound :type Boolean) (NextStage :type Name))
  ;[1 0.38 0] Find the matching stage id and return
  (for _array_element (`self.TutorialMap`)
    (bind ((`StageID_17_8F9D3C5B426A5F9D9E377BA79DE1FFF9` _stageid) (`NextStage_19_5BCD4BA5472F13BC02640097E75CC593` _nextstage)) (break `/Game/FILab/MTS/FMTSStage` _array_element))
    (if (== (`local.StageID`) _stageid)
      (return true _nextstage)))
  (return false "None"))

(fn `TryProcessTutorialStage`
  (params (Client :type "Object Object Reference") (StageID :type Name))
  (returns (bSuccess :type Boolean))
  ;[1 1 1] Check to see if the client can run the stage, if tell the client to handle the stage.
  (bind _bsuccess (`self.CanClientRunNextStage` (`local.Client`) (`local.StageID`)))
  (if _bsuccess
    (message `/Game/FILab/MTS/BPI_MTSListener.HandleNextStage` (`local.Client`) (`.NextStage` (`self.GetNextStage` (`local.StageID`))))
    (return true)
    (else
      (return false))))

(fn `UpdateClientTutorialProgress`
  (params (Key :type "Object Object Reference (by ref)") (Value :type "Name (by ref)"))
  (`BlueprintMapLibrary.Map_Add` (`self.ClientTutorialProgress`) Key Value)
  (`self.Multicast_UpdateClientTutorialProgress` (`self.ClientTutorialProgress`)))