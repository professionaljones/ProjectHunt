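; Listener component for the MTS tutorial system that tracks the current stage ID and announces stage changes.
; HandleNextStage sets the ID directly on the server, while clients route it through a server call, which applies it without validation.
; The setter and the RepNotify both fire NewTutorialStage with the component itself, so receivers read the stage through a getter.
; The input type getter returns a fixed enum value.
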(event `self.ReceiveTick`
  (params (DeltaSeconds :type "Float (single-precision)")))

(event `/Game/FILab/MTS/BPI_MTSListener.HandleNextStage`
  (params (StageID :type Name))
  ;[1 0.38 0] Set the stage ID and broadcast it. We authorize on the server to prevent cheating
  (if (`KismetSystemLibrary.IsServer`)
    (`self.OnSetCurrentStageID` StageID)
    (else
      (`self.Server_SetCurrentStageID` StageID))))

(event `Server_SetCurrentStageID`
  (params (CurrentStageID :type Name))
  ;[1 0.38 0] Set the stage ID and broadcast it. We authorize on the server to prevent cheating
  (`self.OnSetCurrentStageID` CurrentStageID))

(fn `GetCurrentInputType`
  (returns (InputType :type "/Game/FILab/MTS/EInputType Enum"))
  (return "NewEnumerator0"))

(fn `GetCurrentStageID`
  (returns (CurrentStage :type Name))
  (return (`self.CurrentStageID`)))

(fn `OnRep_CurrentStageID`
  ;[1 0.38 0] Report new stage. Get current stage ID via interface
  (`self.NewTutorialStage` self))

(fn `OnSetCurrentStageID`
  (params (CurrentStageID :type Name))
  (set `self.CurrentStageID` CurrentStageID)
  (`self.NewTutorialStage` self))